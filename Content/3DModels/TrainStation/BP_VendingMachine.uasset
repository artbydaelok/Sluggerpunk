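; Train station vending machine that sells the player a drink for gold.
; A sphere overlap shows the purchase prompt and enables Interact input, which is refused with a sound if the player has already drunk.
; PayAndDrink checks and deducts gold, then calls the player's DrinkJuiceEvent after a delay.
; The construction script picks cup or can visuals, and a random-duration timeline flickers the light from BeginPlay.
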(event `self.ReceiveBeginPlay`
  ;[0.5284 0.9502 1] Light Flicker
  (`/Engine/EditorBlueprintResources/StandardMacros.DoOnce` false :!label _label
    (:`Completed`
      (`|ExecutionSequence`
        (:`then_0`
          (bind (_direction _flickerintensity) (`Timeline|Flicker` :`NewTime` (`KismetMathLibrary.RandomFloatInRange` 0.5 3.0) :!via `SetNewTime` :!label _label_2)
            (:`Update`
              (`LightComponent.SetIntensity` (`self.PointLight`) (`KismetMathLibrary.Lerp` 150.0 250.0 _flickerintensity)))
            (:`Finished`
              (goto _label :!via `Reset`))))
        (:`then_1`
          (goto _label_2 :!via `PlayFromStart`))))))

(event `InputAction|Interact`
  (params (Key :type "Key Structure"))
  (:`Pressed`
    (if (`/Game/Player/PlayerBaseCharacter.HasDrank` (stale `self.Sphere.OnComponentBeginOverlap` _asplayer_base_character))
      (`GameplayStatics.PlaySound2D` "/Engine/VREditor/Sounds/UI/Dockable_Window_Drop.Dockable_Window_Drop" 1.0 1.0 0.0 null null)
      (elif (`self.CanInteractVM`)
        (`self.PayAndDrink`)
        (else
          (`GameplayStatics.PlaySound2D` "/Engine/EditorSounds/Notifications/CompileFailed.CompileFailed" 1.0 1.0 0.0 null null))))))

(event `self.Sphere.OnComponentBeginOverlap`
  (params (OverlappedComponent :type "PrimitiveComponent Object Reference") (OtherActor :type "Actor Object Reference") (OtherComp :type "PrimitiveComponent Object Reference") (OtherBodyIndex :type Integer) (bFromSweep :type Boolean) (SweepResult :type "HitResult Structure (by ref)"))
  (bind _returnvalue (`GameplayStatics.GetPlayerCharacter` 0))
  (if (== OtherActor _returnvalue)
    (bind _asplayer_base_character (cast `/Game/Player/PlayerBaseCharacter` _returnvalue))
    (if (`/Game/Player/PlayerBaseCharacter.HasDrank` _asplayer_base_character)
      (`self.EnableInput` (stale _asplayer_base_controller))
      (else
        (`SceneComponent.SetVisibility` (`self.EToPurchase`) true false)
        (set `self.CanInteractVM` true)
        (bind _asplayer_base_controller (cast `/Game/Player/PlayerBaseController` (`GameplayStatics.GetPlayerController` 0)))
        (`self.EnableInput` _asplayer_base_controller)))))

(event `self.Sphere.OnComponentEndOverlap`
  (params (OverlappedComponent :type "PrimitiveComponent Object Reference") (OtherActor :type "Actor Object Reference") (OtherComp :type "PrimitiveComponent Object Reference") (OtherBodyIndex :type Integer))
  (if (== OtherActor (`GameplayStatics.GetPlayerCharacter` 0))
    (`SceneComponent.SetVisibility` (`self.EToPurchase`) false false)
    (set `self.CanInteractVM` false)
    (bind _asplayer_base_controller (cast `/Game/Player/PlayerBaseController` (`GameplayStatics.GetPlayerController` 0)))
    (`self.DisableInput` _asplayer_base_controller)))

(fn `EnemyAttack`
  (returns (AttackDuration :type "Float (double-precision)"))
  (return 0.0))

(fn `EnemyShockwave`
  (returns (`Attack Duration` :type "Float (double-precision)"))
  (return 0.0))

(fn `UserConstructionScript`
  (if (`self.CupIce?`)
    (`SceneComponent.SetVisibility` (`self.CupIce`) true false)
    (`SceneComponent.SetVisibility` (`self.Can`) false false)
    (else
      (`SceneComponent.SetVisibility` (`self.CupIce`) false false)
      (`SceneComponent.SetVisibility` (`self.Can`) true false))))