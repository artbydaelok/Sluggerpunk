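; BP_GlassCoin is a train station actor that breaks into collectible gold when hit by a baseball.
; When its Box collider begins overlapping a BP_Baseball, it spawns a BP_Gold slightly below its own location, passing its CoinValue as the gold's value.
; It then destroys itself, and the class check ignores every other overlapping actor.
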(event `self.Box.OnComponentBeginOverlap`
  (params (OverlappedComponent :type "PrimitiveComponent Object Reference") (OtherActor :type "Actor Object Reference") (OtherComp :type "PrimitiveComponent Object Reference") (OtherBodyIndex :type Integer) (bFromSweep :type Boolean) (SweepResult :type "HitResult Structure (by ref)"))
  (bind (_returnvalue_x _returnvalue_y _returnvalue_z) (`KismetMathLibrary.BreakVector` (`self.K2_GetActorLocation`)))
  (if (== (`GameplayStatics.GetObjectClass` OtherActor) "/Game/Player/BaseballProj/Baseball/BP_Baseball.BP_Baseball_C")
    (`|SpawnActorFromClass` "/Game/Collectibles/BP_Gold.BP_Gold_C" (`KismetMathLibrary.MakeTransform` (`KismetMathLibrary.MakeVector` _returnvalue_x _returnvalue_y (- _returnvalue_z 100.0))) "AdjustIfPossibleButAlwaysSpawn" "OverrideRootScale" null (`self.Coin Value`) "NewEnumerator5" false null)
    (`self.K2_DestroyActor`)))

(fn `UserConstructionScript`)