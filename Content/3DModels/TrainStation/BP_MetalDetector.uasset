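; Train station metal detector prop that reacts when the player walks through it.
; On player overlap, if not already active, it swaps its red lamp meshes to dimmed and its green ones to emissive with a 2D sound.
; After a short delay it restores the red lights and plays a switch sound at the detector's location, with the On flag blocking retriggers meanwhile.
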(event `self.ReceiveActorBeginOverlap`
  (params (OtherActor :type "Actor Object Reference"))
  (if (== OtherActor (`GameplayStatics.GetPlayerCharacter` 0))
    (if (not (`self.On`))
      (`self.Color Switcher`)
      (`KismetSystemLibrary.Delay` 2.0)
      (`self.ColorSwitchBack`))))

(fn `Color Switcher`
  (set `self.On` true)
  (`GameplayStatics.PlaySound2D` "/Engine/VREditor/Sounds/UI/Enter_Play.Enter_Play" 1.0 1.0 0.0 null null)
  (`PrimitiveComponent.SetMaterial` (`self.Red1`) 0 "/Game/Textures/MI_OpacityLight.MI_OpacityLight")
  (`PrimitiveComponent.SetMaterial` (`self.Red2`) 0 "/Game/Textures/MI_OpacityLight.MI_OpacityLight")
  (`PrimitiveComponent.SetMaterial` (`self.Green2`) 0 "/Game/Textures/MI_EmissiveGreen.MI_EmissiveGreen")
  (`PrimitiveComponent.SetMaterial` (`self.Green1`) 0 "/Game/Textures/MI_EmissiveGreen.MI_EmissiveGreen"))

(fn `ColorSwitchBack`
  (set `self.On` false)
  (`GameplayStatics.PlaySoundAtLocation` "/Engine/VREditor/Sounds/UI/Flashlight_Switch.Flashlight_Switch" (`SceneComponent.K2_GetComponentLocation` (`self.MetalDetector`)) (struct) 1.0 1.0 0.0 "/Game/Levels/Milestone2Levels/Melee-Ranged-Mix/RangedLevel/SA_MetalDetectorOff.SA_MetalDetectorOff" null null)
  (`PrimitiveComponent.SetMaterial` (`self.Red1`) 0 "/Game/Textures/MI_EmissiveRed.MI_EmissiveRed")
  (`PrimitiveComponent.SetMaterial` (`self.Red2`) 0 "/Game/Textures/MI_EmissiveRed.MI_EmissiveRed")
  (`PrimitiveComponent.SetMaterial` (`self.Green2`) 0 "/Game/Textures/MI_OpacityLight.MI_OpacityLight")
  (`PrimitiveComponent.SetMaterial` (`self.Green1`) 0 "/Game/Textures/MI_OpacityLight.MI_OpacityLight"))

(fn `UserConstructionScript`)