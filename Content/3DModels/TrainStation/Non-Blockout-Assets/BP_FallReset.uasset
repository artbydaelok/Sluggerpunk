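; BP_FallReset is an actor that returns the player to a set spawn point on overlap, by its name a reset after falling in the train station.
; ActorBeginOverlap filters for player character 0 and calls MovePlayer, which casts to PlayerBaseCharacter and moves it to SpawnLocationTargetPoint without sweeping.
; It then resets controller rotation to the yaw in its ControlRotation variable.
; An EnemyAttack function only returns zero.
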(event `self.ReceiveActorBeginOverlap`
  (params (OtherActor :type "Actor Object Reference"))
  (set `self.Other Actor` OtherActor)
  (if (== (`GameplayStatics.GetPlayerCharacter` 0) OtherActor)
    (`self.Move Player` (`self.Other Actor`))))

(fn `EnemyAttack`
  (returns (AttackDuration :type "Float (double-precision)"))
  (return 0.0))

(fn `Move Player`
  (params (ActorObjectRef :type "Actor Object Reference"))
  (bind _asplayer_base_character (cast `/Game/Player/PlayerBaseCharacter` ActorObjectRef))
  (`self.K2_SetActorLocation` _asplayer_base_character (`self.K2_GetActorLocation` (`self.SpawnLocationTargetPoint`)) false false)
  (`Controller.SetControlRotation` (`GameplayStatics.GetPlayerController` 0) (`KismetMathLibrary.MakeRotator` 0.0 0.0 (`self.ControlRotation`))))

(fn `UserConstructionScript`)