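; Train station hazard that repeatedly sends a train between two points, damaging the player and sending them back on contact.
; A self-restarting event waits a set delay, shows the train, plays audio, slides it along with a timeline lerp, then hides it.
; Box overlap applies damage and teleports the player to a reset point with a set facing.
; The death event and its health check are disconnected.
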(event `ChooChoo`
  (`KismetSystemLibrary.Delay` (stale `self.ReceiveBeginPlay` _output_get))
  (`SceneComponent.SetVisibility` (`self.Train`) true true)
  (`AudioComponent.Play` (`self.Audio`) 0.3)
  (bind (_direction _doppler) (`Timeline|Neeewwww` :!via `PlayFromStart`)
    (:`Update`
      (`SceneComponent.K2_SetRelativeLocation` (`self.Train`) (`KismetMathLibrary.VLerp` (`SceneComponent.RelativeLocation` (`self.StartLocation`)) (`SceneComponent.RelativeLocation` (`self.EndLocation`)) _doppler) false false))
    (:`Finished`
      (`SceneComponent.SetVisibility` (`self.Train`) false true)
      (`KismetSystemLibrary.Delay` 0.2)
      (set `self.TimerAmount` (`self.TimerAmount`))
      (`self.ChooChoo`))))

(event `self.ReceiveBeginPlay`
  ;[1 1 1] If Left is true rotate train to face left, world position
  (if (`self.Left`)
    (`SceneComponent.K2_SetWorldRotation` (`self.Train`) (struct :`Yaw` 180.0) false false))
  ;[1 1 1] Hides train and Executes ChooChoo moving train
  (`SceneComponent.SetVisibility` (`self.Train`) false true)
  (bind _output_get (set `self.TimerAmount` (`self.TimerAmount`)))
  (`KismetSystemLibrary.PrintString` (`KismetStringLibrary.Conv_DoubleToString` _output_get))
  (`self.ChooChoo`))

(event `self.Box.OnComponentBeginOverlap`
  (params (OverlappedComponent :type "PrimitiveComponent Object Reference") (OtherActor :type "Actor Object Reference") (OtherComp :type "PrimitiveComponent Object Reference") (OtherBodyIndex :type Integer) (bFromSweep :type Boolean) (SweepResult :type "HitResult Structure (by ref)"))
  ;[1 1 1] Moves and damages player if player collides with train, if damage would kill player player dies
  (if (== (`GameplayStatics.GetPlayerCharacter` 0) OtherActor)
    (bind _asplayer_base_character (cast `/Game/Player/PlayerBaseCharacter` OtherActor))
    (`/Engine/EditorBlueprintResources/StandardMacros.IsValid` _asplayer_base_character
      (:`Is Valid`
        (`/Game/Combat/I_Combat.TakeDamage` _asplayer_base_character (`self.TrainDamage`) null null null "NewEnumerator4" true 1.0)
        (`/Engine/EditorBlueprintResources/StandardMacros.IsValid` _asplayer_base_character
          (:`Is Valid`
            (`self.K2_SetActorLocation` _asplayer_base_character (`self.K2_GetActorLocation` (`self.ResetPoint`)) false false)
            (`Controller.SetControlRotation` (`GameplayStatics.GetPlayerController` 0) (`KismetMathLibrary.MakeRotator` 0.0 0.0 (`self.PlayerRotation`)))))))))

(event `/Game/Combat/I_Combat.On Death`
  ;[1 1 1] Death Event
  (`KismetSystemLibrary.PrintString` "Player Death")
  (`/Game/Player/PlayerBaseGamemode.PlayerDeath` (cast `/Game/Player/PlayerBaseGamemode` (`GameplayStatics.GetGameMode`) :!pure true)))

(fn `EnemyAttack`
  (returns (AttackDuration :type "Float (double-precision)"))
  (return 0.0))

(fn `EnemyShockwave`
  (returns (`Attack Duration` :type "Float (double-precision)"))
  (return 0.0))

(fn `UserConstructionScript`)