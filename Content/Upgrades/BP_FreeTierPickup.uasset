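; A spinning world pickup that offers the player a free upgrade tier boost, with a name label that yaws to face the player.
; On overlap by a player who owns at least one upgrade, it toggles game pause.
; When paused, it shows a W_FreeTierBoost widget built from the upgrade inventory with UI-only input and mouse cursor.
; It destroys itself after toggling.
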(event `self.ReceiveBeginPlay`
  (bind _returnvalue (`GameplayStatics.GetActorOfClass` "/Game/Player/PlayerBaseCharacter.PlayerBaseCharacter_C"))
  (set `self.Player` _returnvalue)
  (bind (_direction _rotatealpha) (`Timeline|Animation`)
    (:`Update`
      (`self.K2_SetActorRotation` (`KismetMathLibrary.MakeRotator` 0.0 0.0 (`KismetMathLibrary.Lerp` 0.0 360.0 _rotatealpha))))))

(event `self.ReceiveActorBeginOverlap`
  (params (OtherActor :type "Actor Object Reference"))
  (bind _player (`self.Player`))
  (if (and (== OtherActor _player) (> (`KismetArrayLibrary.Array_Length` (`/Game/Player/PlayerBaseCharacter.Upgrades` _player)) 0))
    (`self.Toggle Upgrades`)))

(event `self.ReceiveTick`
  (params (DeltaSeconds :type "Float (single-precision)"))
  (bind (_returnvalue_roll _returnvalue_pitch _returnvalue_yaw) (`KismetMathLibrary.BreakRotator` (`KismetMathLibrary.FindLookAtRotation` (`self.K2_GetActorLocation`) (`self.K2_GetActorLocation` (`self.Player`)))))
  (`SceneComponent.K2_SetWorldRotation` (`self.Name`) (`KismetMathLibrary.MakeRotator` 0.0 0.0 _returnvalue_yaw) false false))

(fn `Toggle Upgrades`
  (bind _returnvalue (`GameplayStatics.GetPlayerController` 0))
  (bind _returnvalue_2 (`GameplayStatics.IsGamePaused`))
  (bind _tierwidget (`self.TierWidget`))
  (bind _returnvalue_3 (`|CreateWidget` "/Game/Player/PlayerWidgets/W_FreeTierBoost.W_FreeTierBoost_C" (`GameplayStatics.GetPlayerController` 0)))
  (set `self.TierWidget` _returnvalue_3)
  (`GameplayStatics.SetGamePaused` (not _returnvalue_2))
  (if _returnvalue_2
    (`UserWidget.AddToViewport` _tierwidget 0)
    (set `PlayerController.bShowMouseCursor` true _returnvalue)
    (`WidgetBlueprintLibrary.SetInputMode_UIOnlyEx` _returnvalue null)
    (`/Game/Player/PlayerWidgets/W_FreeTierBoost.BuildUpgradeInventory` (`self.TierWidget`))
    (`self.K2_DestroyActor`)
    (else
      (`Widget.RemoveFromParent` _tierwidget)
      (set `PlayerController.bShowMouseCursor` false _returnvalue)
      (`WidgetBlueprintLibrary.SetInputMode_GameOnly` _returnvalue)
      (`self.K2_DestroyActor`))))

(fn `UserConstructionScript`)