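; BP_SpecialPickup is an interactable upgrade pickup that grants the player a ball special.
; On BeginPlay it labels its TextRender with the BallSpecial enum name, then runs the parent logic.
; Interact calls the parent, sets the player's CurrentSpecial, shows a W_PickupPopup widget and plays HUD upgrade and charge animations.
; Logic to destroy the other special pickups is present but disconnected.
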(event `self.ReceiveBeginPlay`
  (`TextRenderComponent.K2_SetText` (`self.TextRender`) (`KismetTextLibrary.Conv_StringToText` (`|GetEnumeratorNameAsString` (`self.BallSpecial`))))
  (`parent.ReceiveBeginPlay`))

(event `/Game/Player/I_Interaction._Interact`
  (params (Player :type "/Game/Player/PlayerBaseCharacter Object Reference"))
  (bind _player (`self.Player`))
  (bind _w_hud (`/Game/Player/PlayerBaseCharacter.W_HUD` _player))
  ;[1 1 1] Ball Special
  (`parent._Interact` Player)
  (set `/Game/Player/PlayerBaseCharacter.CurrentSpecial` (`self.BallSpecial`) _player)
  (bind _returnvalue (`|CreateWidget` "/Game/Upgrades/W_PickupPopup.W_PickupPopup_C"))
  (bind _output_get (set `self.Widget` _returnvalue))
  (`UserWidget.AddToViewport` _output_get 0)
  (`/Game/Player/PlayerWidgets/W_PlayerHUD.Play HUD Upgrade Anim` _w_hud)
  (`/Game/Player/PlayerWidgets/W_PlayerHUD.PlayChargeUpdateAnims` _w_hud))

(fn `UserConstructionScript`
  (`parent.UserConstructionScript`))