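; Base upgrade pickup that turns to face the player and, on interact, grants its upgrade, plays a sound and destroys itself.
; On begin play it builds a DT_UpgradeData row name from the upgrade type and enum, then fills its name text and floating icon.
; Interacting increments the game instance's pickup count and passes the data to the player, except for BP_SpecialPickup, which skips that handoff.
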(event `self.ReceiveBeginPlay`
  ;[1 1 1] Begin Play
  (bind _returnvalue (`GameplayStatics.GetActorOfClass` "/Game/Player/PlayerBaseCharacter.PlayerBaseCharacter_C"))
  (set `self.Player` _returnvalue)
  (`self.SetUpgrade`)
  (bind _returnvalue_2 (`GameplayStatics.CreateSound2D` "/Game/Audio/UpgradeAquired.UpgradeAquired" 1.0 1.0 0.0 null))
  (set `self.UpgradeSound` _returnvalue_2))

(event `/Game/Player/I_Interaction._Interact`
  (params (Player :type "/Game/Player/PlayerBaseCharacter Object Reference"))
  (bind _upgradesound (`self.UpgradeSound`))
  ;[1 1 1] Pickup
  (`/Engine/EditorBlueprintResources/StandardMacros.IncrementInt` (`/Game/Player/PlayerBaseGameInstance.Upgrades Picked Up` (cast `/Game/Player/PlayerBaseGameInstance` (`GameplayStatics.GetGameInstance`) :!pure true))
    (:`  `
      ;[1 1 1] Set upgrade details
      (if (not (== (`GameplayStatics.GetObjectClass` self) "/Game/Upgrades/BP_SpecialPickup.BP_SpecialPickup_C"))
        (`/Game/Player/PlayerBaseCharacter.Upgrade Acquired` (`self.Player`) (`/Game/Upgrades/C_UpgradeDetails.UpgradeData` (`self.C_UpgradeDetails`)) false))
      (`self.K2_DestroyActor`)
      (`/Engine/EditorBlueprintResources/StandardMacros.DoOnce` false
        (:`Completed`
          (`AudioComponent.SetPitchMultiplier` _upgradesound 1.0)
          (`AudioComponent.Play` _upgradesound 0.0))))))

(event `self.ReceiveTick`
  (params (DeltaSeconds :type "Float (single-precision)"))
  (bind (_returnvalue_roll _returnvalue_pitch _returnvalue_yaw) (`KismetMathLibrary.BreakRotator` (`KismetMathLibrary.FindLookAtRotation` (`self.K2_GetActorLocation`) (`self.K2_GetActorLocation` (`self.Player`)))))
  (`self.K2_SetActorRotation` (`KismetMathLibrary.MakeRotator` 0.0 0.0 _returnvalue_yaw)))

(fn `Basic Fire Attack Upgrade`
  (params (Player :type "/Game/Player/PlayerBaseCharacter Object Reference")))

(fn `Earth Armor Upgrade`
  (params (Player :type "/Game/Player/PlayerBaseCharacter Object Reference"))
  (bind _returnvalue (`AddComponent|NODE_AddC_HealthAndShield-0` :`self` Player))
  (bind _output_get (set `/Game/Combat/C_HealthAndShield.Max Shield` 200.0 _returnvalue))
  (set `/Game/Combat/C_HealthAndShield.Current Shield` _output_get _returnvalue)
  (`KismetSystemLibrary.PrintString` "More Shield")
  (return))

(fn `SetSpecial`
  (bind _asw_floating_icon (cast `/Game/Upgrades/W_FloatingIcon` (`WidgetComponent.GetUserWidgetObject` (`self.Icon`))))
  (`/Game/Upgrades/W_FloatingIcon.SetIcon` _asw_floating_icon self))

(fn `SetUpgrade`
  (`self.SetUpgradeDataFromTable`)
  (bind _asw_floating_icon (cast `/Game/Upgrades/W_FloatingIcon` (`WidgetComponent.GetUserWidgetObject` (`self.Icon`))))
  (`/Game/Upgrades/W_FloatingIcon.SetIcon` _asw_floating_icon self))

(fn `SetUpgradeDataFromTable`
  (locals (ChosenUpgrade :type String))
  (bind _c_upgradedetails (`self.C_UpgradeDetails`))
  (bind _upgrade_type (`/Game/Upgrades/C_UpgradeDetails.Upgrade Type` (`self.C_UpgradeDetails`)))
  (switch `/Game/Upgrades/E_UpgradeType` _upgrade_type
    (:`NewEnumerator0`
      (set `local.ChosenUpgrade` (`|GetEnumeratorNameAsString` (`/Game/Upgrades/C_UpgradeDetails.MeleeUpgrade` _c_upgradedetails))))
    (:`NewEnumerator1`
      (set `local.ChosenUpgrade` (`|GetEnumeratorNameAsString` (`/Game/Upgrades/C_UpgradeDetails.BallUpgrade` _c_upgradedetails))))
    (:`NewEnumerator6`
      (set `local.ChosenUpgrade` (`|GetEnumeratorNameAsString` (`/Game/Upgrades/C_UpgradeDetails.MovementUpgrade` _c_upgradedetails))))
    (:`NewEnumerator2`
      (set `local.ChosenUpgrade` (`|GetEnumeratorNameAsString` (`/Game/Upgrades/C_UpgradeDetails.DashUpgrade` _c_upgradedetails))))
    (:`NewEnumerator7`
      (set `local.ChosenUpgrade` (`|GetEnumeratorNameAsString` (`/Game/Upgrades/C_UpgradeDetails.DefenseUpgrade` _c_upgradedetails))))
    (:`NewEnumerator5`
      (set `local.ChosenUpgrade` (`|GetEnumeratorNameAsString` (`/Game/Upgrades/C_UpgradeDetails.SpecialUpgrade` _c_upgradedetails)))))
  (bind _returnvalue (`|GetDataTableRow` "/Game/Upgrades/DT_UpgradeData.DT_UpgradeData" (`KismetStringLibrary.Conv_StringToName` (`KismetStringLibrary.Concat_StrStr` (select `/Game/Upgrades/E_UpgradeType` _upgrade_type :`NewEnumerator0` "Melee" :`NewEnumerator1` "Ball" :`NewEnumerator6` "Move" :`NewEnumerator2` "Dash" :`NewEnumerator7` "Defense" :`NewEnumerator5` "Special") "_" (`local.ChosenUpgrade`))))
    (:`then`
      (bind _output_get (set `/Game/Upgrades/C_UpgradeDetails.UpgradeData` _returnvalue (`self.C_UpgradeDetails`)))
      (`TextRenderComponent.K2_SetText` (`self.TextRender`) (`KismetTextLibrary.Conv_StringToText` (`.Name_7_994D3C904FD9DD4E8EEF7C97C81A61E7` (break `/Game/Player/UpgradeComponent/UpgradeData` _output_get))))
      (return))))

(fn `UserConstructionScript`)