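; BP_StickyBomb is a bomb actor that explodes after a fixed timer or when an enemy enters its trigger zone.
; DenationZone overlaps call Detonate, which jumps into the timer's explosion chain if the actor has the Enemy tag.
; That chain spawns fire and sound, sends TakeDamageMessage to Detonate's Object, even on timeout, and destroys the bomb.
; The construction script tints the Bomb component's material black.
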(event `self.ReceiveBeginPlay`
  (`KismetSystemLibrary.K2_SetTimerDelegate` (delegate `TimerExplode`) 10.0))

(event `TimerExplode`
  (bind _returnvalue (`self.K2_GetActorLocation`))
  (`GameplayStatics.SpawnEmitterAtLocation` "/Game/M5VFXVOL2/Particles/Explosion/Fire_Exp_01.Fire_Exp_01" _returnvalue :!label _label)
  (`GameplayStatics.SpawnSoundAtLocation` "/Game/UE4_FPTemplate/FirstPerson/Audio/FirstPersonTemplateWeaponFire02.FirstPersonTemplateWeaponFire02" _returnvalue (struct) 1.0 1.0 0.0 null null)
  (message `/Game/Combat/I_Combat.TakeDamage` (stale `Detonate` Object) 30.0 null null null "NewEnumerator4")
  (`self.K2_DestroyActor`))

(event `Detonate`
  (params (Object :type "Actor Object Reference"))
  (if (`self.ActorHasTag` Object "Enemy")
    (goto _label)))

(event `self.DenationZone.OnComponentBeginOverlap`
  (params (OverlappedComponent :type "PrimitiveComponent Object Reference") (OtherActor :type "Actor Object Reference") (OtherComp :type "PrimitiveComponent Object Reference") (OtherBodyIndex :type Integer) (bFromSweep :type Boolean) (SweepResult :type "HitResult Structure (by ref)"))
  (`self.Detonate` OtherActor))

(fn `UserConstructionScript`
  (`MeshComponent.SetVectorParameterValueOnMaterials` (`self.Bomb`) "Color" (`KismetMathLibrary.Conv_LinearColorToVector` (struct :`A` 1.0))))