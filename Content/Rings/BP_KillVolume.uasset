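; Kill volume that sends the player back to the current checkpoint when they overlap it, rather than destroying them.
; On BeginPlay it caches the level's BP_CheckpointManager.
; On overlap it casts to PlayerBaseCharacter and teleports it to the location and rotation of the manager's current checkpoint box.
; A failed cast or missing manager only prints an on-screen debug message.
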(event `self.ReceiveBeginPlay`
  (bind _returnvalue (`GameplayStatics.GetActorOfClass` "/Game/Rings/BP_CheckpointManager.BP_CheckpointManager_C"))
  (set `self.MyManager` _returnvalue))

(event `self.ReceiveActorBeginOverlap`
  (params (OtherActor :type "Actor Object Reference"))
  (bind _asplayer_base_character (cast `/Game/Player/PlayerBaseCharacter` OtherActor)
    (:`then`
      (bind _mymanager (`self.MyManager`)
        (:`then`
          (bind (_returnvalue_location _returnvalue_rotation) (`KismetMathLibrary.BreakTransform` (`SceneComponent.K2_GetComponentToWorld` (`/Game/Rings/BP_MinorCheckpoint.Box` (`/Game/Rings/BP_CheckpointManager.CurrentCheckpoint` _mymanager)))))
          (`self.K2_TeleportTo` _asplayer_base_character _returnvalue_location _returnvalue_rotation))
        (:`else`
          (`KismetSystemLibrary.PrintString` "KillVolume Get" true true (struct :`R` 1.0 :`G` 0.030354 :`B` 0.070155 :`A` 1.0) 10.0))))
    (:`CastFailed`
      (`KismetSystemLibrary.PrintString` "KillVolume Cast" true true (struct :`R` 1.0 :`B` 0.056108 :`A` 1.0) 10.0))))

(fn `UserConstructionScript`)