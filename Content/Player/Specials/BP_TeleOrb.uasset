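; BP_TeleOrb is a player special projectile that teleports the player to the surface it bounces off.
; On BeginPlay it applies its Velocity variable to the projectile movement and caches the first player's character.
; Bounces off BP_ReflectorBlock are ignored, so the orb keeps travelling.
; Any other bounce moves the player to a point offset along the impact normal, plays the warp sound and overlay, then destroys the orb.
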(event `self.ReceiveBeginPlay`
  (set `MovementComponent.Velocity` (`self.Velocity`) (`self.ProjectileMovement`))
  (bind _asplayer_base_character (cast `/Game/Player/PlayerBaseCharacter` (`GameplayStatics.GetPlayerCharacter` 0)))
  (set `self.PlayerCharacter` _asplayer_base_character))

(event `self.ProjectileMovement.OnProjectileBounce`
  (params (ImpactResult :type "HitResult Structure (by ref)") (ImpactVelocity :type "Vector Structure (by ref)"))
  (bind (_bblockinghit _binitialoverlap _time _distance _location _impactpoint _normal _impactnormal _physmat _hitactor) (`GameplayStatics.BreakHitResult` ImpactResult))
  (if (not (== (`GameplayStatics.GetObjectClass` _hitactor) "/Game/MechanicBlueprints/TeleOrb/BP_ReflectorBlock.BP_ReflectorBlock_C"))
    (`|ExecutionSequence`
      (:`then_0`
        (`self.K2_SetActorLocation` (`self.PlayerCharacter`) (+ _location (* _normal 100.0)) false true)
        (`GameplayStatics.PlaySound2D` "/Game/Audio/WarpSound.WarpSound" 1.0 1.0 0.0 null null)
        (`/Game/Player/PlayerBaseCharacter.PlayWarpOverlay` (`self.PlayerCharacter`)))
      (:`then_1`
        (`self.K2_DestroyActor`)))))

(fn `UserConstructionScript`)