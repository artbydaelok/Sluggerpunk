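; BP_ConvergencePoint is a player special: a moving point that sprays baseballs in random directions for about three seconds.
; On BeginPlay it sets its projectile velocity, plays a sound and starts timers for the barrage and self-destruction.
; Each barrage tick throws a creator-owned, recolored ball, resets the throw cooldown and updates the game mode's ball count.
; Self-destruction clears the creator's ConvergenceActive flag; older homing logic remains unconnected.
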(event `self.ReceiveBeginPlay`
  (set `MovementComponent.Velocity` (`self.Velocity`) (`self.ProjectileMovement`))
  (`KismetSystemLibrary.K2_SetTimerDelegate` (delegate `Barrage`) 0.15 true)
  (`GameplayStatics.PlaySoundAtLocation` "/Game/Audio/Convergence.Convergence" (`self.K2_GetActorLocation`) (struct) 1.0 1.0 0.0 "/Game/Audio/SA_Basic3D.SA_Basic3D" null null)
  (`KismetSystemLibrary.K2_SetTimerDelegate` (delegate `Self-Destroy`) 3.15))

(event `Self-Destroy`
  (`self.K2_DestroyActor`)
  (set `/Game/Player/PlayerBaseCharacter.ConvergenceActive` false (cast `/Game/Player/PlayerBaseCharacter` (`self.Creator`) :!pure true)))

(event `Barrage`
  (bind _c_baseball (`self.C_Baseball`))
  (bind _thrownbaseball (`/Game/Player/BaseballProj/Baseball/C_Baseball.Throw Ball` _c_baseball (+ (`self.K2_GetActorLocation`) (* (`KismetMathLibrary.RandomUnitVector`) 1000.0)) (0.0 0.0 0.0) 4500.0 5.0))
  (set `/Game/Player/BaseballProj/Baseball/BP_Baseball.BallOwner` (`self.Creator`) _thrownbaseball)
  (`/Game/Player/BaseballProj/Baseball/BP_Baseball.Change Ball Color` _thrownbaseball)
  (`/Game/Player/BaseballProj/Baseball/C_Baseball.ResetCooldown` _c_baseball)
  (`/Game/Player/PlayerBaseGamemode.IncreaseBallCount` (cast `/Game/Player/PlayerBaseGamemode` (`GameplayStatics.GetGameMode`) :!pure true) _thrownbaseball))

(fn `UserConstructionScript`)