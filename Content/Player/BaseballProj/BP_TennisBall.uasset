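; Tennis ball projectile the player knocks around to damage combat actors, then gets back.
; On bounce, Serve state returns it immediately; otherwise wall hits arm a flag so the next floor hit starts the return.
; A timeline lerps it toward the player's baseball mesh with a sound.
; DamageRadius overlaps deal base damage plus a growing combo to I_Combat actors; touching the player resets the cooldown and destroys the ball.
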(event `self.ProjectileMovement.OnProjectileBounce`
  (params (ImpactResult :type "HitResult Structure (by ref)") (ImpactVelocity :type "Vector Structure (by ref)"))
  ;[1 1 1] Check if the ball has bounced on a surface with normal equal or close to (+- 0.1) to up Vector to detect for floor collisions.
  (switch `/Game/Player/BaseballProj/E_TennisBallState` (`self.BallState`)
    (:`NewEnumerator0`
      (if (== (`.Normal` (`GameplayStatics.BreakHitResult` ImpactResult)) (`KismetMathLibrary.Vector_Up`) :`ErrorTolerance` 0.1) :!label _label
        (if (`self.hasWallBounced`)
          (set `self.ReturnStartLocation` (`self.K2_GetActorLocation`) :!label _label_2)
          (`AudioComponent.Play` (`self.ReturnSound`) 0.0)
          ;;[1 1 1] If ball hits the ground after bouncing off a wall, attempt to return to the player
          (bind (_direction _alpha) (`Timeline|Timeline_0` :!via `PlayFromStart` :!label _label_3)
            (:`Update`
              (`self.K2_SetActorLocation` (`KismetMathLibrary.VLerp` (`self.ReturnStartLocation`) (`SceneComponent.K2_GetComponentLocation` (`/Game/Player/PlayerBaseCharacter.BaseballMesh` (`/Game/Player/BaseballProj/C_TennisBall.Player` (`self.C_TennisBall`)))) _alpha)))))
        (else
          ;;[1 1 1] Hit a wall
          (set `self.hasWallBounced` true))))
    (:`NewEnumerator1`
      (goto _label_2))
    (:`NewEnumerator2`
      (goto _label))))

(event `StopReturning`
  ;[1 1 1] Check if the ball has bounced on a surface with normal equal or close to (+- 0.1) to up Vector to detect for floor collisions.
  (goto _label_3 :!via `Stop`))

(event `self.DamageRadius.OnComponentBeginOverlap`
  (params (OverlappedComponent :type "PrimitiveComponent Object Reference") (OtherActor :type "Actor Object Reference") (OtherComp :type "PrimitiveComponent Object Reference") (OtherBodyIndex :type Integer) (bFromSweep :type Boolean) (SweepResult :type "HitResult Structure (by ref)"))
  (bind _player (`/Game/Player/BaseballProj/C_TennisBall.Player` (`self.C_TennisBall`)))
  (if (not (== OtherActor _player))
    (if (`KismetSystemLibrary.DoesImplementInterface` OtherActor "/Game/Combat/I_Combat.I_Combat_C")
      (switch `/Game/Player/BaseballProj/E_TennisBallState` (`self.BallState`)
        (:`NewEnumerator0`
          _)
        (:`NewEnumerator2`
          _))
      (set `self.HitActor` OtherActor)
      (message `/Game/Combat/I_Combat.TakeDamage` (`self.HitActor`) (+ (`self.BaseDamage`) (`KismetMathLibrary.Conv_IntToDouble` (`self.Combo`))) null null null "NewEnumerator4" true 1.0)
      (`/Engine/EditorBlueprintResources/StandardMacros.IncrementInt` (`self.Combo`)))
    (else
      (switch `/Game/Player/BaseballProj/E_TennisBallState` (`self.BallState`)
        (:`NewEnumerator0`
          _)
        (:`NewEnumerator2`
          _))
      (`/Game/Player/BaseballProj/C_TennisBall.ResetCooldown` (`/Game/Player/PlayerBaseCharacter.C_TennisBall` _player))
      (`self.K2_DestroyActor`))))

(fn `AddRandomVelocity`
  (params (RandomStrength :type "Float (double-precision)"))
  (bind _projectilemovement (`self.ProjectileMovement`))
  (set `MovementComponent.Velocity` (+ (`MovementComponent.Velocity` _projectilemovement) (* (`KismetMathLibrary.RandomUnitVector`) RandomStrength)) _projectilemovement))

(fn `RedirectBall`
  (params (Velocity :type "Vector Structure"))
  (set `MovementComponent.Velocity` Velocity (`self.ProjectileMovement`))
  (set `self.hasWallBounced` false))

(fn `SetState`
  (params (BallState :type "/Game/Player/BaseballProj/E_TennisBallState Enum" :default "NewEnumerator0"))
  (set `self.BallState` BallState))

(fn `UserConstructionScript`)

(fn `ZeroVelocity`
  (set `MovementComponent.Velocity` (0.0 0.0 0.0) (`self.ProjectileMovement`)))