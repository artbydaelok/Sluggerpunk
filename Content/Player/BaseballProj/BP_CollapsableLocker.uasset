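; A locker actor that topples over when it is hit by enough balls in a short span.
; OnBallHit raises a clamped hit counter, while a looping half-second timer steadily drains it.
; Reaching the hit threshold calls FallOver, which latches the fallen state, plays a pitched-down break sound and runs a timeline that pitches the actor 90 degrees from its initial rotation.
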(event `self.ReceiveBeginPlay`
  (set `self.InitialRotation` (`self.K2_GetActorRotation`))
  (`KismetSystemLibrary.K2_SetTimerDelegate` (delegate `DecreaseBallCount`) 0.5 true))

(event `FallOver`
  (bind (_initialrotation_roll _initialrotation_pitch _initialrotation_yaw) (`KismetMathLibrary.BreakRotator` (`self.InitialRotation`)))
  (if (not (`self.FallenOver`))
    (set `self.FallenOver` true)
    (`GameplayStatics.PlaySoundAtLocation` "/Game/Audio/MachineBreak.MachineBreak" (`self.K2_GetActorLocation`) (struct) 0.7 0.65 0.0 null null null)
    (bind (_direction _alpha) (`Timeline|KnockOverAnim`)
      (:`Update`
        (`self.K2_SetActorRotation` (`KismetMathLibrary.MakeRotator` _initialrotation_roll (+ _initialrotation_pitch (`KismetMathLibrary.Lerp` 0.0 90.0 _alpha)) _initialrotation_yaw))))))

(event `/Game/Player/BaseballProj/I_Baseball.OnBallHit`
  (params (Baseball :type "/Game/Player/BaseballProj/BP_Baseball Object Reference"))
  (`self.IncreaseBallCount`))

(event `DecreaseBallCount`
  (if (not (`self.FallenOver`))
    (bind _result (`/Engine/EditorBlueprintResources/StandardMacros.DecrementInt` (`self.BallCounter`))
      (:`  `
        (set `self.BallCounter` (`KismetMathLibrary.Clamp` _result 0 20))))))

(event `IncreaseBallCount`
  (if (not (`self.FallenOver`))
    (bind _result (`/Engine/EditorBlueprintResources/StandardMacros.IncrementInt` (`self.BallCounter`))
      (:`  `
        (set `self.BallCounter` (`KismetMathLibrary.Clamp` _result 0 20))
        (if (>= (`self.BallCounter`) 3)
          (`self.FallOver`))))))

(fn `UserConstructionScript`)