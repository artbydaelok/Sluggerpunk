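; BP_Baseball is an elemental baseball projectile that damages and debuffs enemies, with optional lifesteal.
; A ball state enum scales damage alongside flight time, ball count and combo hits, and drives portal and sticky-bomb spawns.
; Bounces randomize velocity or redirect to a nearby enemy, while recall homes onto the player, slowing via the ball's CustomTimeDilation inside PlayerDilationField.
; Timers run damage scaling and shrink-out lifespan, and destruction updates the gamemode's ball count.
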(event `self.ReceiveBeginPlay`
  (`self.K2_AddActorLocalRotation` (`KismetMathLibrary.RandomRotator` false))
  (if (`self.ScaleDmgOverTime`)
    (bind _returnvalue (`KismetSystemLibrary.K2_SetTimerDelegate` (delegate `DamageOverTime`) 0.1 true))
    (set `self.DamageScalingTimer` _returnvalue))
  (`self.RedirectBall` (`self.Velocity`))
  ;[1 1 1] Reference to the player and gamemode
  (bind _asplayer_base_character (cast `/Game/Player/PlayerBaseCharacter` (`GameplayStatics.GetPlayerCharacter` 0)))
  (set `self.Player` _asplayer_base_character)
  (`self.UpdateElementAndColor` (`self.ElementalType`))
  (bind _asplayer_base_gamemode (cast `/Game/Player/PlayerBaseGamemode` (`GameplayStatics.GetGameMode`)))
  (set `self.Gamemode` _asplayer_base_gamemode)
  (add `self.OnDestroyed` (delegate `UpdateBallCount`))
  ;[1 1 1] Balls Lifespan Functionality
  (bind _returnvalue_2 (`KismetSystemLibrary.K2_SetTimerDelegate` (delegate `Lifespan`) (`self.LifespanSeconds`)))
  (set `self.LifespanTimer` _returnvalue_2))

(event `UpdateBallCount` :!signature `self.OnDestroyed`
  (params (DestroyedActor :type "Actor Object Reference"))
  ;[1 1 1] Reference to the player and gamemode
  ;;[1 1 1] Updating Ball Count on game mode
  (`/Game/Player/PlayerBaseGamemode.DecreaseBallCount` (`self.Gamemode`) self))

(event `Lifespan`
  ;[1 1 1] Balls Lifespan Functionality
  (bind (_direction _alpha) (`Timeline|Shrink` :!via `PlayFromStart`)
    (:`Update`
      (`self.SetActorScale3D` (`KismetMathLibrary.Conv_DoubleToVector` _alpha)))
    (:`Finished`
      (`self.K2_DestroyActor`))))

(event `DamageOverTime`
  (bind _overtimedmgmultiplier (`self.OverTimeDmgMultiplier`))
  ;[1 1 1] Scale damage over time
  (set `self.OverTimeDmgMultiplier` (+ _overtimedmgmultiplier 0.25))
  (if (>= _overtimedmgmultiplier (`self.MaxTimeDmgMultipler`))
    (`KismetSystemLibrary.K2_ClearAndInvalidateTimerHandle` (`self.DamageScalingTimer`))))

(event `self.PawnDetection.OnComponentBeginOverlap`
  (params (OverlappedComponent :type "PrimitiveComponent Object Reference") (OtherActor :type "Actor Object Reference") (OtherComp :type "PrimitiveComponent Object Reference") (OtherBodyIndex :type Integer) (bFromSweep :type Boolean) (SweepResult :type "HitResult Structure (by ref)"))
  (bind _player (`self.Player`))
  (bind _damage (`self.Damage`))
  (bind _overlappedpawn (`self.OverlappedPawn`))
  (bind _overlappedpawn_2 (`self.OverlappedPawn`))
  (bind _elementaltype (`self.ElementalType`))
  (bind _returnvalue (* _damage 0.5))
  (bind _returnvalue_2 (select `/Game/Player/BaseballProj/E_BallState` (`self.BallState`) :`NewEnumerator0` _damage :`NewEnumerator1` _returnvalue :`NewEnumerator2` _returnvalue :`NewEnumerator3` _damage :`NewEnumerator4` _returnvalue :`NewEnumerator5` _returnvalue :`NewEnumerator7` _returnvalue :`NewEnumerator8` _returnvalue))
  (bind _output_get (set `self.OverlappedPawn` OtherActor))
  (message `/Game/Player/BaseballProj/I_Baseball.OnBallHit` _output_get self)
  ;[1 1 1] After RECALL - Destroy ball and initiate cooldown
  (`/Engine/EditorBlueprintResources/StandardMacros.IsValid` _overlappedpawn_2
    (:`Is Valid`
      (if (and (== _overlappedpawn_2 _player) (`|EnumEquality` (`self.BallState`) "NewEnumerator2"))
        (`/Game/Player/BaseballProj/C_Baseball.ResetCooldown` (`/Game/Player/PlayerBaseCharacter.C_Baseball` _player))
        (`self.K2_DestroyActor`)
        (else
          ;[1 1 1] Damage and Combo system, it adds up whenever an enemy is hit with the ball
          (`/Engine/EditorBlueprintResources/StandardMacros.IsValid` _overlappedpawn
            (:`Is Valid`
              (if (and (`self.ActorHasTag` _overlappedpawn "Enemy") (!= _overlappedpawn (`self.BallOwner`)))
                (`/Game/Player/BaseballProj/C_BallDebuffs.ApplyDebuff` (`self.GetComponentByClass` (`self.OverlappedPawn`) "/Game/Player/BaseballProj/C_BallDebuffs.C_BallDebuffs_C") _elementaltype)
                (message `/Game/Combat/I_Combat.TakeDamage` (`self.OverlappedPawn`) (+ _returnvalue_2 (* _returnvalue_2 (* (`self.OverTimeDmgMultiplier`) 0.01)) (* (`KismetMathLibrary.Conv_IntToDouble` (`/Game/Player/PlayerBaseGamemode.NumOfPlayerBalls` (`self.Gamemode`))) (`KismetMathLibrary.Conv_BoolToDouble` (`self.ScaleDmgNumOfBalls`))) (* (`KismetMathLibrary.Conv_IntToDouble` (`self.ComboCounter`)) (`KismetMathLibrary.Conv_BoolToDouble` (`self.ScaleDmgCombo`)))) null null null _elementaltype false 1.0)
                (`self.Lifesteal`)
                (`AudioComponent.Play` (`self.HitSound`) 0.0)
                (`/Engine/EditorBlueprintResources/StandardMacros.IncrementInt` (`self.ComboCounter`)
                  (:`  `
                    (if (`|EnumEquality` (`self.BallState`) "NewEnumerator8")
                      (`|SpawnActorFromClass` "/Game/StickyBombs/BP_StickyBomb.BP_StickyBomb_C" (`KismetMathLibrary.MakeTransform` (`self.K2_GetActorLocation` (`self.OverlappedPawn`))) "Undefined" "OverrideRootScale" null null))))))))))))

(event `self.PlayerDilationField.OnComponentBeginOverlap`
  (params (OverlappedComponent :type "PrimitiveComponent Object Reference") (OtherActor :type "Actor Object Reference") (OtherComp :type "PrimitiveComponent Object Reference") (OtherBodyIndex :type Integer) (bFromSweep :type Boolean) (SweepResult :type "HitResult Structure (by ref)"))
  ;[1 1 1] Start checking for the distance between player and ball once ball is inside this field
  (if (and (== OtherActor (`self.Player`)) (`|EnumEquality` (`self.BallState`) "NewEnumerator2"))
    (`self.SlowDown`)
    (`PrimitiveComponent.SetCollisionEnabled` (`self.Ball`) "QueryOnly")))

(event `RecallTimeline`
  (params (ConvergePoint :type "Vector Structure"))
  ;[1 0.7569 0.2249] CONVERGE AT POINT
  (`self.ToggleGravity` true)
  (`self.SpeedUp`)
  (bind (_direction _alpha) (`Timeline|ConvergeAtPoint` :!via `PlayFromStart` :!label _label)
    (:`Update`
      (`self.K2_SetActorLocation` (`KismetMathLibrary.VLerp` (`self.K2_GetActorLocation`) ConvergePoint _alpha) false true))
    (:`Finished`
      (`self.AddRandomVelocity` 500.0))))

(event `StopRecall`
  ;[1 0.7569 0.2249] CONVERGE AT POINT
  (goto _label :!via `Stop`))

(event `self.PlayerDilationField.OnComponentEndOverlap`
  (params (OverlappedComponent :type "PrimitiveComponent Object Reference") (OtherActor :type "Actor Object Reference") (OtherComp :type "PrimitiveComponent Object Reference") (OtherBodyIndex :type Integer))
  ;[1 1 1] Stop checking distance between ball and player when ball is out of field
  (if (and (== OtherActor (`self.Player`)) (`|EnumEquality` (`self.BallState`) "NewEnumerator2"))
    (set `ProjectileMovementComponent.ProjectileGravityScale` 1.0 (`self.ProjectileMovement`))
    (`self.SpeedUp`)
    (`PrimitiveComponent.SetCollisionEnabled` (`self.Ball`) "QueryOnly")
    (set `ProjectileMovementComponent.bIsHomingProjectile` false (`self.ProjectileMovement`))
    (set `self.BallState` "NewEnumerator0")))

(event `self.ProjectileMovement.OnProjectileBounce`
  (params (ImpactResult :type "HitResult Structure (by ref)") (ImpactVelocity :type "Vector Structure (by ref)"))
  (bind _returnvalue (`self.K2_GetActorLocation`))
  (`self.ToggleGravity` true)
  (if (`self.BounceToTarget`)
    (set `self.ClosestDistance` 1000.0)
    (bind _outactors (`GameplayStatics.GetAllActorsOfClass` "/Game/AI/Enemy/BP_Enemy.BP_Enemy_C"))
    (for _array_element _outactors
      (bind _returnvalue_2 (`KismetMathLibrary.Vector_Distance` (`self.K2_GetActorLocation`) (`self.K2_GetActorLocation` _array_element)))
      (if (< _returnvalue_2 (`self.ClosestDistance`))
        (set `self.ClosestDistance` _returnvalue_2)
        (set `self.BounceToTargetRef` _array_element)))
    (`/Engine/EditorBlueprintResources/StandardMacros.IsValid` (`self.BounceToTargetRef`)
      (:`Is Valid`
        (`self.RedirectBall` (* (`KismetMathLibrary.GetDirectionUnitVector` (`self.K2_GetActorLocation`) (`self.K2_GetActorLocation` (`self.BounceToTargetRef`))) (`self.BounceToTargetStrength`))))
      (:`Is Not Valid`
        _))
    (set `self.BounceToTarget` false)
    (else
      (`self.AddRandomVelocity` 200.0)))
  (switch `/Game/Player/BaseballProj/E_BallState` (`self.BallState`)
    (:`NewEnumerator0`
      ;[1 0.3395 0.7573] On every bounce -> spawn particles and set boolean for slowing down
      (set `self.BallState` "NewEnumerator4" :!label _label_2)
      (`/Engine/EditorBlueprintResources/StandardMacros.IncrementInt` (`self.BounceTimes`)
        (:`  `
          (set `self.CanSlowDown` true)
          (`ActorComponent.Activate` (`self.NS_Burst`) true))))
    (:`NewEnumerator1`
      (goto _label_2))
    (:`NewEnumerator2`
      (set `ProjectileMovementComponent.bIsHomingProjectile` false (`self.ProjectileMovement`))
      (goto _label_2))
    (:`NewEnumerator3`
      (goto _label_2))
    (:`NewEnumerator4`
      (goto _label_2))
    (:`NewEnumerator5`
      (goto _label_2))
    (:`NewEnumerator7`
      ;[1 1 1] PortalBall
      (`ActorComponent.Activate` (`self.PortalBallVFX`) false)
      (`ActorComponent.Deactivate` (`self.Trail`))
      (bind _outhit (`KismetSystemLibrary.LineTraceSingle` :`Start` _returnvalue :`End` (+ _returnvalue (* (`.Normal` (`GameplayStatics.BreakHitResult` ImpactResult)) 100000.0)) :`TraceChannel` "TraceTypeQuery1" :`DrawTime` 3.0))
      (`SceneComponent.SetVisibility` (`self.Ball`) false false)
      ;;[0.5104 0 0.004513] Spawn Portal and make it throw a new ball
      (bind _returnvalue_3 (`KismetSystemLibrary.K2_SetTimerDelegate` (delegate `Portal Spawn`) 0.1))
      (set `self.Portal Timer` _returnvalue_3))))

(event `Portal Spawn`
  ;[1 1 1] PortalBall
  ;;[0.5104 0 0.004513] Spawn Portal and make it throw a new ball
  (bind (_bblockinghit _binitialoverlap _time _distance _location _impactpoint _normal) (`GameplayStatics.BreakHitResult` (stale `self.ProjectileMovement.OnProjectileBounce` _outhit)))
  (bind _returnvalue (`|SpawnActorFromClass` "/Game/Player/Specials/BP_BallPortal.BP_BallPortal_C" (`KismetMathLibrary.MakeTransform` (+ _location (* _normal 50.0))) "Undefined" "OverrideRootScale" null null))
  (bind _thrownbaseball (`/Game/Player/BaseballProj/C_Baseball.Throw Ball` (`/Game/Player/Specials/BP_BallPortal.C_Baseball` _returnvalue) (+ (+ _location (* _normal 10000.0)) (* (`KismetMathLibrary.RandomUnitVector`) 25.0)) (0.0 0.0 0.0) (`KismetMathLibrary.VSize` (`MovementComponent.Velocity` (`self.ProjectileMovement`))) (`KismetSystemLibrary.K2_GetTimerRemainingTimeHandle` (`self.LifespanTimer`))))
  (set `/Game/Player/BaseballProj/BP_Baseball.BallState` "NewEnumerator7" _thrownbaseball)
  (`self.AddRandomVelocity` _thrownbaseball 1500.0)
  (set `/Game/Player/BaseballProj/BP_Baseball.BallOwner` (`self.Player`) _thrownbaseball)
  (`/Game/Player/PlayerBaseGamemode.IncreaseBallCount` (`self.Gamemode`) _thrownbaseball)
  (`self.Change Ball Color` _thrownbaseball)
  (`self.K2_DestroyActor`))

(event `DisablePortal`
  ;[1 1 1] PortalBall
  ;;[0.5104 0 0.004513] Spawn Portal and make it throw a new ball
  (`KismetSystemLibrary.K2_ClearAndInvalidateTimerHandle` (`self.Portal Timer`))
  (`SceneComponent.SetVisibility` (`self.Ball`) true false))

(event `SlowDown`
  ;[1 1 1] Slowing down and speeding up
  (`/Game/Player/PlayerBaseCharacter.BallDilationSound` (`self.Player`))
  (set `self.CustomTimeDilation` 0.075))

(event `SpeedUp`
  ;[1 1 1] Slowing down and speeding up
  (set `self.CustomTimeDilation` 1.0))

(event `Freeze`
  (`ActorComponent.Activate` (`self.FreezeVFX`) true)
  (for _array_element (`PrimitiveComponent.GetOverlappingActors` (`self.FreezeArea`) "/Game/AI/Enemy/BP_Enemy.BP_Enemy_C")
    (`/Game/Player/BaseballProj/C_BallDebuffs.ApplyDebuff` (`self.GetComponentByClass` _array_element "/Game/Player/BaseballProj/C_BallDebuffs.C_BallDebuffs_C") "NewEnumerator1")))

(event `self.PawnDetection.OnComponentEndOverlap`
  (params (OverlappedComponent :type "PrimitiveComponent Object Reference") (OtherActor :type "Actor Object Reference") (OtherComp :type "PrimitiveComponent Object Reference") (OtherBodyIndex :type Integer)))

(fn `AddRandomVelocity`
  (params (RandomVelocity :type "Float (double-precision)" :default 200.0))
  (bind _projectilemovement (`self.ProjectileMovement`))
  (set `MovementComponent.Velocity` (+ (* (`KismetMathLibrary.RandomUnitVector`) RandomVelocity) (`MovementComponent.Velocity` _projectilemovement)) _projectilemovement)
  (return))

(fn `Change Ball Color`
  (bind _ball (`self.Ball`))
  (bind _elementaltype (`self.ElementalType`))
  (bind _ball_2 (`self.Ball`))
  (bind _trail (`self.Trail`))
  (if (== (`self.BallOwner`) (`self.Player`))
    (`MeshComponent.SetVectorParameterValueOnMaterials` _ball_2 "ColorTint" (1.0 1.0 1.0))
    (`PrimitiveComponent.SetCustomDepthStencilValue` _ball (select `/Game/Combat/E_Element` _elementaltype :`NewEnumerator4` 1 :`NewEnumerator2` 5 :`NewEnumerator3` 4 :`NewEnumerator0` 3 :`NewEnumerator1` 6))
    (`FXSystemComponent.SetColorParameter` _trail "TrailColor" (select `/Game/Combat/E_Element` _elementaltype :`NewEnumerator4` (struct :`R` 1.0 :`G` 0.798821 :`B` 0.870073 :`A` 1.0) :`NewEnumerator2` (struct :`R` 1.0 :`G` 0.984802 :`B` 0.797745 :`A` 1.0) :`NewEnumerator3` (struct :`G` 0.875 :`B` 0.041946 :`A` 1.0) :`NewEnumerator0` (struct :`R` 1.0 :`G` 0.473542 :`B` 0.007351 :`A` 1.0) :`NewEnumerator1` (struct :`R` 0.094229 :`G` 0.541095 :`B` 1.0 :`A` 1.0) :!type "LinearColor Structure"))
    (else
      (`MeshComponent.SetVectorParameterValueOnMaterials` _ball_2 "ColorTint" (0.8 0.1 0.1))
      (`PrimitiveComponent.SetCustomDepthStencilValue` _ball 2)
      (`FXSystemComponent.SetColorParameter` _trail "TrailColor" (struct :`R` 1.0 :`G` 0.008526 :`A` 1.0)))))

(fn `ClearHoming`
  (bind _projectilemovement (`self.ProjectileMovement`))
  (set `ProjectileMovementComponent.HomingTargetComponent` null _projectilemovement)
  (set `ProjectileMovementComponent.bIsHomingProjectile` false _projectilemovement))

(fn `Lifesteal`
  (if (`KismetMathLibrary.RandomBoolWithWeight` (`self.LifestealChance`))
    (bind _asplayer_base_character (cast `/Game/Player/PlayerBaseCharacter` (`self.BallOwner`)))
    (`/Game/Player/PlayerBaseCharacter.Heal/Take Damage` _asplayer_base_character (`self.LifestealAmount`))))

(fn `OnBallHit`
  (params (Baseball :type "/Game/Player/BaseballProj/BP_Baseball Object Reference"))
  (return))

(fn `RecallBall`
  (params (RandomizePosition :type Boolean))
  (locals (Speed :type "Float (double-precision)" :default 0.0))
  (bind _projectilemovement (`self.ProjectileMovement`))
  (set `local.Speed` (`KismetMathLibrary.VSize` (`self.Velocity`)))
  ;[1 1 1] Set Ball State to returning
  (`self.SpeedUp`)
  (if (== (`self.BallOwner`) (`self.Player`))
    (set `self.BallState` "NewEnumerator2")
    ;[1 1 1] Lock On Player
    (`self.ToggleGravity` false)
    (`PrimitiveComponent.SetCollisionEnabled` (`self.Ball`) "NoCollision")
    (set `MovementComponent.Velocity` (* (`KismetMathLibrary.GetDirectionUnitVector` (`self.K2_GetActorLocation`) (`self.K2_GetActorLocation` (`self.Player`))) (`local.Speed`)) _projectilemovement)
    (if (`local.RandomizePosition`)
      (`self.AddRandomVelocity` 500.0))
    (set `ProjectileMovementComponent.HomingTargetComponent` (`|GetArrayItem` (`self.GetComponentsByTag` (`self.Player`) "/Script/Engine.SceneComponent" "HomingTarget")) _projectilemovement)
    (set `ProjectileMovementComponent.bIsHomingProjectile` true _projectilemovement)
    (set `ProjectileMovementComponent.HomingAccelerationMagnitude` 20000.0 _projectilemovement)))

(fn `RedirectBall`
  (params (`New Velocity` :type "Vector Structure") (WasHit :type Boolean))
  (set `self.WasHit` WasHit)
  (set `MovementComponent.Velocity` `New Velocity` (`self.ProjectileMovement`)))

(fn `ResetBounces`
  (set `self.BounceTimes` 0))

(fn `ToggleGravity`
  (params (HasGravity :type Boolean))
  (bind _projectilemovement (`self.ProjectileMovement`))
  (if HasGravity
    (set `ProjectileMovementComponent.ProjectileGravityScale` 1.0 _projectilemovement)
    (else
      (set `ProjectileMovementComponent.ProjectileGravityScale` 0.0 _projectilemovement))))

(fn `UpdateElementAndColor`
  (params (ElementType :type "/Game/Combat/E_Element Enum" :default "NewEnumerator4"))
  (set `self.ElementalType` ElementType)
  (`self.Change Ball Color`))

(fn `UserConstructionScript`)