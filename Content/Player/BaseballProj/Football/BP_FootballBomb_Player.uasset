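; BP_FootballBomb_Player is the player's football bomb projectile, which explodes on impact.
; At BeginPlay it applies its Velocity variable to the projectile component.
; On hit it spawns and triggers a BP_Explosion owned by the struck actor, then destroys itself.
; Both a hit and a DashPickUp event set the player's CFootball state to its first enum value, with pickup destroying the ball without exploding.
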(event `self.ReceiveBeginPlay`
  (set `MovementComponent.Velocity` (`self.Velocity`) (`self.Projectile`)))

(event `self.ReceiveHit`
  (params (MyComp :type "PrimitiveComponent Object Reference") (Other :type "Actor Object Reference") (OtherComp :type "PrimitiveComponent Object Reference") (bSelfMoved :type Boolean) (HitLocation :type "Vector Structure") (HitNormal :type "Vector Structure") (NormalImpulse :type "Vector Structure") (Hit :type "HitResult Structure (by ref)"))
  (bind _returnvalue (`|SpawnActorFromClass` "/Game/AI/ExplosionMechanic/BP_Explosion.BP_Explosion_C" (`KismetMathLibrary.MakeTransform` (`self.K2_GetActorLocation`)) "Undefined" "OverrideRootScale" Other null))
  (`/Game/AI/ExplosionMechanic/BP_Explosion.Explode` _returnvalue)
  (set `/Game/Player/BaseballProj/Football/C_Football.FootballState` "NewEnumerator0" (`/Game/Player/PlayerBaseCharacter.C_Football` (`self.Player`)))
  (`self.K2_DestroyActor`))

(event `DashPickUp`
  (set `/Game/Player/BaseballProj/Football/C_Football.FootballState` "NewEnumerator0" (`/Game/Player/PlayerBaseCharacter.C_Football` (`self.Player`)))
  (`self.K2_DestroyActor`))

(fn `UserConstructionScript`
  (`parent.UserConstructionScript`))