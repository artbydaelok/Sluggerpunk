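; Gold collectible that spins and adds gold to the player when touched.
; When not flagged as a pickup, it waits a short random time, then flies to the player along timeline-driven lerps with a height offset.
; On overlap, it picks an amount by enemy type (random with multipliers, or GoldValue by default), credits player and GameInstance totals, updates the HUD, plays a pitch-varied sound, scales the mesh, then destroys itself after delays.
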(event `self.ReceiveBeginPlay`
  (bind _asplayer_base_character (cast `/Game/Player/PlayerBaseCharacter` (`GameplayStatics.GetPlayerCharacter` 0)))
  (set `self.PlayerCharacter` _asplayer_base_character)
  (set `self.StartLocation` (`self.K2_GetActorLocation`))
  (set `self.StartScale` (`SceneComponent.RelativeScale3D` (`self.StaticMesh`)))
  (if (`self.isPickup?`)
    (bind (_direction _like_a_record) (`Timeline|You Spin Me Right 'Round` :!via `PlayFromStart` :!label _label)
      (:`Update`
        (`SceneComponent.K2_SetRelativeRotation` (`self.StaticMesh`) (`KismetMathLibrary.RLerp` (struct) (struct :`Yaw` 360.0) _like_a_record) false false)))
    (else
      (`KismetSystemLibrary.K2_SetTimerDelegate` (delegate `FlyToPlayer`) (`KismetMathLibrary.RandomFloatInRange` 1.0 1.5))
      (goto _label :!via `PlayFromStart`))))

(event `FlyToPlayer`
  (bind (_direction _x_y_alpha _z_alpha) (`Timeline|LocationUpdate` :!via `PlayFromStart`)
    (:`Update`
      (bind (_returnvalue_x _returnvalue_y _returnvalue_z) (`KismetMathLibrary.BreakVector` (`KismetMathLibrary.VLerp` (`self.StartLocation`) (`self.K2_GetActorLocation` (`self.PlayerCharacter`)) _x_y_alpha)))
      (`self.K2_SetActorLocation` (`KismetMathLibrary.MakeVector` _returnvalue_x _returnvalue_y (+ _returnvalue_z (`KismetMathLibrary.Lerp` 0.0 200.0 _z_alpha)))))))

(event `self.ReceiveActorBeginOverlap`
  (params (OtherActor :type "Actor Object Reference"))
  (bind _returnvalue (`KismetMathLibrary.RandomIntegerInRange` 7 10))
  (bind _playercharacter (`self.PlayerCharacter`))
  (bind _returnvalue_2 (* _returnvalue 3))
  (bind _returnvalue_3 (* _returnvalue 5))
  (bind _asplayer_base_game_instance (cast `/Game/Player/PlayerBaseGameInstance` (`GameplayStatics.GetGameInstance`) :!pure true))
  (bind _w_hud (`/Game/Player/PlayerBaseCharacter.W_HUD` _playercharacter))
  (if (== OtherActor _playercharacter)
    (bind _output_get (set `self.GoldEarned` (select `/Game/AI/Enemy/E_EnemyTypes` (`self.EnemyType`) :`NewEnumerator5` (`self.GoldValue`) :`NewEnumerator0` _returnvalue :`NewEnumerator3` _returnvalue :`NewEnumerator7` _returnvalue_2 :`NewEnumerator8` _returnvalue_2 :`NewEnumerator1` (* _returnvalue 2) :`NewEnumerator9` _returnvalue_3 :`NewEnumerator2` _returnvalue_3)))
    (set `/Game/Player/PlayerBaseCharacter.CurrentGold` (+ (`/Game/Player/PlayerBaseCharacter.CurrentGold` _playercharacter) _output_get) _playercharacter)
    (set `/Game/Player/PlayerWidgets/W_PlayerHUD.GoldEarned` (`self.GoldEarned`) _w_hud)
    (set `/Game/Player/PlayerBaseGameInstance.Total Gold` (+ (`/Game/Player/PlayerBaseGameInstance.Total Gold` _asplayer_base_game_instance) (`self.GoldEarned`)) _asplayer_base_game_instance)
    (`/Game/Player/PlayerWidgets/W_PlayerHUD.PlayEarnedAnimation` _w_hud)
    (`PrimitiveComponent.SetCollisionEnabled` (`self.Sphere`) "NoCollision")
    (`GameplayStatics.PlaySound2D` "/Game/Audio/CoinPickupSFX.CoinPickupSFX" 1.0 (`KismetMathLibrary.RandomFloatInRange` 0.8 1.2) 0.0 null null)
    (bind (_direction _shut_up_and_take_my_money) (`Timeline|Ka-Ching ka-Ching`)
      (:`Update`
        (`SceneComponent.SetRelativeScale3D` (`self.StaticMesh`) (`KismetMathLibrary.VLerp` (0.0 0.0 0.0) (`self.StartScale`) _shut_up_and_take_my_money)))
      (:`Finished`
        (`KismetSystemLibrary.Delay` 0.2)
        (set `/Game/Player/PlayerWidgets/W_PlayerHUD.FlashGold` false _w_hud)
        (`KismetSystemLibrary.Delay` 5.0)
        (`/Game/Player/PlayerWidgets/W_PlayerHUD.ToggleEarnedVisible` _w_hud "Hidden")
        (`self.K2_DestroyActor`)))))

(fn `UserConstructionScript`)