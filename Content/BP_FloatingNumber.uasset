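; Actor that shows a floating damage number through a widget component and removes itself once the animation finishes.
; Its Initialize event stores the text, which BeginPlay passes to the W_FloatingDamageNumber widget, so it only reaches the widget if set before BeginPlay.
; BeginPlay also binds to the widget's animation-finished event, with HandleAnimFinished destroying the actor.
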(event `self.ReceiveBeginPlay`
  (bind _asw_floating_damage_number (cast `/Game/FloatingDamageNumbers/W_FloatingDamageNumber` (`WidgetComponent.GetUserWidgetObject` (`self.Widget`))))
  (add `/Game/FloatingDamageNumbers/W_FloatingDamageNumber.OnDamageNumberAnimFinished` _asw_floating_damage_number (`|CreateDelegate` :!event `HandleAnimFinished`))
  (`/Game/FloatingDamageNumbers/W_FloatingDamageNumber.Initialize` _asw_floating_damage_number (`self.Text`)))

(event `self.Initialize`
  (params (text :type "Text (by ref)"))
  (set `self.Text` text))

(fn `HandleAnimFinished`
  (`self.K2_DestroyActor`))

(fn `UserConstructionScript`)