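; Spline-driven wire prop Blueprint that builds a wire mesh along an editable spline.
; The construction script adds a forward-X spline mesh with query and physics collision for each segment between consecutive points, matching their positions and tangents.
; It then adds static meshes as end pieces at the first point and at the final loop index, oriented along the spline tangent.
; The event graph holds no active logic.
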(fn `UserConstructionScript`
  (bind _spline (`self.Spline`))
  (bind _spline_2 (`self.Spline`))
  (bind (_location _tangent) (`SplineComponent.GetLocationAndTangentAtSplinePoint` (`self.Spline`) 0 "Local"))
  (for _index (range (+ (- (`SplineComponent.GetNumberOfSplinePoints` (`self.Spline`)) 2) 1))
    (bind _returnvalue (`AddComponent|NODE_AddSplineMeshComponent-0`))
    (`SplineMeshComponent.SetForwardAxis` _returnvalue "X" true)
    (`PrimitiveComponent.SetCollisionEnabled` _returnvalue "QueryAndPhysics")
    (bind _returnvalue_2 (`SplineComponent.GetLocationAtSplinePoint` _spline _index "Local"))
    (bind _returnvalue_3 (`SplineComponent.GetTangentAtSplinePoint` _spline _index "Local"))
    (bind _returnvalue_4 (+ _index 1))
    (`SplineMeshComponent.SetStartAndEnd` _returnvalue _returnvalue_2 _returnvalue_3 (`SplineComponent.GetLocationAtSplinePoint` _spline_2 _returnvalue_4 "Local") (`SplineComponent.GetTangentAtSplinePoint` _spline_2 _returnvalue_4 "Local") true))
  (bind _returnvalue_5 (`AddComponent|NODE_AddStaticMeshComponent-0`))
  (`SceneComponent.K2_SetRelativeLocationAndRotation` _returnvalue_5 _location (`KismetMathLibrary.Conv_VectorToRotator` _tangent) false false)
  (bind _returnvalue_6 (`AddComponent|NODE_AddStaticMeshComponent-1`))
  (`SceneComponent.K2_SetRelativeLocationAndRotation` _returnvalue_6 _returnvalue_2 (`KismetMathLibrary.Conv_VectorToRotator` _returnvalue_3) false false))