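; BP_CustomNavLink is a smart nav link that lets one enemy at a time use it to climb up or down.
; When an agent reaches it, a DoOnce gate disables the link, sets its nav modifier to a null area, stores the agent and calls ClimbUpDown on BP_Enemy.
; A Reset event clears the current pawn, restores the link and default area, and reopens the gate.
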(event `Reset`
  ;[1 1 1] Only 1 enemy can use the Nav Link at a time
  ;;[1 1 1] Reactivate Nav Link
  (set `self.Current Pawn` (`self.Null Pawn`))
  (`self.SetSmartLinkEnabled` true)
  (`NavModifierComponent.SetAreaClass` (`self.NavModifier`) "/Script/NavigationSystem.NavArea_Default")
  (goto _label :!via `Reset`))

(event `self.ReceiveSmartLinkReached`
  (params (Agent :type "Actor Object Reference") (Destination :type "Vector Structure (by ref)"))
  ;[1 1 1] Only 1 enemy can use the Nav Link at a time
  (set `self.Destination` Destination)
  (if (`self.IsSmartLinkEnabled`)
    (if (not (== Agent (`self.Current Pawn`)))
      ;;[1 1 1] Turn Off Nav Link
      (`/Engine/EditorBlueprintResources/StandardMacros.DoOnce` false :!label _label
        (:`Completed`
          (`self.SetSmartLinkEnabled` false)
          (`NavModifierComponent.SetAreaClass` (`self.NavModifier`) "/Script/NavigationSystem.NavArea_Null")
          (bind _output_get (set `self.Current Pawn` Agent))
          (bind _asbp_enemy (cast `/Game/AI/Enemy/BP_Enemy` _output_get))
          (bind _output_get_2 (set `self.Current Agent` _asbp_enemy))
          (`/Game/AI/Enemy/BP_Enemy.Climb Up/Down` _output_get_2 self))))))

(fn `UserConstructionScript`)