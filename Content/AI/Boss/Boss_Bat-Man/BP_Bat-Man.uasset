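; Bat-Man boss that makes a melee attack and enters a frantic special at health thresholds.
; Attacks play a montage, then capsule-trace forward to damage and debuff the player with the boss's element.
; Damage taken while vulnerable consumes crossed SpecialPoints and triggers the behavior tree special.
; The once-gated special spawns an attack-line actor and writes its target to the blackboard; the exhaustion and reset chain is unconnected.
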(event `self.ReceiveBeginPlay`
  (`parent.ReceiveBeginPlay`))

(event `Play Attack Animation`
  (bind _ac_bossstats (`self.AC_BossStats`))
  (bind _capsulecomponent (`self.CapsuleComponent`))
  (bind _returnvalue (`SceneComponent.K2_GetComponentLocation` _capsulecomponent))
  (bind _boss_element (`/Game/AI/Boss/C_BossStats.Boss Element` _ac_bossstats))
  ;[1 1 1] Attack
  (`SkeletalMeshComponent.PlayAnimation` (`self.Mesh`) "/Game/3DModels/ArtistStuff/Version2/Bat_man/AM_BatManAttack.AM_BatManAttack" false)
  (`KismetSystemLibrary.Delay` 0.5)
  (bind _outhit (`KismetSystemLibrary.CapsuleTraceSingle` :`Start` _returnvalue :`End` (+ _returnvalue (* (`SceneComponent.GetForwardVector` _capsulecomponent) (`/Game/AI/Boss/C_BossStats.Attack Range` (`self.AC_BossStats`)))) :`Radius` 100.0 :`TraceChannel` "TraceTypeQuery3" :`DrawDebugType` "ForDuration"))
  (bind (_bblockinghit _binitialoverlap _time _distance _location _impactpoint _normal _impactnormal _physmat _hitactor) (`GameplayStatics.BreakHitResult` _outhit))
  (if (== _hitactor (`GameplayStatics.GetPlayerCharacter` 0))
    (message `/Game/Combat/I_Combat.TakeDamage` _hitactor (`/Game/AI/Boss/C_BossStats.Damage` _ac_bossstats) null null self _boss_element true 1.0)
    (message `/Game/Combat/I_Combat.ApplyDebuff` _hitactor 0.0 null null self _boss_element)))

(event `Special Mechanic`
  (`/Engine/EditorBlueprintResources/StandardMacros.DoOnce` false :!label _label
    (:`Completed`
      (set `self.Frantic?` true)
      (`self.Frantic Attack`))))

(event `Reset Special Mechanic`
  (goto _label :!via `Reset`))

(event `Frantic Attack`
  (`self.Spawn Attack Path`))

(event `Spawn Attack Path`
  (bind (_returnvalue_x _returnvalue_y _returnvalue_z) (`KismetMathLibrary.BreakVector` (`self.K2_GetActorLocation`)))
  (bind _returnvalue (`|SpawnActorFromClass` "/Game/AI/Boss/Boss_Bat-Man/BP_FranticAttackLine.BP_FranticAttackLine_C" (`KismetMathLibrary.MakeTransform` (`KismetMathLibrary.MakeVector` _returnvalue_x _returnvalue_y (- _returnvalue_z 130.0)) (`KismetMathLibrary.Conv_VectorToRotator` (`KismetMathLibrary.GetForwardVector` (`self.K2_GetActorRotation`)))) "AlwaysSpawn" "OverrideRootScale" null null))
  (`BlackboardComponent.SetValueAsVector` (`AIBlueprintHelperLibrary.GetBlackboard` self) (`self.TargetLocation`) (`SceneComponent.K2_GetComponentLocation` (`/Game/AI/Boss/Boss_Bat-Man/BP_FranticAttackLine.Target` _returnvalue))))

(fn `Boss Take Damage`
  (params (Damage :type "Float (double-precision)") (Element :type "/Game/Combat/E_Element Enum" :default "NewEnumerator4") (IgnoreShield :type Boolean))
  (if (not (`self.Invulnerable`))
    (`parent.Boss Take Damage` Damage Element IgnoreShield)
    (`/Engine/EditorBlueprintResources/StandardMacros.IsValid` self
      (:`Is Valid`
        (`self.Check To See If Do Special`)))))

(fn `Check for target point`
  (`/Engine/EditorBlueprintResources/StandardMacros.IsValid` (`self.Target Points`)
    (:`Is Valid`
      (set `self.Frantic?` true))
    (:`Is Not Valid`
      (`KismetSystemLibrary.PrintString` "Point does not exist")
      (`self.Spawn Attack Path`))))

(fn `Check To See If Do Special`
  (locals (WorkingIndex :type Integer))
  (bind _ac_healthandshield (`self.AC_HealthAndShield`))
  (bind _specialpoints (`/Game/AI/Boss/C_BossStats.SpecialPoints` (`self.AC_BossStats`)))
  (if (not (<= (`KismetArrayLibrary.Array_Length` (`/Game/AI/Boss/C_BossStats.SpecialPoints` (`self.AC_BossStats`))) 0))
    (for (_array_element _array_index) (`/Game/AI/Boss/C_BossStats.SpecialPoints` (`self.AC_BossStats`))
      (if (<= (/ (`/Game/Combat/C_HealthAndShield.Current Health` _ac_healthandshield) (`/Game/Combat/C_HealthAndShield.Max Health` _ac_healthandshield)) _array_element)
        (set `local.WorkingIndex` _array_index)
        (break)
        (else
          (set `local.WorkingIndex` -1))))
    (if (>= (`local.WorkingIndex`) 0)
      (`KismetArrayLibrary.Array_Remove` _specialpoints (`local.WorkingIndex`))
      (`KismetSystemLibrary.PrintString` (`KismetStringLibrary.Conv_IntToString` (`KismetArrayLibrary.Array_Length` _specialpoints)))
      (`self.Execute Special On BT`))))

(fn `Do Special Mechanic`
  (`self.Special Mechanic`))

(fn `EnemyAttack`
  (returns (AttackDuration :type "Float (double-precision)"))
  (`self.Play Attack Animation`)
  (return (`/Game/AI/Boss/C_BossStats.Attack Duration` (`self.AC_BossStats`))))

(fn `UserConstructionScript`)