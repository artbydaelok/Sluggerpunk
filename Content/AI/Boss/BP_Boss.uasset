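; Base boss enemy that takes elemental damage and spawns rewards on death, with empty or stub special and attack functions.
; Incoming damage passes through base and per-element reductions from ACBossStats, is applied negated to the health/shield component, and shows as a damage number.
; Death spawns gold and a health fountain, resets the player's fountain values, increments the kill count and destroys the boss; upgrade-drop logic is unconnected.
; Helpers toggle the behavior tree's special-attack blackboard flag.
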(event `self.ReceiveBeginPlay`
  (bind _returnvalue (`GameplayStatics.GetActorOfClass` "/Game/Player/PlayerBaseCharacter.PlayerBaseCharacter_C"))
  (set `self.Player` _returnvalue)
  (set `self.BossState` "NewEnumerator0")
  (set `self.EnemyType` "NewEnumerator2"))

(event `/Game/Combat/I_Combat.TakeDamage`
  (params (Damage :type "Float (single-precision)") (Player :type "/Game/Player/PlayerBaseCharacter Object Reference") (Enemy :type "/Game/AI/Enemy/BP_Enemy Object Reference") (Boss :type "/Game/AI/Boss/BP_Boss Object Reference") (Element :type "/Game/Combat/E_Element Enum" :default "NewEnumerator4") (DealsKnockback :type Boolean) (`KB Multiplier` :type "Float (single-precision)"))
  ;[1 1 1] Boss takes damage
  (`self.Boss Take Damage` Damage Element))

(event `/Game/Combat/I_Combat.On Death`
  (`self.Boss Death`))

(fn `Boss Death`
  (bind _player (`self.Player`))
  (bind _fountainanchor (`self.FountainAnchor`))
  (`|SpawnActorFromClass` "/Game/Collectibles/BP_Gold.BP_Gold_C" (`KismetMathLibrary.MakeTransform` (`SceneComponent.K2_GetComponentLocation` (`self.GoldSpawnAnchor`))) "Undefined" "OverrideRootScale" null 5 (`self.EnemyType`) false null)
  (`|SpawnActorFromClass` "/Game/MechanicBlueprints/BP_HealthFountain.BP_HealthFountain_C" (`KismetMathLibrary.MakeTransform` (`SceneComponent.K2_GetComponentLocation` _fountainanchor) (`SceneComponent.K2_GetComponentRotation` _fountainanchor)) "Undefined" "OverrideRootScale" null null)
  (set `/Game/Player/PlayerBaseCharacter.CurrentCostHealthFountain` 50 _player)
  (set `/Game/Player/PlayerBaseCharacter.CurrentHealingHealthFountain` 50.0 _player)
  (`/Engine/EditorBlueprintResources/StandardMacros.IncrementInt` (`/Game/Player/PlayerBaseGameInstance.Enemies Killed` (cast `/Game/Player/PlayerBaseGameInstance` (`GameplayStatics.GetGameInstance`) :!pure true))
    (:`  `
      (`self.K2_DestroyActor`))))

(fn `Boss Take Damage`
  (params (Damage :type "Float (double-precision)") (Element :type "/Game/Combat/E_Element Enum" :default "NewEnumerator4") (IgnoreShield :type Boolean))
  (bind _damage (`self.Calculate Damage After Reduction` Damage Element))
  (`/Game/Combat/C_HealthAndShield.Heal/Take Damage` (`self.AC_HealthAndShield`) _damage IgnoreShield)
  (`/Game/Player/PlayerBaseCharacter.SpawnDamageNumber` (`self.Player`) (`KismetTextLibrary.Conv_DoubleToText` (`KismetMathLibrary.Abs` _damage) "HalfToEven" false true 1 324 0 0) (`self.K2_GetActorLocation`)))

(fn `Calculate Damage After Reduction`
  (params (`Initial Damage` :type "Float (double-precision)") (`Damage Element` :type "/Game/Combat/E_Element Enum (by ref)"))
  (returns (Damage :type "Float (double-precision)"))
  (locals (`After Base Reduction` :type "Float (double-precision)" :default 0.0) (`Damage Out` :type "Float (double-precision)" :default 0.0))
  (bind _after_base_reduction (`local.After Base Reduction`))
  (bind (_value _returnvalue) (`BlueprintMapLibrary.Map_Find` (`/Game/AI/Boss/C_BossStats.Elemental Damage Reduction (Percent)` (`self.AC_BossStats`)) `Damage Element`))
  (set `local.After Base Reduction` (- `Initial Damage` (* `Initial Damage` (`/Game/AI/Boss/C_BossStats.Base Damage Reduction (Percent)` (`self.AC_BossStats`)))))
  (if _returnvalue
    (set `local.Damage Out` (- _after_base_reduction (* _after_base_reduction _value)))
    (else
      (set `local.Damage Out` (`local.After Base Reduction`))))
  (set `local.Damage Out` (- 0.0 (`local.Damage Out`)))
  (return (`local.Damage Out`)))

(fn `Check To See If Do Special`)

(fn `Do Special Mechanic`)

(fn `EnemyAttack`
  (returns (AttackDuration :type "Float (double-precision)"))
  (return 0.0))

(fn `EnemyShockwave`
  (returns (`Attack Duration` :type "Float (double-precision)"))
  (return 0.0))

(fn `Execute Special On BT`
  (`BlackboardComponent.SetValueAsBool` (`AIBlueprintHelperLibrary.GetBlackboard` self) "DoSpecial?" true))

(fn `Reset Special On BT`
  (`BlackboardComponent.SetValueAsBool` (`AIBlueprintHelperLibrary.GetBlackboard` self) "DoSpecial?" false))

(fn `UserConstructionScript`)