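; Summoner boss character that fights with a forward melee trace and a knockback shockwave, and summons melee minions.
; Damage that drops health past a SpecialPoints threshold signals the behavior tree to run the special mechanic.
; The special moves it toward SpecialLocation, makes it invulnerable with a swapped material, and spawns escalating regular and elite waves in spawn boxes.
; A looping timer ends the phase once all summons are gone.
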(event `self.ReceiveBeginPlay`
  (`parent.ReceiveBeginPlay`)
  (set `self.EnemyType` "NewEnumerator2")
  (bind _returnvalue (`GameplayStatics.GetActorOfClass` "/Game/AI/Boss/SpecialLocation.SpecialLocation_C"))
  (bind _output_get (set `self.SpecialLocation` _returnvalue))
  (`/Engine/EditorBlueprintResources/StandardMacros.IsValid` _output_get
    (:`Is Valid`
      (`KismetSystemLibrary.PrintString` "Special Location Found"))
    (:`Is Not Valid`
      (`KismetSystemLibrary.PrintString` "ERROR: No Special Location Found"))))

(event `Play Attack Animation`
  (bind _ac_bossstats (`self.AC_BossStats`))
  (bind _capsulecomponent (`self.CapsuleComponent`))
  (bind _returnvalue (`SceneComponent.K2_GetComponentLocation` _capsulecomponent))
  (bind _boss_element (`/Game/AI/Boss/C_BossStats.Boss Element` _ac_bossstats))
  ;[1 1 1] Normal Attack
  (`|PlayMontage` (`self.Mesh`) "/Game/Animations/Attack_PrimaryA_Montage.Attack_PrimaryA_Montage"
    (:`then`
      (`KismetSystemLibrary.Delay` 0.45)
      (bind _outhit (`KismetSystemLibrary.CapsuleTraceSingle` :`Start` _returnvalue :`End` (+ _returnvalue (* (`SceneComponent.GetForwardVector` _capsulecomponent) (`/Game/AI/Boss/C_BossStats.Attack Range` (`self.AC_BossStats`)))) :`Radius` 100.0 :`TraceChannel` "TraceTypeQuery3" :`DrawDebugType` "ForDuration"))
      (bind (_bblockinghit _binitialoverlap _time _distance _location _impactpoint _normal _impactnormal _physmat _hitactor) (`GameplayStatics.BreakHitResult` _outhit))
      (if (== _hitactor (`GameplayStatics.GetPlayerCharacter` 0))
        (message `/Game/Combat/I_Combat.TakeDamage` _hitactor (`/Game/AI/Boss/C_BossStats.Damage` _ac_bossstats) null null self _boss_element true 1.0)
        (message `/Game/Combat/I_Combat.ApplyDebuff` _hitactor 0.0 null null self _boss_element)))))

(event `Do Shock Wave`
  (bind _returnvalue (`GameplayStatics.GetPlayerCharacter` 0))
  (bind _ac_bossstats (`self.AC_BossStats`))
  (bind _returnvalue_2 (`SceneComponent.K2_GetComponentLocation` (`self.CapsuleComponent`)))
  (bind _charactermovement (`Character.CharacterMovement` (cast `/Game/Player/PlayerBaseCharacter` _returnvalue :!pure true)))
  ;[1 1 1] Shock Wave Attack
  (`|PlayMontage` (`self.Mesh`) "/Game/Animations/Attack_PrimaryA_Montage.Attack_PrimaryA_Montage"
    (:`then`
      (`KismetSystemLibrary.Delay` 0.45)
      (bind _outhit (`KismetSystemLibrary.CapsuleTraceSingle` :`Start` _returnvalue_2 :`End` _returnvalue_2 :`Radius` 500.0 :`TraceChannel` "TraceTypeQuery3" :`DrawDebugType` "ForDuration"))
      (bind (_bblockinghit _binitialoverlap _time _distance _location _impactpoint _normal _impactnormal _physmat _hitactor) (`GameplayStatics.BreakHitResult` _outhit))
      (if (== _hitactor (`GameplayStatics.GetPlayerCharacter` 0))
        (message `/Game/Combat/I_Combat.TakeDamage` _hitactor (/ (`/Game/AI/Boss/C_BossStats.Damage` _ac_bossstats) 2.0) null null self (`/Game/AI/Boss/C_BossStats.Boss Element` _ac_bossstats) true 1.0)
        ;;[1 1 1] Knockback
        (set `CharacterMovementComponent.GroundFriction` 0.0 _charactermovement)
        (`self.LaunchCharacter` _returnvalue (* (`KismetMathLibrary.Normal` (`KismetMathLibrary.Conv_RotatorToVector` (`KismetMathLibrary.FindLookAtRotation` (`self.K2_GetActorLocation` _returnvalue) (`SceneComponent.K2_GetComponentLocation` (`self.CapsuleComponent`))))) -5000.0) true true)
        (`KismetSystemLibrary.Delay` 1.0)
        (set `CharacterMovementComponent.GroundFriction` 8.0 _charactermovement)))))

(event `Wait`
  (`KismetSystemLibrary.Delay` 0.5))

(event `Special Mechanic`
  (`/Engine/EditorBlueprintResources/StandardMacros.DoOnce` false :!label _label
    (:`Completed`
      (`self.Special Mechanic Spawn Enemies`))))

(event `Reset Special Mechanic`
  (goto _label :!via `Reset`))

(event `Enemies Defeated`
  (`KismetSystemLibrary.K2_ClearAndInvalidateTimerHandle` (stale `Check For Enemies` _returnvalue))
  (`self.Revert Aesthetic`))

(event `Check For Enemies`
  (bind _returnvalue (`KismetSystemLibrary.K2_SetTimer` null "Check If Spawned Enemies Still Exist" 1.0 true 2.0)))

(fn `BasicSummon`
  (locals (`Spawn Enemy` :type Boolean) (EnemiesSpawned :type Integer))
  (`SkeletalMeshComponent.PlayAnimation` (`self.Mesh`) "/Game/3DModels/ArtistStuff/Version2/GrandMaster/AnimSummon_Anim.AnimSummon_Anim" false)
  (`NavMovementComponent.StopActiveMovement` (`self.CharacterMovement`))
  (set `local.Spawn Enemy` true)
  (while (`local.Spawn Enemy`)
    (set `self.EnemyFailedToSpawn` 0)
    (bind _summon_location (`self.GetSummonedEnemyLocations`))
    (bind _returnvalue (`AIBlueprintHelperLibrary.SpawnAIFromClass` "/Game/AI/Enemy/Melee/BP_MeleeEnemy.BP_MeleeEnemy_C" "/Game/AI/Enemy/Melee/BT_MeleeEnemy.BT_MeleeEnemy" _summon_location (struct) false null :!label _label))
    (`self.Wait`)
    (`/Engine/EditorBlueprintResources/StandardMacros.IsValid` _returnvalue
      (:`Is Valid`
        (`KismetArrayLibrary.Array_Add` (`self.Special_EnemiesSpawned1`) _returnvalue))
      (:`Is Not Valid`
        (`self.Enemy Failed To Spawn`
          (:`then`
            _)
          (:`else`
            (goto _label)))))
    (set `local.EnemiesSpawned` (+ (`local.EnemiesSpawned`) 1))
    (if (>= (`local.EnemiesSpawned`) 4)
      (set `local.Spawn Enemy` false)))
  (`self.Check For Enemies`))

(fn `Boss Take Damage`
  (params (Damage :type "Float (double-precision)") (Element :type "/Game/Combat/E_Element Enum" :default "NewEnumerator4") (IgnoreShield :type Boolean))
  (if (not (`self.Invulnerable`))
    (`parent.Boss Take Damage` Damage Element IgnoreShield)
    (`/Engine/EditorBlueprintResources/StandardMacros.IsValid` self
      (:`Is Valid`
        (`self.Check To See If Do Special`)))))

(fn `Change Aesthetic`
  (`SkeletalMeshComponent.PlayAnimation` (`self.Mesh`) "/Game/3DModels/ArtistStuff/Version2/GrandMaster/Chin_Scratch_Anim.Chin_Scratch_Anim" true)
  (`PrimitiveComponent.SetMaterial` (`self.Mesh`) 0 "/Game/AI/Boss/M_Boss_SpecialMaterial.M_Boss_SpecialMaterial")
  (set `/Game/AI/Boss/C_BossStats.Special` true (`self.AC_BossStats`)))

(fn `Check If Spawned Enemies Still Exist`
  (for _array_element (`self.Special_EnemiesSpawned1`)
    (`/Engine/EditorBlueprintResources/StandardMacros.IsValid` _array_element
      (:`Is Valid`
        (set `self.Enemies Still Exist?` true)
        (break))
      (:`Is Not Valid`
        (set `self.Enemies Still Exist?` false))))
  (if (not (`self.Enemies Still Exist?`))
    (`KismetArrayLibrary.Array_Clear` (`self.Special_EnemiesSpawned1`))
    (`self.Reset Special On BT`)
    (set `self.Invulnerable` false)
    (`self.Reset Special Mechanic`)
    (`self.Enemies Defeated`)))

(fn `Check To See If Do Special`
  (locals (WorkingIndex :type Integer))
  (bind _ac_healthandshield (`self.AC_HealthAndShield`))
  (bind _specialpoints (`/Game/AI/Boss/C_BossStats.SpecialPoints` (`self.AC_BossStats`)))
  (if (not (<= (`KismetArrayLibrary.Array_Length` (`/Game/AI/Boss/C_BossStats.SpecialPoints` (`self.AC_BossStats`))) 0))
    (for (_array_element _array_index) (`/Game/AI/Boss/C_BossStats.SpecialPoints` (`self.AC_BossStats`))
      (if (<= (/ (`/Game/Combat/C_HealthAndShield.Current Health` _ac_healthandshield) (`/Game/Combat/C_HealthAndShield.Max Health` _ac_healthandshield)) _array_element)
        (set `local.WorkingIndex` _array_index)
        (break)
        (else
          (set `local.WorkingIndex` -1))))
    (if (>= (`local.WorkingIndex`) 0)
      (`KismetArrayLibrary.Array_Remove` _specialpoints (`local.WorkingIndex`))
      (`KismetSystemLibrary.PrintString` (`KismetStringLibrary.Conv_IntToString` (`KismetArrayLibrary.Array_Length` _specialpoints)))
      (`self.Execute Special On BT`))))

(fn `Do Special Mechanic`
  (locals (SpawnEnemy :type Boolean :default true) (EnemiesSpawned :type Integer))
  (`self.Special Mechanic`)
  (`self.Change Aesthetic`))

(fn `EnemyAttack`
  (returns (AttackDuration :type "Float (double-precision)"))
  (`self.Play Attack Animation`)
  (return (`/Game/AI/Boss/C_BossStats.Attack Duration` (`self.AC_BossStats`))))

(fn `EnemyShockwave`
  (returns (`Attack Duration` :type "Float (double-precision)"))
  (`self.Do Shock Wave`)
  (return (`/Game/AI/Boss/C_BossStats.Attack Duration` (`self.AC_BossStats`))))

(fn `GetSummonedEnemyLocations`
  (returns (`Summon Location` :type "Vector Structure"))
  (locals (`Summoning Loc` :type "Array of /Game/Levels/LevelManager_NEW/BP_SummonerSpawnRadius Object Reference") (Valid :type Boolean) (`Summon Loc` :type "Vector Structure" :default (0.0 0.0 0.0)))
  (bind _spawnradius (`/Game/Levels/LevelManager_NEW/BP_SummonerSpawnRadius.SpawnRadius` (`KismetArrayLibrary.Array_Random` (`local.Summoning Loc`))))
  (bind (_returnvalue_x _returnvalue_y _returnvalue_z) (`KismetMathLibrary.BreakVector` (`SceneComponent.K2_GetComponentLocation` _spawnradius)))
  (bind (_returnvalue_x_2 _returnvalue_y_2) (`KismetMathLibrary.BreakVector` (`BoxComponent.GetScaledBoxExtent` _spawnradius)))
  (bind _outactors (`GameplayStatics.GetAllActorsOfClass` "/Game/Levels/LevelManager_NEW/BP_SummonerSpawnRadius.BP_SummonerSpawnRadius_C"))
  (bind _output_get (set `local.Summoning Loc` _outactors))
  (for _array_element _output_get
    (`/Engine/EditorBlueprintResources/StandardMacros.IsValid` _array_element
      (:`Is Valid`
        (set `local.Valid` true)
        (break))
      (:`Is Not Valid`
        (set `local.Valid` false))))
  (if (`local.Valid`)
    (set `local.Summon Loc` (`KismetMathLibrary.RandomPointInBoundingBox` (`KismetMathLibrary.MakeVector` _returnvalue_x _returnvalue_y _returnvalue_z) (`KismetMathLibrary.MakeVector` _returnvalue_x_2 _returnvalue_y_2 1.0)))
    (else
      (set `local.Summon Loc` (`NavigationSystemV1.K2_GetRandomLocationInNavigableRadius` (`self.K2_GetActorLocation` (`self.SpecialLocation`)) 400.0 null null))))
  (return (`local.Summon Loc`)))

(fn `Revert Aesthetic`
  (`PrimitiveComponent.SetMaterial` (`self.Mesh`) 0 "/Game/UE4_Mannequin/Character/Materials/M_Male_Body.M_Male_Body")
  (set `/Game/AI/Boss/C_BossStats.Special` false (`self.AC_BossStats`)))

(fn `Special Mechanic Spawn Enemies`
  (locals (SpawnEnemy :type Boolean) (EnemiesSpawned :type Integer))
  (`SkeletalMeshComponent.PlayAnimation` (`self.Mesh`) "/Game/3DModels/ArtistStuff/Version2/GrandMaster/AnimSummon_Anim.AnimSummon_Anim" false)
  (set `self.Invulnerable` true)
  (set `local.SpawnEnemy` true)
  (set `local.EnemiesSpawned` 0)
  (`AIBlueprintHelperLibrary.SimpleMoveToActor` (`self.GetController`) (`self.SpecialLocation`))
  (switch `int` (`self.Current Special Wave`)
    (:`0`
      ;[1 1 1] Wave 1: 4 Reg Melee
      (set `self.Special_EnemiesSpawnCount` 4)
      (while (`local.SpawnEnemy`)
        (set `self.EnemyFailedToSpawn` 0)
        (bind _summon_location (`self.GetSummonedEnemyLocations`))
        (bind _returnvalue (`AIBlueprintHelperLibrary.SpawnAIFromClass` "/Game/AI/Enemy/Melee/BP_MeleeEnemy.BP_MeleeEnemy_C" "/Game/AI/Enemy/Melee/BT_MeleeEnemy.BT_MeleeEnemy" _summon_location (struct) false null :!label _label))
        (`/Engine/EditorBlueprintResources/StandardMacros.IsValid` _returnvalue
          (:`Is Valid`
            (`KismetArrayLibrary.Array_Add` (`self.Special_EnemiesSpawned1`) _returnvalue))
          (:`Is Not Valid`
            (`self.Enemy Failed To Spawn`
              (:`then`
                _)
              (:`else`
                (goto _label)))))
        (set `local.EnemiesSpawned` (+ (`local.EnemiesSpawned`) 1) :!label _label_2)
        (if (>= (`local.EnemiesSpawned`) (`self.Special_EnemiesSpawnCount`))
          (set `local.SpawnEnemy` false)
          (`/Engine/EditorBlueprintResources/StandardMacros.IncrementInt` (`self.Current Special Wave`)))))
    (:`1`
      ;[1 1 1] Wave 2: 2 Reg and 2 Elite Melee
      (set `self.Special_EnemiesSpawnCount` 2)
      (while (`local.SpawnEnemy`)
        (set `self.EnemyFailedToSpawn` 0)
        (bind _summon_location_2 (`self.GetSummonedEnemyLocations`))
        (bind _returnvalue_2 (`AIBlueprintHelperLibrary.SpawnAIFromClass` "/Game/AI/Enemy/Melee/BP_MeleeEnemy.BP_MeleeEnemy_C" "/Game/AI/Enemy/Melee/BT_MeleeEnemy.BT_MeleeEnemy" _summon_location_2 (struct) false null :!label _label_3))
        (`/Engine/EditorBlueprintResources/StandardMacros.IsValid` _returnvalue_2
          (:`Is Valid`
            (`KismetArrayLibrary.Array_Add` (`self.Special_EnemiesSpawned1`) _returnvalue_2)
            (bind _summon_location_3 (`self.GetSummonedEnemyLocations`))
            (bind _returnvalue_3 (`AIBlueprintHelperLibrary.SpawnAIFromClass` "/Game/AI/Enemy/Melee/BP_EliteMelee.BP_EliteMelee_C" "/Game/AI/Enemy/Melee/BT_MeleeEnemy.BT_MeleeEnemy" _summon_location_3 (struct) false null :!label _label_4))
            (`/Engine/EditorBlueprintResources/StandardMacros.IsValid` _returnvalue_3
              (:`Is Valid`
                (`KismetArrayLibrary.Array_Add` (`self.Special_EnemiesSpawned1`) _returnvalue_3)
                (goto _label_2))
              (:`Is Not Valid`
                (goto _label_4))))
          (:`Is Not Valid`
            (`self.Enemy Failed To Spawn`
              (:`then`
                (goto _label_2))
              (:`else`
                (goto _label_3)))))))
    (:`2`
      ;[1 1 1] Wave 3: 4 Elite Melee
      (set `self.Special_EnemiesSpawnCount` 4)
      (while (`local.SpawnEnemy`)
        (set `self.EnemyFailedToSpawn` 0)
        (bind _summon_location_4 (`self.GetSummonedEnemyLocations`))
        (bind _returnvalue_4 (`AIBlueprintHelperLibrary.SpawnAIFromClass` "/Game/AI/Enemy/Melee/BP_EliteMelee.BP_EliteMelee_C" "/Game/AI/Enemy/Melee/BT_MeleeEnemy.BT_MeleeEnemy" _summon_location_4 (struct) false null :!label _label_5))
        (`/Engine/EditorBlueprintResources/StandardMacros.IsValid` _returnvalue_4
          (:`Is Valid`
            (`KismetArrayLibrary.Array_Add` (`self.Special_EnemiesSpawned1`) _returnvalue_4)
            (goto _label_2))
          (:`Is Not Valid`
            (`self.Enemy Failed To Spawn`
              (:`then`
                (goto _label_2))
              (:`else`
                (goto _label_5))))))))
  (`self.Check For Enemies`))

(fn `UserConstructionScript`
  (`parent.UserConstructionScript`))