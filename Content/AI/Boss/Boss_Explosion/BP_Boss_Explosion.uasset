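; Explosion boss that makes a montage-timed capsule-trace melee attack, damaging and debuffing the player.
; Crossing a SpecialPoints health threshold consumes it and triggers the special through the behavior tree.
; The DoOnce-guarded special makes it invulnerable, swaps its material, sends it to SpecialLocation and recursively spawns delayed explosions at random navigable points near the player.
; Finishing restores vulnerability and appearance, re-arms the special and increases the next explosion count.
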(event `self.ReceiveBeginPlay`
  (`parent.ReceiveBeginPlay`)
  (set `self.EnemyType` "NewEnumerator2")
  (set `self.Special_ExplosionSpawnCount` 10)
  (bind _returnvalue (`GameplayStatics.GetActorOfClass` "/Game/AI/Boss/SpecialLocation.SpecialLocation_C"))
  (bind _output_get (set `self.SpecialLocation` _returnvalue))
  (`/Engine/EditorBlueprintResources/StandardMacros.IsValid` _output_get
    (:`Is Valid`
      (`KismetSystemLibrary.PrintString` "Special Location Found"))
    (:`Is Not Valid`
      (`KismetSystemLibrary.PrintString` "ERROR: No Special Location Found"))))

(event `Play Attack Animation`
  (bind _ac_bossstats (`self.AC_BossStats`))
  (bind _capsulecomponent (`self.CapsuleComponent`))
  (bind _returnvalue (`SceneComponent.K2_GetComponentLocation` _capsulecomponent))
  (bind _boss_element (`/Game/AI/Boss/C_BossStats.Boss Element` _ac_bossstats))
  (`|PlayMontage` (`self.Mesh`) "/Game/Animations/Attack_PrimaryA_Montage.Attack_PrimaryA_Montage"
    (:`then`
      (`KismetSystemLibrary.Delay` 0.45)
      (bind _outhit (`KismetSystemLibrary.CapsuleTraceSingle` :`Start` _returnvalue :`End` (+ _returnvalue (* (`SceneComponent.GetForwardVector` _capsulecomponent) (`/Game/AI/Boss/C_BossStats.Attack Range` (`self.AC_BossStats`)))) :`Radius` 100.0 :`TraceChannel` "TraceTypeQuery3" :`DrawDebugType` "ForDuration"))
      (bind (_bblockinghit _binitialoverlap _time _distance _location _impactpoint _normal _impactnormal _physmat _hitactor) (`GameplayStatics.BreakHitResult` _outhit))
      (if (== _hitactor (`GameplayStatics.GetPlayerCharacter` 0))
        (message `/Game/Combat/I_Combat.TakeDamage` _hitactor (`/Game/AI/Boss/C_BossStats.Damage` _ac_bossstats) null null self _boss_element)
        (message `/Game/Combat/I_Combat.ApplyDebuff` _hitactor 0.0 null null self _boss_element)))))

(event `Special Mechanic`
  (`/Engine/EditorBlueprintResources/StandardMacros.DoOnce` false :!label _label
    (:`Completed`
      (`self.Do Explosion Phase`))))

(event `Reset Special Mechanic`
  (goto _label :!via `Reset`))

(event `Do Explosion Phase`
  (set `self.Invulnerable` true)
  (`AIBlueprintHelperLibrary.SimpleMoveToActor` (`self.GetController`) (`self.SpecialLocation`))
  (set `self.Explosions Spawned` 0)
  (`KismetSystemLibrary.Delay` 0.5)
  (`self.Spawn Explosions`))

(event `Spawn Explosions`
  (if (< (`self.Explosions Spawned`) (`self.Special_ExplosionSpawnCount`))
    (`KismetSystemLibrary.Delay` 0.5)
    (`/Game/AI/ExplosionMechanic/C_Explosion.Spawn Explosion` (`self.C_Explosion`) (`NavigationSystemV1.K2_GetRandomLocationInNavigableRadius` (`SceneComponent.K2_GetComponentLocation` (`Character.CapsuleComponent` (`GameplayStatics.GetPlayerCharacter` 0))) 300.0 null null))
    (set `self.Explosions Spawned` (+ (`self.Explosions Spawned`) 1))
    (`self.Spawn Explosions`)
    (else
      (`KismetSystemLibrary.Delay` 2.1)
      (`self.Finish Special Mechanic`))))

(fn `Boss Take Damage`
  (params (Damage :type "Float (double-precision)") (Element :type "/Game/Combat/E_Element Enum" :default "NewEnumerator4") (IgnoreShield :type Boolean))
  (if (not (`self.Invulnerable`))
    (`parent.Boss Take Damage` Damage Element IgnoreShield)
    (`/Engine/EditorBlueprintResources/StandardMacros.IsValid` self
      (:`Is Valid`
        (`self.Check To See If Do Special`)))))

(fn `Change Aesthetic`
  (`PrimitiveComponent.SetMaterial` (`self.Mesh`) 0 "/Game/AI/Boss/M_Boss_SpecialMaterial.M_Boss_SpecialMaterial")
  (set `/Game/AI/Boss/C_BossStats.Special` true (`self.AC_BossStats`)))

(fn `Check To See If Do Special`
  (locals (WorkingIndex :type Integer))
  (bind _ac_healthandshield (`self.AC_HealthAndShield`))
  (bind _specialpoints (`/Game/AI/Boss/C_BossStats.SpecialPoints` (`self.AC_BossStats`)))
  (if (not (<= (`KismetArrayLibrary.Array_Length` (`/Game/AI/Boss/C_BossStats.SpecialPoints` (`self.AC_BossStats`))) 0))
    (for (_array_element _array_index) (`/Game/AI/Boss/C_BossStats.SpecialPoints` (`self.AC_BossStats`))
      (if (<= (/ (`/Game/Combat/C_HealthAndShield.Current Health` _ac_healthandshield) (`/Game/Combat/C_HealthAndShield.Max Health` _ac_healthandshield)) _array_element)
        (set `local.WorkingIndex` _array_index)
        (break)
        (else
          (set `local.WorkingIndex` -1))))
    (if (>= (`local.WorkingIndex`) 0)
      (`KismetArrayLibrary.Array_Remove` _specialpoints (`local.WorkingIndex`))
      (`KismetSystemLibrary.PrintString` (`KismetStringLibrary.Conv_IntToString` (`KismetArrayLibrary.Array_Length` _specialpoints)))
      (`self.Execute Special On BT`))))

(fn `Do Special Mechanic`
  (locals (SpawnEnemy :type Boolean :default true) (EnemiesSpawned :type Integer))
  (`self.Special Mechanic`)
  (`self.Change Aesthetic`))

(fn `EnemyAttack`
  (returns (AttackDuration :type "Float (double-precision)"))
  (`self.Play Attack Animation`)
  (return (`/Game/AI/Boss/C_BossStats.Attack Duration` (`self.AC_BossStats`))))

(fn `Finish Special Mechanic`
  (locals (`Still Exist?` :type Boolean))
  (`self.Reset Special On BT`)
  (set `self.Invulnerable` false)
  (`self.Reset Special Mechanic`)
  (`self.Revert Aesthetic`)
  (set `self.Special_ExplosionSpawnCount` (+ (`self.Special_ExplosionSpawnCount`) 5)))

(fn `Revert Aesthetic`
  (`PrimitiveComponent.SetMaterial` (`self.Mesh`) 0 "/Game/UE4_Mannequin/Character/Materials/M_Male_Body.M_Male_Body")
  (set `/Game/AI/Boss/C_BossStats.Special` false (`self.AC_BossStats`)))

(fn `UserConstructionScript`
  (`parent.UserConstructionScript`))