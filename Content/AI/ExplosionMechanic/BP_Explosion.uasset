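; Explosion actor that blinks a warning radius with a sizzle sound, then deals area damage and destroys itself.
; StartExplosion drives the radius color on a dynamic material through a timeline, then calls Explode when it finishes.
; Explode runs two debug-drawn capsule traces, sending full damage through I_Combat within the inner radius and half within the outer, which ignores inner hits.
; ExplodeFX+Death then spawns the fire emitter and sound before destroying the actor.
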(event `Start Explosion`
  (bind _explosionsizzle (`self.ExplosionSizzle`))
  ;[1 1 1] Do the explosion radius blinking
  (bind _returnvalue (`PrimitiveComponent.CreateDynamicMaterialInstance` (`self.Explosion Radius`) 0 "/Game/Textures/PlaceHolders(PH)/M_ExplosionRed_PH.M_ExplosionRed_PH" "None"))
  (set `self.M_ExplosionRadiusMaterial` _returnvalue)
  (`AudioComponent.Play` _explosionsizzle 0.0)
  (bind (_direction _color_graph) (`Timeline|T_ExplosionBlinking` :!via `PlayFromStart`)
    (:`Update`
      (`MaterialInstanceDynamic.SetVectorParameterValue` (`self.M_ExplosionRadiusMaterial`) "Explosion Radius Color" _color_graph))
    (:`Finished`
      (`AudioComponent.Stop` _explosionsizzle)
      ;[1 1 1] Explode and deal damage
      (`self.Explode`))))

(event `ExplodeFX+Death`
  (bind _returnvalue (`self.K2_GetActorLocation`))
  ;[1 1 1] Sound and Animation
  (`GameplayStatics.SpawnEmitterAtLocation` "/Game/M5VFXVOL2/Particles/Explosion/Fire_Exp_01.Fire_Exp_01" _returnvalue (struct :`Pitch` 45.0))
  (`GameplayStatics.SpawnSoundAtLocation` "/Game/UE4_FPTemplate/FirstPerson/Audio/FirstPersonTemplateWeaponFire02.FirstPersonTemplateWeaponFire02" _returnvalue (struct) 1.0 1.0 0.0 null null)
  (`self.K2_DestroyActor`))

(event `Explode`
  (bind _returnvalue (`SceneComponent.K2_GetComponentLocation` (`self.DefaultSceneRoot`)))
  (bind _returnvalue_2 (`SceneComponent.K2_GetComponentLocation` (`self.DefaultSceneRoot`)))
  ;[1 1 1] Explode and deal damage
  ;;[1 1 1] Explosion inner radius hit
  (bind _outhits (`KismetSystemLibrary.CapsuleTraceMulti` :`Start` _returnvalue_2 :`End` (+ _returnvalue_2 (0.0 0.0 50.0)) :`Radius` (`self.Explosion Inner Radius`) :`TraceChannel` "TraceTypeQuery4" :`DrawDebugType` "ForDuration"))
  (for _array_element _outhits
    (bind (_bblockinghit _binitialoverlap _time _distance _location _impactpoint _normal _impactnormal _physmat _hitactor) (`GameplayStatics.BreakHitResult` _array_element))
    (`KismetArrayLibrary.Array_Add` (`self.Inner Explosion Hit Actors`) _hitactor)
    (if (`KismetSystemLibrary.DoesImplementInterface` _hitactor "/Game/Combat/I_Combat.I_Combat_C")
      (message `/Game/Combat/I_Combat.TakeDamage` _hitactor (`self.Explosion Damage`) null null null "NewEnumerator4" true 1.0)
      (else
        (`KismetSystemLibrary.PrintString` "I hit nothing" :!label _label))))
  ;;[1 1 1] Explosion outer radius hit
  (bind _outhits_2 (`KismetSystemLibrary.CapsuleTraceMulti` _returnvalue (+ _returnvalue (0.0 0.0 50.0)) (`self.Explosion Outer Radius`) 0.0 "TraceTypeQuery4" false (`self.Inner Explosion Hit Actors`) "ForDuration" true (struct :`R` 1.0 :`B` 0.299212 :`A` 1.0) (struct :`G` 1.0 :`B` 0.23749 :`A` 1.0)))
  (for _array_element_2 _outhits_2
    (bind (_bblockinghit_2 _binitialoverlap_2 _time_2 _distance_2 _location_2 _impactpoint_2 _normal_2 _impactnormal_2 _physmat_2 _hitactor_2) (`GameplayStatics.BreakHitResult` _array_element_2))
    (if (`KismetSystemLibrary.DoesImplementInterface` _hitactor_2 "/Game/Combat/I_Combat.I_Combat_C")
      (message `/Game/Combat/I_Combat.TakeDamage` _hitactor_2 (/ (`self.Explosion Damage`) 2.0) null null null "NewEnumerator4" true 1.0)
      (else
        (goto _label))))
  (`self.ExplodeFX+Death`))

(fn `UserConstructionScript`)