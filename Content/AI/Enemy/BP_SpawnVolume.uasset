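; BP_SpawnVolume is a trigger volume that spawns AI enemies the first time the player character overlaps it.
; It loops over its SpawnPoints array, reading each BP_SpawnLocation's EnemyType to pick a pawn class and behavior tree, then spawns that AI at the point's location.
; An EnemiesSpawned flag prevents repeat spawns.
; The Boss type is unimplemented and only prints a placeholder message.
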(event `self.ReceiveBeginPlay`)

(event `self.ReceiveActorBeginOverlap`
  (params (OtherActor :type "Actor Object Reference"))
  (bind _asplayer_base_character (cast `/Game/Player/PlayerBaseCharacter` OtherActor))
  (set `self.PlayerCharacter` _asplayer_base_character)
  (if (not (`self.EnemiesSpawned`))
    (for _array_element (`self.SpawnPoints`)
      (bind _asbp_spawn_location (cast `/Game/AI/Enemy/BP_SpawnLocation` _array_element))
      (switch `/Game/AI/Enemy/E_EnemyTypes` (`/Game/AI/Enemy/BP_SpawnLocation.EnemyType` _asbp_spawn_location)
        (:`NewEnumerator0`
          (set `self.Pawn Class` "/Game/AI/Enemy/Melee/BP_MeleeEnemy.BP_MeleeEnemy_C")
          (set `self.Behavior` "/Game/AI/Enemy/Melee/BT_MeleeEnemy.BT_MeleeEnemy")
          (`AIBlueprintHelperLibrary.SpawnAIFromClass` (`self.Pawn Class`) (`self.Behavior`) (`self.K2_GetActorLocation` _array_element) (struct) false null :!label _label))
        (:`NewEnumerator3`
          (set `self.Pawn Class` "/Game/AI/Enemy/Range/BP_RangeEnemy.BP_RangeEnemy_C")
          (set `self.Behavior` "/Game/AI/Enemy/Range/BT_RangeEnemy.BT_RangeEnemy")
          (goto _label))
        (:`NewEnumerator7`
          (set `self.Pawn Class` "/Game/AI/Enemy/Melee/BP_MeleeEnemy_Exploder.BP_MeleeEnemy_Exploder_C")
          (set `self.Behavior` "/Game/AI/Enemy/Melee/BT_MeleeEnemy.BT_MeleeEnemy")
          (goto _label))
        (:`NewEnumerator8`
          (set `self.Pawn Class` "/Game/AI/Enemy/Grenadier/BP_Grenadier.BP_Grenadier_C")
          (set `self.Behavior` "/Game/AI/Enemy/Grenadier/BT_Grenadier.BT_Grenadier")
          (goto _label))
        (:`NewEnumerator1`
          (set `self.Pawn Class` "/Game/AI/Enemy/Melee/BP_EliteMelee.BP_EliteMelee_C")
          (set `self.Behavior` "/Game/AI/Enemy/Melee/BT_EliteMelee.BT_EliteMelee")
          (goto _label))
        (:`NewEnumerator9`
          (set `self.Pawn Class` "/Game/AI/Enemy/Range/BP_EliteRange.BP_EliteRange_C")
          (set `self.Behavior` "/Game/AI/Enemy/Range/BT_EliteRange.BT_EliteRange")
          (goto _label))
        (:`NewEnumerator2`
          (`KismetSystemLibrary.PrintString` "This class hasn't been defined yet... nerd"))))
    (set `self.EnemiesSpawned` true)))

(fn `UserConstructionScript`)