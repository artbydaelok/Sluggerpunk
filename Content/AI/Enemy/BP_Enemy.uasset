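; Enemy character Blueprint with health/shield, an overhead health bar shown near the player, and stub attack and shockwave functions.
; TakeDamage shows damage numbers, boosts Ice damage by half and optionally launches knockback.
; BeginPlay scales attack damage by game mode and room; death drops gold or a rare upgrade and increments the kill count.
; ClimbUp/Down computes ballistic launches to nav-link destinations so enemies can jump between platforms.
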(event Custom|Climb%20Up/Down
  (params (Nav%20Link%20Ref :type BP%20Custom%20Nav%20Link%20Object%20Reference))
  (bind _returnvalue (Transformation|GetActorLocation))
  (bind _destination (Variables|/Game/AI/BP_CustomNavLink.BP_CustomNavLink_C|GetDestination Nav%20Link%20Ref))
  (bind (_x _y _z) (Math|Vector|BreakVector _destination))
  (bind (_x_2 _y_2 _z_2) (Math|Vector|BreakVector _returnvalue))
  (Character|LaunchCharacter (Math|Vector|MakeVector (|((DestinationX-StartX)/{791021B3-49F7-A5FB-B731-0D863CB28DD6}) _x _x_2) (|((DestinationY-StartY)/{791021B3-49F7-A5FB-B731-0D863CB28DD6}) _y _y_2) (|((DestinationHeight-(StartHeight-(((Power({791021B3-49F7-A5FB-B731-0D863CB28DD6},2))*0.500000)*{E3B4C1C9-4A34-AC0D-7799-EFBBB0E80BC3})))/{791021B3-49F7-A5FB-B731-0D863CB28DD6}) _z _z_2)) true true)
  (Utilities|FlowControl|Delay 1.0)
  (Default|Reset Nav%20Link%20Ref))

(event EventBeginPlay
  (bind _auraparticle (Variables|Default|GetAuraParticle))
  (bind _relativelocation (Variables|/Script/Engine.SceneComponent|GetRelativeLocation _auraparticle))
  (bind _returnvalue (Actor|GetActorOfClass "/Game/Player/PlayerBaseCharacter.PlayerBaseCharacter_C"))
  (Variables|Default|SetPlayer%20Ref _returnvalue)
  (Utilities|FlowControl|Sequence
    (:then_0
      (bind _asw_enemy_health (Utilities|Casting|CastToW_EnemyHealth (UserInterface|GetWidget (Variables|Default|GetHealthBar))))
      (bind _output_get (Variables|Default|SetHealth%20Wid%20Ref _asw_enemy_health))
      (Default|SetReference _output_get self)
      (Variables|Default|SetState "NewEnumerator0")
      (bind _woooaahahawhahwahwhdaojf (Timeline|ByeByeNiagara PlayFromStart)
        (:Update
          (Transformation|SetRelativeLocation (Variables|Default|GetAuraParticle) (Math|Vector|Lerp(Vector) _relativelocation (- _relativelocation "0, 0,90.000000") _woooaahahawhahwahwhdaojf) false false)
          (CallFunction|DamageScaling)
          (bind _returnvalue_2 (Audio|CreateSound2D "/Game/Audio/Enemy_Death.Enemy_Death" 1.0 1.0 0.0 0))
          (Variables|Default|SetEnemyDeath _returnvalue_2)
          (bind _returnvalue_3 (Audio|CreateSound2D "/Game/Audio/enemy_attack_melee.enemy_attack_melee" 1.0 1.0 0.0 0))
          (Variables|Default|Setenemy%20attack _returnvalue_3))))))

(event EventTakeDamage
  (params (Damage :type Float%20%28single-precision%29) (Player :type Player%20Base%20Character%20Object%20Reference) (Enemy :type BP%20Enemy%20Object%20Reference) (Boss :type BP%20Boss%20Object%20Reference) (Element :type E_Element%20Enum :default "NewEnumerator4") (DealsKnockback :type Boolean) (KB%20Multiplier :type Float%20%28single-precision%29))
  ;[1 1 1] Enemy takes damage from Player
  (Variables|Default|SetKnockbackMult KB%20Multiplier)
  (Default|SpawnDamageNumber (Variables|Default|GetPlayer%20Ref) (Utilities|Text|ToText(Float) (* Damage 1e+01) "HalfToEven" false true 1 324 0 0) (Transformation|GetActorLocation))
  (bind _output_get (Variables|Default|SetElementalType Element))
  (switch Utilities|FlowControl|Switch|SwitchonE_Element _output_get
    (:NewEnumerator4
      (Default|Heal/TakeDamage (Variables|Default|GetAC_HealthAndShield) (- 0.0 Damage) false :!label _label))
    (:NewEnumerator3
      (goto _label))
    (:NewEnumerator1
      (Default|Heal/TakeDamage (Variables|Default|GetAC_HealthAndShield) (* (- 0.0 Damage) 1.5) false)))
  (Utilities|IsValid self
    (:Is%20Valid
      (if (and DealsKnockback (not (Variables|/Game/Player/BaseballProj/C_BallDebuffs.C_BallDebuffs_C|GetGrounded (Variables|Default|GetC_BallDebuffs))))
        ;;[1 1 1] Knockback
        (Class|NavMovementComponent|StopActiveMovement (Variables|Character|GetCharacterMovement))
        (Variables|/Script/Engine.CharacterMovementComponent|SetGroundFriction (Variables|Character|GetCharacterMovement) 0.0)
        (Variables|Default|SetKB%20Start%20Loc (Transformation|GetWorldLocation (Variables|Collision|GetCapsuleComponent)))
        (Character|LaunchCharacter (* (Math|Vector|Normalize (Math|Rotator|GetRotationXVector (Math|Rotator|FindLookatRotation (Variables|Default|GetKB%20Start%20Loc) (Transformation|GetActorLocation (Game|GetPlayerCharacter 0))))) (Variables|Default|GetKB%20Distance)) true true)
        (Variables|Default|SetKnockbackMult 1.0)))))

(event EventOnDeath
  ;[1 1 1] Enemy takes damage from Player
  ;;[1 1 1] Death
  (CallFunction|EnemyDeath))

(event EventTick
  (params (DeltaSeconds :type Float%20%28single-precision%29))
  (bind _health_wid_ref (Variables|Default|GetHealth%20Wid%20Ref))
  ;[1 1 1] Appearing/Disappearing Health Bar
  (if (>= (Math|Vector|GetPointDistancetoLine (Transformation|GetActorLocation (Game|GetPlayerCharacter 0)) (Transformation|GetActorLocation self) "0, 0, 0") 2.5e+03)
    (Widget|SetVisibility _health_wid_ref "Hidden")
    (else
      (Widget|SetVisibility _health_wid_ref "Visible"))))

(fn ConstructionScript
  (Rendering|SetVisibility (Variables|Default|GetHealthBar) true false))

(fn EnemyKnockback
  (bind _returnvalue (Transformation|GetActorForwardVector))
  (Utilities|IsValid self
    (:Is%20Valid
      (Class|NavMovementComponent|StopActiveMovement (Variables|Character|GetCharacterMovement))
      (bind _output_get (Variables|Default|SetKB%20Start%20Loc (Transformation|GetWorldLocation (Variables|Collision|GetCapsuleComponent))))
      (bind (_outhit _returnvalue_2) (Collision|CapsuleTraceByChannel _output_get (+ (Variables|Default|GetKB%20Start%20Loc) (* (Math|Vector|Normalize (Math|Rotator|GetRotationXVector (Math|Rotator|FindLookatRotation (Variables|Default|GetKB%20Start%20Loc) (Transformation|GetActorLocation (Game|GetPlayerCharacter 0))))) (Variables|Default|GetKB%20Distance))) 3e+01 5e+01 "TraceTypeQuery1" false 0 "ForDuration"))
      (if _returnvalue_2
        ;[1 1 1] If something was hit, KB to the hit location minus the enemy's capsule radius
        (Variables|Default|SetKB%20End%20Loc (+ (.Location (Collision|BreakHitResult _outhit)) (* (Transformation|GetActorForwardVector) -39.0)))
        ;[1 1 1] Direction is Backward
        (Variables|Default|SetKB%20Dir _returnvalue)
        (else
          ;[1 1 1] If nothing was hit, KB to location
          (Variables|Default|SetKB%20End%20Loc (.TraceEnd (Collision|BreakHitResult _outhit)))
          (Variables|Default|SetKB%20Dir _returnvalue)))
      (return (Variables|Default|GetKB%20End%20Loc) (Variables|Default|GetKB%20Dir)))))

(fn EnemyDeath
  (bind _enemydeath (Variables|Default|GetEnemyDeath))
  (if (Variables|Default|GetCanDropUpgrade)
    (if (Math|Random|RandomBoolwithWeight 0.05)
      (bind _upgrade (Default|DropUpgrade (Variables|Default|GetC_UpgradeDrop) (Transformation|GetWorldLocation (Variables|Default|GetGoldSpawnAnchor)) false "NewEnumerator3"))
      (Default|SetUpgrade _upgrade)
      (else
        (Game|SpawnActorfromClass "/Game/Collectibles/BP_Gold.BP_Gold_C" (Math|Transform|MakeTransform (Transformation|GetWorldLocation (Variables|Default|GetGoldSpawnAnchor)) "0, 0, 0" "1,1,1") "Undefined" 0 5 (Variables|Default|GetEnemyType) false 0 :!label _label)))
    (else
      (goto _label)))
  (Math|Integer|IncrementInt (Variables|/Game/Player/PlayerBaseGameInstance.PlayerBaseGameInstance_C|GetEnemies%20Killed (.AsPlayer%20Base%20Game%20Instance (Utilities|Casting|CastToPlayerBaseGameInstance (Game|GetGameInstance))))
    (:%20%20
      (Actor|DestroyActor)
      (Utilities|FlowControl|DoOnce false
        (:Completed
          (Audio|Components|Audio|SetPitchMultiplier _enemydeath (Math|Random|RandomFloatinRange 1.0 1.4))
          (Audio|Components|Audio|Play _enemydeath 0.0))))))

(fn ElementDebuffCheck
  (params (Element :type E_Element%20Enum :default "NewEnumerator4")))

(fn ResetInvincibility
  (Variables|Default|SetisInvincible false))

(fn DamageScaling
  (LocalVariables|SetLoop%20Check 0)
  (LocalVariables|SetDamage%20Scaled 5.0)
  (bind _asplayer_base_game_instance (Utilities|Casting|CastToPlayerBaseGameInstance (Game|GetGameInstance)))
  (switch Utilities|FlowControl|Switch|SwitchonE_Gamemodes (Variables|/Game/Player/PlayerBaseGameInstance.PlayerBaseGameInstance_C|GetGamemode _asplayer_base_game_instance)
    (:NewEnumerator0
      ;[1 1 1] Story damage scaling
      (if (Math|Integer|InRange(Integer) (Variables|/Game/Player/PlayerBaseGameInstance.PlayerBaseGameInstance_C|GetCurrentRoom _asplayer_base_game_instance) 1 5)
        (LocalVariables|SetDamage%20Scaled 5.0)
        (elif (Math|Integer|InRange(Integer) (Variables|/Game/Player/PlayerBaseGameInstance.PlayerBaseGameInstance_C|GetCurrentRoom _asplayer_base_game_instance) 6 10)
          (LocalVariables|SetDamage%20Scaled 5.25)
          (elif (Math|Integer|InRange(Integer) (Variables|/Game/Player/PlayerBaseGameInstance.PlayerBaseGameInstance_C|GetCurrentRoom _asplayer_base_game_instance) 11 15)
            (LocalVariables|SetDamage%20Scaled 5.5)
            (else
              (LocalVariables|SetDamage%20Scaled 6.0)))))
      (Variables|Default|SetDamage (LocalVariables|GetDamage%20Scaled)))
    (:NewEnumerator1
      ;[1 1 1] Endless damage scaling
      (while (< (LocalVariables|GetLoop%20Check) (- (Variables|/Game/Player/PlayerBaseGameInstance.PlayerBaseGameInstance_C|GetCurrentRoom _asplayer_base_game_instance) 5))
        (LocalVariables|SetDamage%20Scaled (Math|Float|Clamp(Float) (+ (LocalVariables|GetDamage%20Scaled) (LocalVariables|GetDamage%20Base%20Increase)) 5.0 8.0))
        (Math|Integer|IncrementInt (LocalVariables|GetLoop%20Check)))
      (Variables|Default|SetDamage (LocalVariables|GetDamage%20Scaled)))))

(fn EnemyAttack
  (return 0.0))

(fn EnemyShockwave
  (return 0.0))