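; BP_EliteMelee is an elite melee enemy that attacks the player with fire or ice elemental damage debuffs.
; On BeginPlay it attaches its weapon to the mesh grip socket, randomly picks one of two elements and sets the matching bat material.
; EnemyAttack, apparently triggered by a behavior tree task, plays the montage and immediately capsule-traces forward with debug drawing.
; A player hit sends damage and applies the element's timed debuff.
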(event `self.ReceiveBeginPlay`
  (`parent.ReceiveBeginPlay`)
  (`SceneComponent.K2_AttachToComponent` (`self.WeaponRoot`) (`self.Mesh`) "GripPoint" "SnapToTarget" "SnapToTarget" "KeepWorld" true)
  (set `self.EnemyType` "NewEnumerator1")
  ;[1 1 1] Once more element types are available, change to bottom code
  (bind _output_get (set `self.Current Element` (`|GetArrayItem` (`self.Element Array`) (`KismetMathLibrary.RandomIntegerInRange` 0 1))))
  ;[1 0.1577 0] Fire Type
  (if (`|EnumEquality` _output_get "NewEnumerator0")
    (`PrimitiveComponent.SetMaterial` (`self.MeleeWeapon`) 0 "/Game/AI/Enemy/EnemyWeapons/FireBat_Color.FireBat_Color")
    (else
      ;[0 0.778 1] Ice Type Ice
      (if (`|EnumEquality` _output_get "NewEnumerator1")
        (`PrimitiveComponent.SetMaterial` (`self.MeleeWeapon`) 0 "/Game/AI/Enemy/EnemyWeapons/WaterBat_Color.WaterBat_Color")))))

(event `PlayAnimation`
  ;[1 1 1] Enemy attacks/ Message is sent from the BBTask
  (`|PlayMontage` (`self.Mesh`) "/Game/Animations/Attack_PrimaryA_Montage.Attack_PrimaryA_Montage"))

(fn `EnemyAttack`
  (returns (AttackDuration :type "Float (double-precision)"))
  (bind _capsulecomponent (`self.CapsuleComponent`))
  (bind _returnvalue (`SceneComponent.K2_GetComponentLocation` _capsulecomponent))
  (`self.PlayAnimation`)
  (bind _outhit (`KismetSystemLibrary.CapsuleTraceSingle` :`Start` _returnvalue :`End` (+ _returnvalue (* (`SceneComponent.GetForwardVector` _capsulecomponent) 150.0)) :`Radius` 50.0 :`TraceChannel` "TraceTypeQuery3" :`DrawDebugType` "ForDuration" :`DrawTime` 2.5))
  (bind (_bblockinghit _binitialoverlap _time _distance _location _impactpoint _normal _impactnormal _physmat _hitactor) (`GameplayStatics.BreakHitResult` _outhit))
  (if (== _hitactor (`GameplayStatics.GetPlayerCharacter` 0))
    (message `/Game/Combat/I_Combat.TakeDamage` _hitactor (`self.Damage`) null self null "NewEnumerator4" true 1.0)
    (message `/Game/Combat/I_Combat.ApplyDebuff` (`self.AC_DebuffType`) 3.0 null self null (`self.Current Element`))
    (return (`self.AttackDuration`))))

(fn `UserConstructionScript`)