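; Melee enemy variant that attacks the player at close range and explodes when it dies.
; EnemyAttack plays a montage and runs a debug-drawn capsule trace forward; hitting the player sends damage and applies an elemental debuff.
; Death spawns an explosion through CExplosion at the capsule location before running parent death logic.
; The construction script snaps the weapon root to the mesh's GripPoint socket.
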(event `self.ReceiveBeginPlay`
  (`parent.ReceiveBeginPlay`)
  (set `self.EnemyType` "NewEnumerator7"))

(event `PlayAnimation`
  ;[1 1 1] Enemy attacks/ Message is sent from the BBTask
  (`|PlayMontage` (`self.Mesh`) "/Game/Animations/Attack_PrimaryA_Montage.Attack_PrimaryA_Montage"))

(fn `Enemy Death`
  (`/Game/AI/ExplosionMechanic/C_Explosion.Spawn Explosion` (`self.C_Explosion`) (`SceneComponent.K2_GetComponentLocation` (`self.CapsuleComponent`)))
  (`parent.Enemy Death`))

(fn `EnemyAttack`
  (returns (AttackDuration :type "Float (double-precision)"))
  (bind _capsulecomponent (`self.CapsuleComponent`))
  (bind _returnvalue (`SceneComponent.K2_GetComponentLocation` _capsulecomponent))
  (`self.PlayAnimation`)
  (bind _outhit (`KismetSystemLibrary.CapsuleTraceSingle` :`Start` _returnvalue :`End` (+ _returnvalue (* (`SceneComponent.GetForwardVector` _capsulecomponent) 150.0)) :`Radius` 50.0 :`TraceChannel` "TraceTypeQuery3" :`DrawDebugType` "ForDuration" :`DrawTime` 2.5))
  (bind (_bblockinghit _binitialoverlap _time _distance _location _impactpoint _normal _impactnormal _physmat _hitactor) (`GameplayStatics.BreakHitResult` _outhit))
  (if (== _hitactor (`GameplayStatics.GetPlayerCharacter` 0))
    (message `/Game/Combat/I_Combat.TakeDamage` _hitactor (`self.Damage`) null self null "NewEnumerator4" true 1.0)
    (`self.ApplyDebuff` 0.0 null self null "NewEnumerator1")
    (return (`self.AttackDuration`))))

(fn `UserConstructionScript`
  (`parent.UserConstructionScript`)
  (`SceneComponent.K2_AttachToComponent` (`self.WeaponRoot`) (`self.Mesh`) "GripPoint" "SnapToTarget" "SnapToTarget" "KeepWorld" true))