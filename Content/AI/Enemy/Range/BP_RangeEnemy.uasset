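; BP_RangeEnemy is a ranged enemy, built on a parent enemy class, that attacks by spawning BP_RangedProjectile.
; The construction script snaps WeaponRoot to the mesh's GripPoint socket, and BeginPlay sets the enemy type and prints the current state.
; EnemyAttack spawns the projectile at the Sphere component, facing along the capsule with random, asymmetric pitch and yaw spread, then returns the attack duration.
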(event `self.ReceiveBeginPlay`
  (`parent.ReceiveBeginPlay`)
  (set `self.EnemyType` "NewEnumerator3")
  (`KismetSystemLibrary.PrintString` (`|GetEnumeratorNameAsString` (`self.State`))))

(fn `EnemyAttack`
  (returns (AttackDuration :type "Float (double-precision)"))
  (bind (_returnvalue_roll _returnvalue_pitch _returnvalue_yaw) (`KismetMathLibrary.BreakRotator` (`SceneComponent.K2_GetComponentRotation` (`self.CapsuleComponent`))))
  (`|SpawnActorFromClass` "/Game/AI/Enemy/Range/BP_RangedProjectile.BP_RangedProjectile_C" (`KismetMathLibrary.MakeTransform` (`SceneComponent.K2_GetComponentLocation` (`self.Sphere`)) (`KismetMathLibrary.MakeRotator` _returnvalue_roll (+ _returnvalue_pitch (`KismetMathLibrary.RandomFloatInRange` -2.5 5.0)) (+ _returnvalue_yaw (`KismetMathLibrary.RandomFloatInRange` -10.0 15.0)))) "AdjustIfPossibleButAlwaysSpawn" "OverrideRootScale" null null)
  (return (`self.AttackDuration`)))

(fn `UserConstructionScript`
  (`parent.UserConstructionScript`)
  (`SceneComponent.K2_AttachToComponent` (`self.Weapon Root`) (`self.Mesh`) "GripPoint" "SnapToTarget" "SnapToTarget" "KeepWorld" true))