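; BP_RangedProjectile is a ranged enemy projectile that damages the player on impact.
; On hit, it sends a TakeDamageMessage with its Damage value if the other actor is the player character, then destroys itself whatever it struck.
; The construction script tints the Cone mesh's materials orange-red through the ColorTint parameter.
; An EnemyAttack function is present but only returns zero.
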(event `self.ReceiveHit`
  (params (MyComp :type "PrimitiveComponent Object Reference") (Other :type "Actor Object Reference") (OtherComp :type "PrimitiveComponent Object Reference") (bSelfMoved :type Boolean) (HitLocation :type "Vector Structure") (HitNormal :type "Vector Structure") (NormalImpulse :type "Vector Structure") (Hit :type "HitResult Structure (by ref)"))
  (bind _returnvalue (`GameplayStatics.GetPlayerCharacter` 0))
  (if (== Other _returnvalue)
    (message `/Game/Combat/I_Combat.TakeDamage` _returnvalue (`self.Damage`) null null null "NewEnumerator4")
    (`self.K2_DestroyActor`)
    (else
      (`self.K2_DestroyActor`))))

(fn `EnemyAttack`
  (returns (AttackDuration :type "Float (double-precision)"))
  (return 0.0))

(fn `UserConstructionScript`
  (`MeshComponent.SetVectorParameterValueOnMaterials` (`self.Cone`) "ColorTint" (`KismetMathLibrary.Conv_LinearColorToVector` (struct :`R` 0.578125 :`G` 0.036349 :`A` 1.0))))