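; BP_EliteRange is an elite ranged enemy that fires homing baseball projectiles at the player.
; On BeginPlay it sets its enemy type, prints its state and attaches its weapon to the mesh's GripPoint socket.
; EnemyAttack spawns a BP_Baseball at the sphere component with random yaw and pitch spread, then zeroes its gravity and velocity so homing acceleration alone steers it toward the first player's capsule.
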(event `self.ReceiveBeginPlay`
  (`parent.ReceiveBeginPlay`)
  (set `self.EnemyType` "NewEnumerator9")
  (`KismetSystemLibrary.PrintString` (`|GetEnumeratorNameAsString` (`self.State`)))
  (`SceneComponent.K2_AttachToComponent` (`self.Weapon Root`) (`self.Mesh`) "GripPoint" "SnapToTarget" "SnapToTarget" "KeepWorld" true))

(fn `EnemyAttack`
  (returns (AttackDuration :type "Float (double-precision)"))
  (bind (_returnvalue_roll _returnvalue_pitch _returnvalue_yaw) (`KismetMathLibrary.BreakRotator` (`SceneComponent.K2_GetComponentRotation` (`self.CapsuleComponent`))))
  (bind _returnvalue (`|SpawnActorFromClass` "/Game/Player/BaseballProj/Baseball/BP_Baseball.BP_Baseball_C" (`KismetMathLibrary.MakeTransform` (`SceneComponent.K2_GetComponentLocation` (`self.Sphere`)) (`KismetMathLibrary.MakeRotator` _returnvalue_roll (+ _returnvalue_pitch (`KismetMathLibrary.RandomFloatInRange` -2.5 5.0)) (+ _returnvalue_yaw (`KismetMathLibrary.RandomFloatInRange` -10.0 15.0))) (* (`self.Projectile Scale`) 1.0)) "AdjustIfPossibleButAlwaysSpawn" "OverrideRootScale" null (1000.0 1000.0 1000.0) "NewEnumerator4" self "NewEnumerator0" (`self.Damage`) 0.0 false 100.0 false false 3.0 null))
  (bind _output_get (set `self.Baseball Ref` _returnvalue))
  (`self.SetLifeSpan` _output_get (`self.Ball Life`))
  (bind _projectilemovement (`/Game/Player/BaseballProj/Baseball/BP_Baseball.ProjectileMovement` _output_get))
  (set `ProjectileMovementComponent.ProjectileGravityScale` 0.0 _projectilemovement)
  (set `MovementComponent.Velocity` (0.0 0.0 0.0) _projectilemovement)
  (set `ProjectileMovementComponent.HomingTargetComponent` (`Character.CapsuleComponent` (`GameplayStatics.GetPlayerCharacter` 0)) _projectilemovement)
  (set `ProjectileMovementComponent.bIsHomingProjectile` true _projectilemovement)
  (set `ProjectileMovementComponent.HomingAccelerationMagnitude` 7500.0 _projectilemovement)
  (return (`self.AttackDuration`)))

(fn `UserConstructionScript`
  (`parent.UserConstructionScript`))