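; BP_FirePool is a Grenadier enemy hazard that telegraphs an explosion, then damages and debuffs the player.
; StartExplosion blinks the radius indicator red through a timeline-driven dynamic material, then calls Explode.
; Explode runs a multi capsule trace and, on player hits, sends damage and elemental debuff messages.
; Fire particles and sound play at the actor, which destroys itself after the debuff duration.
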(event `Start Explosion`
  (bind _returnvalue (`self.K2_GetActorLocation`))
  ;[1 1 1] Do the explosion radius blinking
  (bind _returnvalue_2 (`PrimitiveComponent.CreateDynamicMaterialInstance` (`self.Explosion Radius`) 0 "/Game/Textures/PlaceHolders(PH)/M_ExplosionRed_PH.M_ExplosionRed_PH" "None"))
  (set `self.M_ExplosionRadiusMaterial` _returnvalue_2)
  (bind (_direction _color_graph) (`Timeline|T_ExplosionBlinking` :!via `PlayFromStart`)
    (:`Update`
      (`MaterialInstanceDynamic.SetVectorParameterValue` (`self.M_ExplosionRadiusMaterial`) "Explosion Radius Color" _color_graph))
    (:`Finished`
      ;[1 1 1] Explode and deal damage
      (`self.Explode`)
      ;[1 1 1] Explosion Art
      (`GameplayStatics.SpawnEmitterAtLocation` "/Game/M5VFXVOL2/Particles/Explosion/Fire_Exp_01.Fire_Exp_01" _returnvalue)
      (`GameplayStatics.SpawnSoundAtLocation` "/Game/UE4_FPTemplate/FirstPerson/Audio/FirstPersonTemplateWeaponFire02.FirstPersonTemplateWeaponFire02" _returnvalue (struct) 1.0 1.0 0.0 null null)
      (`KismetSystemLibrary.Delay` (`self.Debuff Duration`))
      (`self.K2_DestroyActor`))))

(event `Explode`
  (bind _returnvalue (`GameplayStatics.GetPlayerCharacter` 0))
  (bind _c_debufftype (`self.C_DebuffType`))
  (bind _returnvalue_2 (`SceneComponent.K2_GetComponentLocation` (`self.DefaultSceneRoot`)))
  ;[1 1 1] Explode and deal damage
  (bind _outhits (`KismetSystemLibrary.CapsuleTraceMulti` _returnvalue_2 (+ _returnvalue_2 (0.0 0.0 50.0)) 200.0 0.0 "TraceTypeQuery4"))
  (for _array_element _outhits
    (if (== (`.HitActor` (`GameplayStatics.BreakHitResult` _array_element)) _returnvalue)
      (message `/Game/Combat/I_Combat.TakeDamage` _returnvalue (`self.Explosion Damage`) null null null "NewEnumerator4")
      (message `/Game/Combat/I_Combat.ApplyDebuff` _c_debufftype (`self.Debuff Duration`) (`/Game/Combat/C_DebuffType.Player Ref` _c_debufftype) null null "NewEnumerator0"))))

(fn `UserConstructionScript`)