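; BP_Grenadier is an enemy character that attacks by spawning football bombs.
; On BeginPlay it runs the parent logic, then sets its enemy type and current element.
; The construction script snaps the weapon root to the mesh's GripPoint socket.
; EnemyAttack spawns a BP_FootballBomb at the projectile spawn point, using the capsule's rotation and the football component's scale, then returns the attack duration.
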(event `self.ReceiveBeginPlay`
  (`parent.ReceiveBeginPlay`)
  (set `self.EnemyType` "NewEnumerator8")
  (set `self.Current Element` "NewEnumerator0"))

(fn `EnemyAttack`
  (returns (AttackDuration :type "Float (double-precision)"))
  (`|SpawnActorFromClass` "/Game/AI/Enemy/Grenadier/BP_FootballBomb.BP_FootballBomb_C" (`KismetMathLibrary.MakeTransform` (`SceneComponent.K2_GetComponentLocation` (`self.Projectile Spawn`)) (`SceneComponent.K2_GetComponentRotation` (`self.CapsuleComponent`)) (`SceneComponent.K2_GetComponentScale` (`self.Footbal`))) "Undefined" "OverrideRootScale" null null)
  (return (`self.Attack Duration`)))

(fn `UserConstructionScript`
  (`parent.UserConstructionScript`)
  (`SceneComponent.K2_AttachToComponent` (`self.Weapon Root`) (`self.Mesh`) "GripPoint" "SnapToTarget" "SnapToTarget" "KeepWorld" true))