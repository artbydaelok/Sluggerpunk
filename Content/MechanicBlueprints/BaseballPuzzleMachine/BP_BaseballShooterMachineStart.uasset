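; Starting machine of the baseball puzzle, which takes in the player's baseball and fires one out along its arrow.
; Overlapping the rotating collision shows a prompt widget and lets Interact turn the rotating root in 90-degree steps.
; OnBallHit destroys player-owned balls after a short delay; their OnDestroyed event then triggers a delayed CBaseball throw in the arrow's forward direction.
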(event `self.ReceiveBeginPlay`
  (bind _returnvalue (`|CreateWidget` "/Game/Player/PlayerWidgets/W_BaseballShooterMachine.W_BaseballShooterMachine_C"))
  (set `self.BB Machine Widget` _returnvalue)
  (bind _asplayer_base_character (cast `/Game/Player/PlayerBaseCharacter` (`GameplayStatics.GetPlayerCharacter` 0)))
  (set `self.As Player Base Character` _asplayer_base_character)
  (`self.EnableInput` (`GameplayStatics.GetPlayerController` 0)))

(event `self.RotatingCollision.OnComponentBeginOverlap`
  (params (OverlappedComponent :type "PrimitiveComponent Object Reference") (OtherActor :type "Actor Object Reference") (OtherComp :type "PrimitiveComponent Object Reference") (OtherBodyIndex :type Integer) (bFromSweep :type Boolean) (SweepResult :type "HitResult Structure (by ref)"))
  (if (== OtherActor (`self.As Player Base Character`))
    (`UserWidget.AddToViewport` (`self.BB Machine Widget`) 0)
    (set `self.PlayerInRadius` true)))

(event `self.RotatingCollision.OnComponentEndOverlap`
  (params (OverlappedComponent :type "PrimitiveComponent Object Reference") (OtherActor :type "Actor Object Reference") (OtherComp :type "PrimitiveComponent Object Reference") (OtherBodyIndex :type Integer))
  (if (== OtherActor (`self.As Player Base Character`))
    (`Widget.RemoveFromParent` (`self.BB Machine Widget`))
    (set `self.PlayerInRadius` false)))

(event `InputAction|Interact` :consume false
  (params (Key :type "Key Structure"))
  (:`Pressed`
    (if (`self.PlayerInRadius`)
      (`SceneComponent.K2_AddWorldRotation` (`self.RotatingRoot`) (struct :`Yaw` 90.0) false false))))

(event `/Game/Player/BaseballProj/I_Baseball.OnBallHit`
  (params (Baseball :type "/Game/Player/BaseballProj/BP_Baseball Object Reference"))
  (if (== (`/Game/Player/BaseballProj/BP_Baseball.BallOwner` Baseball) (`GameplayStatics.GetPlayerCharacter` 0))
    (add `self.OnDestroyed` Baseball (delegate `Ball Accepted`))
    (`KismetSystemLibrary.Delay` 0.5)
    (`self.K2_DestroyActor` Baseball)))

(event `Ball Accepted` :!signature `self.OnDestroyed`
  (params (DestroyedActor :type "Actor Object Reference"))
  (bind _arrow (`self.Arrow`))
  (`KismetSystemLibrary.Delay` 0.5)
  (`/Game/Player/BaseballProj/C_Baseball.Throw Ball` (`self.C_Baseball`) (+ (`SceneComponent.K2_GetComponentLocation` _arrow) (* (`KismetMathLibrary.Normal` (`SceneComponent.GetForwardVector` _arrow)) 500.0)) (0.0 0.0 100.0) 4500.0))

(event `self.Baseball Collision.OnComponentBeginOverlap`
  (params (OverlappedComponent :type "PrimitiveComponent Object Reference") (OtherActor :type "Actor Object Reference") (OtherComp :type "PrimitiveComponent Object Reference") (OtherBodyIndex :type Integer) (bFromSweep :type Boolean) (SweepResult :type "HitResult Structure (by ref)")))

(event `self.Baseball Collision.OnComponentEndOverlap`
  (params (OverlappedComponent :type "PrimitiveComponent Object Reference") (OtherActor :type "Actor Object Reference") (OtherComp :type "PrimitiveComponent Object Reference") (OtherBodyIndex :type Integer)))

(fn `UserConstructionScript`)