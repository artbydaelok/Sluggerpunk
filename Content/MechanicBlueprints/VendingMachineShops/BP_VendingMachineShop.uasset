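; BP_VendingMachineShop is an interactable vending machine actor that opens an item shop for the player.
; It creates the interact and shop widgets at BeginPlay, and overlaps on ShopInteractRadius toggle the prompt and an in-radius flag.
; Pressing Interact in range plays a sound, shows the shop, disables movement, hides the player and switches to cursor-driven UI-only input.
; This graph has no close logic to restore player state.
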(event `self.ReceiveBeginPlay`
  (bind _returnvalue (`|CreateWidget` "/Game/Player/PlayerWidgets/W_Interact.W_Interact_C"))
  (set `self.Interact Widget` _returnvalue)
  (bind _returnvalue_2 (`|CreateWidget` "/Game/Player/PlayerWidgets/W_ItemShop.W_ItemShop_C"))
  (set `self.ItemShop Widget` _returnvalue_2)
  (bind _asplayer_base_character (cast `/Game/Player/PlayerBaseCharacter` (`GameplayStatics.GetPlayerCharacter` 0)))
  (set `self.As Player Base Character` _asplayer_base_character)
  (`self.EnableInput` (`GameplayStatics.GetPlayerController` 0)))

(event `self.ShopInteractRadius.OnComponentBeginOverlap`
  (params (OverlappedComponent :type "PrimitiveComponent Object Reference") (OtherActor :type "Actor Object Reference") (OtherComp :type "PrimitiveComponent Object Reference") (OtherBodyIndex :type Integer) (bFromSweep :type Boolean) (SweepResult :type "HitResult Structure (by ref)"))
  (if (== OtherActor (`self.As Player Base Character`))
    (`UserWidget.AddToViewport` (`self.Interact Widget`) 0)
    (set `self.PlayerInRadius?` true)))

(event `self.ShopInteractRadius.OnComponentEndOverlap`
  (params (OverlappedComponent :type "PrimitiveComponent Object Reference") (OtherActor :type "Actor Object Reference") (OtherComp :type "PrimitiveComponent Object Reference") (OtherBodyIndex :type Integer))
  (if (== OtherActor (`self.As Player Base Character`))
    (`Widget.RemoveFromParent` (`self.Interact Widget`))
    (set `self.PlayerInRadius?` false)))

(event `InputAction|Interact` :consume false
  (params (Key :type "Key Structure"))
  (bind _returnvalue (`GameplayStatics.GetPlayerController` 0))
  (:`Pressed`
    (if (`self.PlayerInRadius?`)
      (`CharacterMovementComponent.DisableMovement` (`Character.CharacterMovement` (`self.As Player Base Character`)))
      (`Widget.RemoveFromParent` (`self.Interact Widget`))
      (`GameplayStatics.PlaySound2D` "/Game/Audio/OpenShop.OpenShop" 1.0 1.0 0.0 null null)
      (`UserWidget.AddToViewport` (`self.ItemShop Widget`) 0)
      (`WidgetBlueprintLibrary.SetInputMode_UIOnlyEx` _returnvalue null)
      (set `PlayerController.bShowMouseCursor` true _returnvalue)
      (`self.SetActorHiddenInGame` (`self.As Player Base Character`) true))))

(fn `UserConstructionScript`)