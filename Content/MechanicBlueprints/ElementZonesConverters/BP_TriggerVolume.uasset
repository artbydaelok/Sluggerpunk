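; BP_TriggerVolume is a one-shot trigger that switches on lights and can open doors when the player character enters it.
; The first player overlap plays a spotlight switch sound, sets every referenced light to a configured intensity and sets a flag blocking repeats.
; If door triggering is enabled, it then calls OpenDoor on each referenced door, printing a red warning if none are valid.
; Nothing fires, doors included, unless at least one light is assigned.
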(event `self.ReceiveActorBeginOverlap`
  (params (OtherActor :type "Actor Object Reference"))
  (bind _doors (`self.Doors`))
  (if (and (== OtherActor (`GameplayStatics.GetPlayerCharacter` 0)) (`KismetArrayLibrary.Array_IsValidIndex` (`self.Lights`)) (not (`self.LightsTriggered`)))
    (`GameplayStatics.PlaySound2D` "/Game/Audio/SpotlightSwitch_SFX.SpotlightSwitch_SFX" 1.0 1.0 0.0 null null)
    (for _array_element (`self.Lights`)
      (`LightComponent.SetIntensity` (`Light.LightComponent` _array_element) (`self.LightStrength`)))
    (set `self.LightsTriggered` true)
    (if (`self.TriggersDoor`)
      (if (`KismetArrayLibrary.Array_IsValidIndex` _doors)
        (for _array_element_2 _doors
          (`/Game/Levels/OLD_LevelManager_OLD/BP_Door.Open Door` _array_element_2))
        (else
          (`KismetSystemLibrary.PrintString` "No Valid Doors Selected (Nerd)" true true (struct :`R` 1.0 :`A` 1.0)))))))

(fn `UserConstructionScript`)