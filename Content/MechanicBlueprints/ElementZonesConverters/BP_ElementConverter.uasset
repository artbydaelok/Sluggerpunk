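; BP_ElementConverter is a placeable zone that converts the element of the player's baseball on contact.
; On BeginPlay it caches the player character and tints the Converter mesh to match its ElementType of Earth, Fire or Ice.
; When the Box overlaps a player-owned BP_Baseball's Ball component, ignoring its other collision components, it calls UpdateElementAndColor to pass on that element.
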(event `self.ReceiveBeginPlay`
  (bind _converter (`self.Converter`))
  (bind _asplayer_base_character (cast `/Game/Player/PlayerBaseCharacter` (`GameplayStatics.GetPlayerCharacter` 0)))
  (set `self.PlayerCharacter` _asplayer_base_character)
  (switch `/Game/Combat/E_Element` (`self.Element Type`)
    (:`NewEnumerator3`
      (`PrimitiveComponent.SetMaterial` _converter 0 "/Game/Textures/OpacityMaterials/MI_EarthBrown.MI_EarthBrown"))
    (:`NewEnumerator0`
      (`PrimitiveComponent.SetMaterial` _converter 0 "/Game/Textures/OpacityMaterials/MI_FireRed.MI_FireRed"))
    (:`NewEnumerator1`
      (`PrimitiveComponent.SetMaterial` _converter 0 "/Game/Textures/OpacityMaterials/MI_WaterBlue.MI_WaterBlue"))))

(event `self.Box.OnComponentBeginOverlap`
  (params (OverlappedComponent :type "PrimitiveComponent Object Reference") (OtherActor :type "Actor Object Reference") (OtherComp :type "PrimitiveComponent Object Reference") (OtherBodyIndex :type Integer) (bFromSweep :type Boolean) (SweepResult :type "HitResult Structure (by ref)"))
  (bind _asbp_baseball (cast `/Game/Player/BaseballProj/Baseball/BP_Baseball` OtherActor))
  ;[1 1 1] Checking if the Ball is owned by the Player AND that the component is the Ball itself (Not the Collision Spheres)
  (if (and (== (`self.PlayerCharacter`) (`/Game/Player/BaseballProj/Baseball/BP_Baseball.BallOwner` _asbp_baseball)) (== (`/Game/Player/BaseballProj/Baseball/BP_Baseball.Ball` _asbp_baseball) OtherComp))
    (`/Game/Player/BaseballProj/Baseball/BP_Baseball.UpdateElementAndColor` _asbp_baseball (`self.Element Type`))))

(fn `UserConstructionScript`)