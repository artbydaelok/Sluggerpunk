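; Element zone that turns into Earth, Fire or Ice when hit by an elemental baseball, or from a manual preset at BeginPlay.
; Macros swap the cube's material, collision and state, with edits gated by an uneditable flag and short cooldown.
; Earth blocks until plain-ball hits wear it down and reset it.
; Ice lowers walkers' ground friction, while Fire damages overlapping health components through a flag-gated looping timer that is never cleared.
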(event `self.ReceiveBeginPlay`
  (bind _asplayer_base_character (cast `/Game/Player/PlayerBaseCharacter` (`GameplayStatics.GetPlayerCharacter` 0)))
  (bind _output_get (set `self.PlayerCharacter` _asplayer_base_character))
  (set `self.CharacterMovement` (`Character.CharacterMovement` _output_get))
  ;[1 1 1] Manual Element Set
  (if (`self.ManualElement`)
    (switch `/Game/Combat/E_Element` (`self.BallElement`)
      (:`NewEnumerator3`
        (`self.GroundMacro`))
      (:`NewEnumerator0`
        (`self.FireMacro`))
      (:`NewEnumerator1`
        (`self.IceMacro`)))))

(event `/Game/Player/BaseballProj/I_Baseball.OnBallHit`
  (params (Baseball :type "/Game/Player/BaseballProj/BP_Baseball Object Reference"))
  (set `self.BallElement` (`/Game/Player/BaseballProj/BP_Baseball.ElementalType` Baseball))
  (if (not (`self.IsUneditable`))
    (if (not (`self.IsOnCooldown`))
      ;[1 1 1] Gets Baseball's Element and Proceeds with Corresponding Element
      (switch `/Game/Combat/E_Element` (`self.BallElement`)
        (:`NewEnumerator4`
          (if (`|EnumEquality` (`self.ElementState`) "NewEnumerator0")
            (`self.GroundExec`)
            (`self.Cooldown`)))
        (:`NewEnumerator3`
          (`self.GroundMacro`))
        (:`NewEnumerator0`
          (`self.FireMacro`))
        (:`NewEnumerator1`
          (`self.IceMacro`))))
    (else
      (`KismetSystemLibrary.PrintString` "This Zone is Uneditable"))))

(event `self.WalkingSurface.OnComponentBeginOverlap`
  (params (OverlappedComponent :type "PrimitiveComponent Object Reference") (OtherActor :type "Actor Object Reference") (OtherComp :type "PrimitiveComponent Object Reference") (OtherBodyIndex :type Integer) (bFromSweep :type Boolean) (SweepResult :type "HitResult Structure (by ref)"))
  (bind _returnvalue (`self.GetComponentByClass` OtherActor "/Script/Engine.CharacterMovementComponent"))
  ;[1 1 1] Making Player Have Less Friction on the Ice Surface
  (if (`self.ActorHasTag` OtherActor "Character")
    (`/Engine/EditorBlueprintResources/StandardMacros.IsValid` _returnvalue
      (:`Is Valid`
        (if (`|EnumEquality` (`self.ElementState`) "NewEnumerator1")
          (set `CharacterMovementComponent.GroundFriction` 0.5 _returnvalue)
          (`KismetSystemLibrary.PrintString` "Low Friction Activated" true true (struct :`G` 0.421423 :`B` 1.0 :`A` 1.0))
          (else
            (set `CharacterMovementComponent.GroundFriction` 8.0 _returnvalue)
            (`KismetSystemLibrary.PrintString` "Friction Returned to Normal" true true (struct :`R` 0.916743 :`G` 0.012008 :`B` 1.0 :`A` 1.0) :!label _label))))
      (:`Is Not Valid`
        (`KismetSystemLibrary.PrintString` "Owner does not have Movement Component" :!label _label_2)))))

(event `self.WalkingSurface.OnComponentEndOverlap`
  (params (OverlappedComponent :type "PrimitiveComponent Object Reference") (OtherActor :type "Actor Object Reference") (OtherComp :type "PrimitiveComponent Object Reference") (OtherBodyIndex :type Integer))
  (bind _returnvalue (`self.GetComponentByClass` OtherActor "/Script/Engine.CharacterMovementComponent"))
  ;[1 1 1] Making Player Have Less Friction on the Ice Surface
  (if (`self.ActorHasTag` OtherActor "Character")
    (`/Engine/EditorBlueprintResources/StandardMacros.IsValid` _returnvalue
      (:`Is Valid`
        (set `CharacterMovementComponent.GroundFriction` 8.0 _returnvalue)
        (goto _label))
      (:`Is Not Valid`
        (goto _label_2)))))

(event `self.Cube.OnComponentBeginOverlap`
  (params (OverlappedComponent :type "PrimitiveComponent Object Reference") (OtherActor :type "Actor Object Reference") (OtherComp :type "PrimitiveComponent Object Reference") (OtherBodyIndex :type Integer) (bFromSweep :type Boolean) (SweepResult :type "HitResult Structure (by ref)"))
  (bind _returnvalue (`self.GetComponentByClass` OtherActor "/Game/Combat/C_HealthAndShield.C_HealthAndShield_C"))
  ;[1 1 1] If Fire, Deal Damage Every Second While Overlapping. On End Overlap, Stop Dealing damage
  (`/Engine/EditorBlueprintResources/StandardMacros.IsValid` _returnvalue
    (:`Is Valid`
      (set `self.HP/SH Component` _returnvalue)
      (if (`|EnumEquality` (`self.ElementState`) "NewEnumerator2")
        (set `self.IsInsideFire` true)
        (`KismetSystemLibrary.K2_SetTimerDelegate` (delegate `ApplyFireDamage`) 0.5 true)))))

(event `ApplyFireDamage`
  ;[1 1 1] If Fire, Deal Damage Every Second While Overlapping. On End Overlap, Stop Dealing damage
  (if (`self.IsInsideFire`)
    (`/Game/Combat/C_HealthAndShield.Heal/Take Damage` (`self.HP/SH Component`) -40.0 false)))

(event `self.Cube.OnComponentEndOverlap`
  (params (OverlappedComponent :type "PrimitiveComponent Object Reference") (OtherActor :type "Actor Object Reference") (OtherComp :type "PrimitiveComponent Object Reference") (OtherBodyIndex :type Integer))
  ;[1 1 1] If Fire, Deal Damage Every Second While Overlapping. On End Overlap, Stop Dealing damage
  (`/Engine/EditorBlueprintResources/StandardMacros.IsValid` (`self.GetComponentByClass` OtherActor "/Game/Combat/C_HealthAndShield.C_HealthAndShield_C")
    (:`Is Valid`
      (set `self.IsInsideFire` false))))

(fn `EnemyAttack`
  (returns (AttackDuration :type "Float (double-precision)"))
  (return 0.0))

(fn `GroundExec`
  (bind _cube (`self.Cube`))
  ;[1 1 1] Changes Durability of Ground Element Zone before Destroying
  (switch `int` (`self.HitsOnBox`)
    (:`0`
      (`PrimitiveComponent.SetMaterial` _cube 0 "/Game/Textures/ColoredMeshes/MI_Brown.MI_Brown")
      (`KismetSystemLibrary.PrintString` "Hit 1")
      (`/Engine/EditorBlueprintResources/StandardMacros.IncrementInt` (`self.HitsOnBox`) :!label _label
        (:`  `
          (return))))
    (:`1`
      (`PrimitiveComponent.SetMaterial` _cube 0 "/Game/Textures/ColoredMeshes/MI_DarkBrown.MI_DarkBrown")
      (`KismetSystemLibrary.PrintString` "Hit 2")
      (goto _label))
    (:`2`
      (`self.ResetZone`)
      (`KismetSystemLibrary.PrintString` "Destroyed"))))

(fn `ResetZone`
  (bind _cube (`self.Cube`))
  (set `self.HitsOnBox` 0)
  (set `self.ElementState` "NewEnumerator4")
  (set `self.ManualElement` false)
  (`PrimitiveComponent.SetCollisionResponseToAllChannels` _cube "ECR_Ignore")
  (`PrimitiveComponent.SetMaterial` _cube 0 "/Game/Textures/M_DefaultElementZone.M_DefaultElementZone"))

(fn `UserConstructionScript`)