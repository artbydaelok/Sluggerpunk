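; Purchasable upgrade computer that the player buys with gold to spawn an upgrade drop, then destroys itself.
; BeginPlay randomizes the price and scales the yaw randomly, passing the price to a popup widget.
; Sphere overlap toggles that popup and the interact flag, and enables input.
; Interact deducts gold if affordable and runs a timeline that enlarges the TV mesh before the drop, otherwise playing a failure sound.
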(event `self.ReceiveBeginPlay`
  (bind (_returnvalue_roll _returnvalue_pitch _returnvalue_yaw) (`KismetMathLibrary.BreakRotator` (`SceneComponent.K2_GetComponentRotation` (`self.SM_TV`))))
  (`self.K2_SetActorRotation` (* (`KismetMathLibrary.MakeRotator` 0.0 0.0 _returnvalue_yaw) (`KismetMathLibrary.RandomFloatInRange` 0.0 50.0)))
  (bind _output_get (set `self.UpgradePrice` (+ (* (`KismetMathLibrary.RandomIntegerInRange` 0 10) 10) 50)))
  (bind _asw_price_popup (cast `/Game/3DModels/TrainStation/W_PricePopup` (`WidgetComponent.GetWidget` (`self.EToPurchase`))))
  (bind _output_get_2 (set `self.PricePopup` _asw_price_popup))
  (set `/Game/3DModels/TrainStation/W_PricePopup.Price` _output_get _output_get_2)
  (set `self.TVScale` (`SceneComponent.K2_GetComponentScale` (`self.SM_TV`))))

(event `self.Sphere.OnComponentBeginOverlap`
  (params (OverlappedComponent :type "PrimitiveComponent Object Reference") (OtherActor :type "Actor Object Reference") (OtherComp :type "PrimitiveComponent Object Reference") (OtherBodyIndex :type Integer) (bFromSweep :type Boolean) (SweepResult :type "HitResult Structure (by ref)"))
  (bind _returnvalue (`GameplayStatics.GetPlayerCharacter` 0))
  (if (== OtherActor _returnvalue)
    (bind _asplayer_base_character (cast `/Game/Player/PlayerBaseCharacter` _returnvalue))
    (set `self.Player` _asplayer_base_character)
    (`SceneComponent.SetVisibility` (`self.EToPurchase`) true false)
    (set `self.CanInteractComputer` true)
    (bind _asplayer_base_controller (cast `/Game/Player/PlayerBaseController` (`GameplayStatics.GetPlayerController` 0)))
    (`self.EnableInput` _asplayer_base_controller)))

(event `self.Sphere.OnComponentEndOverlap`
  (params (OverlappedComponent :type "PrimitiveComponent Object Reference") (OtherActor :type "Actor Object Reference") (OtherComp :type "PrimitiveComponent Object Reference") (OtherBodyIndex :type Integer))
  (bind _returnvalue (`GameplayStatics.GetPlayerCharacter` 0))
  (if (== OtherActor _returnvalue)
    (bind _asplayer_base_character (cast `/Game/Player/PlayerBaseCharacter` _returnvalue))
    (set `self.Player` _asplayer_base_character)
    (`SceneComponent.SetVisibility` (`self.EToPurchase`) false false)
    (set `self.CanInteractComputer` false)
    (bind _asplayer_base_controller (cast `/Game/Player/PlayerBaseController` (`GameplayStatics.GetPlayerController` 0)))
    (`self.EnableInput` _asplayer_base_controller)))

(event `InputAction|Interact`
  (params (Key :type "Key Structure"))
  (bind _player (`self.Player`))
  (bind _tvscale (`self.TVScale`))
  (:`Pressed`
    (if (and (>= (`/Game/Player/PlayerBaseCharacter.CurrentGold` (`self.Player`)) (`self.UpgradePrice`)) (`self.CanInteractComputer`))
      (set `self.CanInteractComputer` false)
      (set `/Game/Player/PlayerBaseCharacter.CurrentGold` (- (`/Game/Player/PlayerBaseCharacter.CurrentGold` _player) (`self.UpgradePrice`)) _player)
      (`GameplayStatics.PlaySound2D` "/Engine/VREditor/Sounds/UI/Dockable_Window_Drop.Dockable_Window_Drop" 1.0 1.0 0.0 null null)
      (bind (_direction _computing) (`Timeline|ComputingComputed` :!via `PlayFromStart`)
        (:`Update`
          (bind (_returnvalue_location _returnvalue_rotation _returnvalue_scale) (`KismetMathLibrary.BreakTransform` (`KismetMathLibrary.TLerp` (`KismetMathLibrary.MakeTransform` (0.0 0.0 0.0) (struct) _tvscale) (`KismetMathLibrary.MakeTransform` (0.0 0.0 0.0) (struct) (* _tvscale 2.0)) _computing)))
          (`SceneComponent.SetWorldScale3D` (`self.SM_TV`) _returnvalue_scale))
        (:`Finished`
          (bind _upgrade (`/Game/Upgrades/C_UpgradeDrop.DropUpgrade` (`self.C_UpgradeDrop`) (`SceneComponent.K2_GetComponentLocation` (`self.SpawnPoint`)) false "NewEnumerator3"))
          (`/Game/Upgrades/BP_ParentUpgrade.SetUpgrade` _upgrade)
          (`self.K2_DestroyActor`)))
      (else
        (`GameplayStatics.PlaySound2D` "/Engine/EditorSounds/Notifications/CompileFailed.CompileFailed" 1.0 1.0 0.0 null null)))))

(fn `UserConstructionScript`)