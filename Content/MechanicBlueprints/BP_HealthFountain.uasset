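; Health fountain the player interacts with to buy healing for gold, with a prompt widget shown while inside its sphere.
; Interact plays a fail sound at zero gold or full health; otherwise, if affordable, it deducts gold and heals up to max health.
; Price and heal amount live on the player character: each use lowers healing, the first two double cost, and the third destroys the sphere.
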(event `self.ReceiveBeginPlay`
  (bind _returnvalue (`|CreateWidget` "/Game/Player/PlayerWidgets/W_HealthFountain.W_HealthFountain_C"))
  (set `self.W_HealthFountain` _returnvalue)
  (bind _asplayer_base_character (cast `/Game/Player/PlayerBaseCharacter` (`GameplayStatics.GetPlayerCharacter` 0)))
  (set `self.As Player Base Character` _asplayer_base_character)
  (`self.EnableInput` (`GameplayStatics.GetPlayerController` 0)))

(event `self.Sphere.OnComponentBeginOverlap`
  (params (OverlappedComponent :type "PrimitiveComponent Object Reference") (OtherActor :type "Actor Object Reference") (OtherComp :type "PrimitiveComponent Object Reference") (OtherBodyIndex :type Integer) (bFromSweep :type Boolean) (SweepResult :type "HitResult Structure (by ref)"))
  (if (== OtherActor (`self.As Player Base Character`))
    (`UserWidget.AddToViewport` (`self.W_HealthFountain`) 0)
    (set `self.Player in Radius?` true)))

(event `self.Sphere.OnComponentEndOverlap`
  (params (OverlappedComponent :type "PrimitiveComponent Object Reference") (OtherActor :type "Actor Object Reference") (OtherComp :type "PrimitiveComponent Object Reference") (OtherBodyIndex :type Integer))
  (if (== OtherActor (`self.As Player Base Character`))
    (`Widget.RemoveFromParent` (`self.W_HealthFountain`))
    (set `self.Player in Radius?` false)))

(event `InputAction|Interact` :consume false
  (params (Key :type "Key Structure"))
  (bind _as_player_base_character (`self.As Player Base Character`))
  (bind _as_player_base_character_2 (`self.As Player Base Character`))
  (bind _as_player_base_character_3 (`self.As Player Base Character`))
  (bind _currentcosthealthfountain (`/Game/Player/PlayerBaseCharacter.CurrentCostHealthFountain` _as_player_base_character))
  (bind _currentgold (`/Game/Player/PlayerBaseCharacter.CurrentGold` _as_player_base_character))
  (bind _c_healthandshield (`/Game/Player/PlayerBaseCharacter.C_HealthAndShield` (`self.As Player Base Character`)))
  (bind _c_healthandshield_2 (`/Game/Player/PlayerBaseCharacter.C_HealthAndShield` _as_player_base_character_3))
  (bind _c_healthandshield_3 (`/Game/Player/PlayerBaseCharacter.C_HealthAndShield` (`self.As Player Base Character`)))
  (bind _returnvalue (- (`/Game/Player/PlayerBaseCharacter.CurrentHealingHealthFountain` _as_player_base_character_2) 10.0))
  (:`Pressed`
    (if (`self.Player in Radius?`)
      (if (<= _currentgold 0)
        (`GameplayStatics.PlaySound2D` "/Engine/EditorSounds/Notifications/CompileFailed.CompileFailed" 1.0 1.0 0.0 null null :!label _label)
        (elif (== (`/Game/Combat/C_HealthAndShield.Current Health` _c_healthandshield) (`/Game/Combat/C_HealthAndShield.Max Health` _c_healthandshield))
          (goto _label)
          (elif (>= _currentgold _currentcosthealthfountain)
            (set `/Game/Player/PlayerBaseCharacter.CurrentGold` (- _currentgold _currentcosthealthfountain) _as_player_base_character_3)
            (set `/Game/Combat/C_HealthAndShield.Current Health` (+ (`/Game/Player/PlayerBaseCharacter.CurrentHealingHealthFountain` _as_player_base_character_3) (`/Game/Combat/C_HealthAndShield.Current Health` _c_healthandshield_2)) _c_healthandshield_2)
            (if (> (`/Game/Combat/C_HealthAndShield.Current Health` _c_healthandshield_3) (`/Game/Combat/C_HealthAndShield.Max Health` _c_healthandshield_3))
              (set `/Game/Combat/C_HealthAndShield.Current Health` (`/Game/Combat/C_HealthAndShield.Max Health` _c_healthandshield_2) _c_healthandshield_2))
            (set `self.CurrentUses` (+ (`self.CurrentUses`) 1))
            (if (== (`self.CurrentUses`) 1)
              (set `/Game/Player/PlayerBaseCharacter.CurrentHealingHealthFountain` _returnvalue _as_player_base_character_2 :!label _label_2)
              (set `/Game/Player/PlayerBaseCharacter.CurrentCostHealthFountain` (* (`/Game/Player/PlayerBaseCharacter.CurrentCostHealthFountain` _as_player_base_character_2) 2) _as_player_base_character_2)
              (elif (== (`self.CurrentUses`) 2)
                (goto _label_2)
                (elif (== (`self.CurrentUses`) 3)
                  (set `/Game/Player/PlayerBaseCharacter.CurrentHealingHealthFountain` _returnvalue _as_player_base_character_2)
                  (`ActorComponent.K2_DestroyComponent` (`self.Sphere`)))))))))))

(fn `UserConstructionScript`)