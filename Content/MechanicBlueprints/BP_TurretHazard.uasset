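; Turret hazard that fires gravity-free baseballs at the player and drops gold when destroyed.
; Each tick it finds the nearest player in range with line of sight, rotates toward it and, once aligned and off cooldown, fires a short DoN-looped burst through CBaseball.
; Baseballs it does not own damage its health component until it explodes.
; Its health bar widget hides when the player is far away.
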(event `self.ReceiveBeginPlay`
  (bind _shoot (`self.Shoot`))
  (bind _asplayer_base_character (cast `/Game/Player/PlayerBaseCharacter` (`GameplayStatics.GetPlayerCharacter` 0)))
  (set `self.As Player Base Character` _asplayer_base_character)
  (bind _asw_turret_health (cast `/Game/AI/Enemy/W_TurretHealth` (`WidgetComponent.GetWidget` (`self.Health Bar`))))
  (bind _output_get (set `self.As W Turret Health` _asw_turret_health))
  (`/Game/AI/Enemy/W_TurretHealth.Set Reference` _output_get self)
  (set `AudioComponent.VolumeModulationMax` 1.0 _shoot)
  (set `AudioComponent.VolumeModulationMin` 1.0 _shoot))

(event `self.ReceiveTick`
  (params (DeltaSeconds :type "Float (single-precision)"))
  (bind _as_w_turret_health (`self.As W Turret Health`))
  (if (>= (`KismetMathLibrary.GetPointDistanceToLine` (`self.K2_GetActorLocation` (`GameplayStatics.GetPlayerCharacter` 0)) (`self.K2_GetActorLocation` self)) 2500.0)
    (`Widget.SetVisibility` _as_w_turret_health "Hidden")
    (else
      (`Widget.SetVisibility` _as_w_turret_health "Visible")))
  (`self.FindTarget`)
  (`self.Target`
    (:`then`
      (`self.UpdateTurretRotation` DeltaSeconds)
      (`self.UpdateFire`))
    (:`else`)))

(event `Fire`
  (bind _c_baseball (`self.C_Baseball`))
  (bind _target (`self.Target`))
  (set `self.TimeOfLastFire` (`KismetSystemLibrary.GetGameTimeInSeconds`))
  (`|ExecutionSequence`
    (:`then_0`
      (goto _label :!via `Reset`))
    (:`then_1`
      (`/Engine/EditorBlueprintResources/StandardMacros.Do N` 2 :!label _label
        (:`Exit`
          (`/Engine/EditorBlueprintResources/StandardMacros.IsValid` _target
            (:`Is Valid`
              (bind _thrownbaseball (`/Game/Player/BaseballProj/C_Baseball.Throw Ball` _c_baseball (+ (`self.K2_GetActorLocation` _target) (0.0 0.0 50.0)) (0.0 0.0 140.0) 5000.0 3.0))
              (`self.Play Sound`)
              (`/Game/Player/BaseballProj/BP_Baseball.ToggleGravity` _thrownbaseball false)
              (`/Game/Player/BaseballProj/C_Baseball.ResetCooldown` _c_baseball)
              (`KismetSystemLibrary.Delay` 0.2)
              (goto _label))))))))

(event `Play Sound`
  (bind _shoot (`self.Shoot`))
  (if (not (`AudioComponent.IsPlaying` _shoot))
    (`AudioComponent.SetPitchMultiplier` _shoot (`KismetMathLibrary.RandomFloatInRange` 1.0 1.2))
    (`AudioComponent.Play` _shoot 0.0)
    (`KismetSystemLibrary.Delay` 0.25)
    (`AudioComponent.Play` _shoot 0.0)))

(event `self.Collision.OnComponentBeginOverlap`
  (params (OverlappedComponent :type "PrimitiveComponent Object Reference") (OtherActor :type "Actor Object Reference") (OtherComp :type "PrimitiveComponent Object Reference") (OtherBodyIndex :type Integer) (bFromSweep :type Boolean) (SweepResult :type "HitResult Structure (by ref)"))
  (bind _c_healthandshield (`self.C_HealthAndShield`))
  (bind _asbp_baseball (cast `/Game/Player/BaseballProj/BP_Baseball` OtherActor))
  (bind _output_get (set `self.As BP Baseball` _asbp_baseball))
  (`ActorComponent.Activate` (`self.Sparks`) false)
  (if (!= (`/Game/Player/BaseballProj/BP_Baseball.BallOwner` _output_get) self)
    (`KismetSystemLibrary.Delay` 0.5)
    (`/Game/Combat/C_HealthAndShield.Heal/Take Damage` _c_healthandshield -34.0 false)
    (`/Engine/EditorBlueprintResources/StandardMacros.IsValid` null
      (:`Is Valid`
        (if (<= (`/Game/Combat/C_HealthAndShield.Current Health` _c_healthandshield) 0.0)
          (`KismetSystemLibrary.Delay` 0.2)
          (`self.On Death`))))))

(event `self.TakeDamage`
  (params (Damage :type "Float (single-precision)") (Player :type "/Game/Player/PlayerBaseCharacter Object Reference") (Enemy :type "/Game/AI/Enemy/BP_Enemy Object Reference") (Boss :type "/Game/AI/Boss/BP_Boss Object Reference") (Element :type "/Game/Combat/E_Element Enum" :default "NewEnumerator4") (DealsKnockback :type Boolean) (`KB Multiplier` :type "Float (single-precision)"))
  (bind _c_healthandshield (`self.C_HealthAndShield`))
  (`/Game/Combat/C_HealthAndShield.Heal/Take Damage` _c_healthandshield -34.0 false)
  (`/Engine/EditorBlueprintResources/StandardMacros.IsValid` null
    (:`Is Valid`
      (if (<= (`/Game/Combat/C_HealthAndShield.Current Health` _c_healthandshield) 0.0)
        (`KismetSystemLibrary.Delay` 0.2)
        (`self.On Death`)))))

(event `self.On Death`
  (bind _returnvalue (`self.K2_GetActorLocation`))
  (`|SpawnActorFromClass` "/Game/Collectibles/BP_Gold.BP_Gold_C" (`KismetMathLibrary.MakeTransform` (`SceneComponent.K2_GetComponentLocation` (`self.GoldAnchor`))) "Undefined" "OverrideRootScale" null 5 "NewEnumerator5" false null)
  (`GameplayStatics.SpawnEmitterAtLocation` "/Game/M5VFXVOL2/Particles/Explosion/Fire_Exp_01.Fire_Exp_01" _returnvalue (struct :`Pitch` 45.0))
  (`GameplayStatics.SpawnSoundAtLocation` "/Game/UE4_FPTemplate/FirstPerson/Audio/FirstPersonTemplateWeaponFire02.FirstPersonTemplateWeaponFire02" _returnvalue (struct) 1.0 1.0 0.0 null null)
  (`self.K2_DestroyActor`))

(fn `EnemyAttack`
  (returns (AttackDuration :type "Float (double-precision)"))
  (return 0.0))

(fn `EnemyShockwave`
  (returns (`Attack Duration` :type "Float (double-precision)"))
  (return 0.0))

(fn `FindTarget`
  (locals (BestTarget :type "Actor Object Reference") (CurrentTarget :type "Actor Object Reference") (CurrentDistance :type "Float (double-precision)") (Distance :type "Float (double-precision)"))
  (set `local.Distance` (+ (`self.Range`) 1.0))
  (bind _outactors (`KismetSystemLibrary.SphereOverlapActors` (`self.K2_GetActorLocation`) (`self.Range`) (`|MakeArray` "ObjectTypeQuery3" :!type "EObjectTypeQuery Enum") "/Game/Player/PlayerBaseCharacter.PlayerBaseCharacter_C"))
  (for _array_element _outactors
    (bind _output_get (set `local.CurrentTarget` _array_element))
    (bind _output_get_2 (set `local.CurrentDistance` (`self.GetDistanceTo` _output_get self)))
    (if (or (< _output_get_2 (`local.Distance`)) (not (`KismetSystemLibrary.IsValid` (`local.BestTarget`))))
      (bind _result (`self.HasLineOfSight` (`SceneComponent.K2_GetComponentLocation` (`self.Body`)) (`self.K2_GetActorLocation` (`local.CurrentTarget`)) (`|MakeArray` self (`local.CurrentTarget`) :!type "Actor Object Reference")))
      (if _result
        (set `local.BestTarget` (`local.CurrentTarget`))
        (set `local.Distance` (`local.CurrentDistance`)))))
  (set `self.Target` (`local.BestTarget`)))

(fn `HasLineOfSight`
  (params (From :type "Vector Structure") (To :type "Vector Structure") (ActorsToIgnore :type "Array of Actor Object Reference (by ref)"))
  (returns (Result :type Boolean))
  (bind (_outhit _returnvalue) (`KismetSystemLibrary.LineTraceSingle` From To "TraceTypeQuery1" false ActorsToIgnore))
  (return (not _returnvalue)))

(fn `UpdateFire`
  (if (> (- (`KismetSystemLibrary.GetGameTimeInSeconds`) (`self.TimeOfLastFire`)) (`self.RateOfFire`))
    (if (> (`KismetMathLibrary.Dot_VectorVector` (`KismetMathLibrary.GetDirectionUnitVector` (`SceneComponent.K2_GetComponentLocation` (`self.Body`)) (`self.K2_GetActorLocation` (`self.Target`))) (`SceneComponent.GetForwardVector` (`self.Body`))) 0.99)
      (`self.Fire`))))

(fn `UpdateTurretRotation`
  (params (DeltaSeconds :type "Float (double-precision)"))
  (`SceneComponent.K2_SetWorldRotation` (`self.Body`) (`KismetMathLibrary.RInterpTo_Constant` (`SceneComponent.K2_GetComponentRotation` (`self.Body`)) (`KismetMathLibrary.FindLookAtRotation` (`SceneComponent.K2_GetComponentLocation` (`self.Body`)) (`self.K2_GetActorLocation` (`self.Target`))) (`local.DeltaSeconds`) (`self.Interp Speed`)) false false))

(fn `UserConstructionScript`
  (`SceneComponent.SetVisibility` (`self.Health Bar`) true false))