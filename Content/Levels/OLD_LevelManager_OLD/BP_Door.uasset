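; Level door actor, filed under an old level manager folder, that moves a Door and an EntranceBlocker vertically through open and close events.
; OpenDoor animates both components with one timeline, offset from their cached heights.
; Both close events instantly lower the blocker a fixed distance, then animate the Door.
; CloseDoorEntrance offsets from the Door's cached height, while CloseDoorExit uses its timeline value directly as relative Z.
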(event `Close Door Entrance`
  (bind _door (`self.Door`))
  (bind _entranceblocker (`self.EntranceBlocker`))
  (bind (_relativelocation_x _relativelocation_y _relativelocation_z) (`KismetMathLibrary.BreakVector` (`SceneComponent.RelativeLocation` _entranceblocker)))
  (bind (_relativelocation_x_2 _relativelocation_y_2 _relativelocation_z_2) (`KismetMathLibrary.BreakVector` (`SceneComponent.RelativeLocation` (`self.Door`))))
  (bind (_relativelocation_x_3 _relativelocation_y_3) (`KismetMathLibrary.BreakVector` (`SceneComponent.RelativeLocation` _door)))
  (`SceneComponent.K2_SetRelativeLocation` _entranceblocker (`KismetMathLibrary.MakeVector` _relativelocation_x _relativelocation_y (- _relativelocation_z 400.0)) false false)
  (set `self.Relative Door Location Z` _relativelocation_z_2)
  (bind (_direction _newtrack_0) (`Timeline|T_Close Door Entrance` :!via `PlayFromStart`)
    (:`Update`
      (`SceneComponent.K2_SetRelativeLocation` _door (`KismetMathLibrary.MakeVector` _relativelocation_x_3 _relativelocation_y_3 (+ (`self.Relative Door Location Z`) _newtrack_0)) false false))))

(event `Open Door`
  (bind _door (`self.Door`))
  (bind _entranceblocker (`self.EntranceBlocker`))
  (bind (_relativelocation_x _relativelocation_y) (`KismetMathLibrary.BreakVector` (`SceneComponent.RelativeLocation` _door)))
  (bind (_relativelocation_x_2 _relativelocation_y_2) (`KismetMathLibrary.BreakVector` (`SceneComponent.RelativeLocation` _entranceblocker)))
  (bind (_relativelocation_x_3 _relativelocation_y_3 _relativelocation_z) (`KismetMathLibrary.BreakVector` (`SceneComponent.RelativeLocation` (`self.Door`))))
  (bind (_relativelocation_x_4 _relativelocation_y_4 _relativelocation_z_2) (`KismetMathLibrary.BreakVector` (`SceneComponent.RelativeLocation` (`self.EntranceBlocker`))))
  (set `self.Relative Door Location Z` _relativelocation_z)
  (set `self.Relative Door Blocker Location Z` _relativelocation_z_2)
  (bind (_direction _newtrack_0) (`Timeline|T_Open Door` :!via `PlayFromStart`)
    (:`Update`
      (`SceneComponent.K2_SetRelativeLocation` _door (`KismetMathLibrary.MakeVector` _relativelocation_x _relativelocation_y (+ (`self.Relative Door Location Z`) _newtrack_0)) false false)
      (`SceneComponent.K2_SetRelativeLocation` _entranceblocker (`KismetMathLibrary.MakeVector` _relativelocation_x_2 _relativelocation_y_2 (+ (`self.Relative Door Blocker Location Z`) _newtrack_0)) false false))))

(event `Close Door Exit`
  (bind _door (`self.Door`))
  (bind _entranceblocker (`self.EntranceBlocker`))
  (bind (_relativelocation_x _relativelocation_y _relativelocation_z) (`KismetMathLibrary.BreakVector` (`SceneComponent.RelativeLocation` _entranceblocker)))
  (bind (_relativelocation_x_2 _relativelocation_y_2) (`KismetMathLibrary.BreakVector` (`SceneComponent.RelativeLocation` _door)))
  (`SceneComponent.K2_SetRelativeLocation` _entranceblocker (`KismetMathLibrary.MakeVector` _relativelocation_x _relativelocation_y (- _relativelocation_z 400.0)) false false)
  (bind (_direction _newtrack_0) (`Timeline|T_Close Door Exit` :!via `PlayFromStart`)
    (:`Update`
      (`SceneComponent.K2_SetRelativeLocation` _door (`KismetMathLibrary.MakeVector` _relativelocation_x_2 _relativelocation_y_2 _newtrack_0) false false))))

(fn `UserConstructionScript`)