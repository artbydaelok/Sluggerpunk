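; BP_EndLevel is an interactable level exit that returns the player to the MainMenu level.
; When CanEndLevel is set, the player entering or leaving its Box toggles CanInteract, the character's CanInteractEnd flag and the actor's input from the player controller.
; Pressing E while CanInteract is true opens MainMenu by name and clears both interaction flags.
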(event `Key|E`
  (params (Key :type "Key Structure"))
  (:`Pressed`
    (if (`self.CanInteract`)
      (`GameplayStatics.OpenLevel` "MainMenu")
      (set `self.CanInteract` false)
      (set `/Game/Player/PlayerBaseCharacter.CanInteractEnd` false (stale `self.Box.OnComponentBeginOverlap` _asplayer_base_character)))))

(event `self.Box.OnComponentBeginOverlap`
  (params (OverlappedComponent :type "PrimitiveComponent Object Reference") (OtherActor :type "Actor Object Reference") (OtherComp :type "PrimitiveComponent Object Reference") (OtherBodyIndex :type Integer) (bFromSweep :type Boolean) (SweepResult :type "HitResult Structure (by ref)"))
  (bind _returnvalue (`GameplayStatics.GetPlayerCharacter` 0))
  (if (`self.Can End Level?`)
    (if (== OtherActor _returnvalue)
      (set `self.CanInteract` true)
      (bind _asplayer_base_character (cast `/Game/Player/PlayerBaseCharacter` _returnvalue))
      (set `/Game/Player/PlayerBaseCharacter.CanInteractEnd` true _asplayer_base_character)
      (bind _asplayer_base_controller (cast `/Game/Player/PlayerBaseController` (`GameplayStatics.GetPlayerController` 0)))
      (`self.EnableInput` _asplayer_base_controller))))

(event `self.Box.OnComponentEndOverlap`
  (params (OverlappedComponent :type "PrimitiveComponent Object Reference") (OtherActor :type "Actor Object Reference") (OtherComp :type "PrimitiveComponent Object Reference") (OtherBodyIndex :type Integer))
  (bind _returnvalue (`GameplayStatics.GetPlayerCharacter` 0))
  (if (`self.Can End Level?`)
    (if (== OtherActor _returnvalue)
      (set `self.CanInteract` false)
      (bind _asplayer_base_character (cast `/Game/Player/PlayerBaseCharacter` _returnvalue))
      (set `/Game/Player/PlayerBaseCharacter.CanInteractEnd` false _asplayer_base_character)
      (bind _asplayer_base_controller (cast `/Game/Player/PlayerBaseController` (`GameplayStatics.GetPlayerController` 0)))
      (`self.DisableInput` _asplayer_base_controller))))

(fn `UserConstructionScript`)