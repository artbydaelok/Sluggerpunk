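; BP_RoomManager is a level room controller that spawns the room's enemies when the player first triggers its PlayerDetectEnemySpawn overlap.
; SpawnEnemies selects an enemy class from each spawn location's type, initializes its AIC_Enemy controller, and records it in EnemiesSpawned.
; A FinishedSpawning flag blocks repeat spawns.
; ExplosionMelee and Boss have no class assigned, and the OpenDoors and CloseDoors functions are empty stubs.
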(event `self.PlayerDetectEnemySpawn.OnActorBeginOverlap`
  (params (OverlappedActor :type "Actor Object Reference") (OtherActor :type "Actor Object Reference"))
  (if (and (== OtherActor (`GameplayStatics.GetPlayerCharacter` 0)) (not (`self.FinishedSpawning`)))
    (`self.SpawnEnemies`)))

(fn `CloseDoors`)

(fn `OpenDoors`)

(fn `SpawnEnemies`
  (for _array_element (`self.SpawnLocations`)
    (bind _enemytype (`/Game/AI/Enemy/BP_SpawnLocation.EnemyType` _array_element))
    (bind _returnvalue (`|SpawnActorFromClass` (select `/Game/AI/Enemy/E_EnemyTypes` _enemytype :`NewEnumerator0` "/Game/AI/Enemy/Melee/BP_MeleeEnemy.BP_MeleeEnemy_C" :`NewEnumerator3` "/Game/AI/Enemy/Range/BP_RangeEnemy.BP_RangeEnemy_C" :`NewEnumerator8` "/Game/AI/Enemy/Grenadier/BP_Grenadier.BP_Grenadier_C" :`NewEnumerator1` "/Game/AI/Enemy/Melee/BP_EliteMelee.BP_EliteMelee_C" :`NewEnumerator9` "/Game/AI/Enemy/Range/BP_EliteRange.BP_EliteRange_C" :!type "Actor Class Reference") (`self.GetTransform` _array_element) "Undefined" "OverrideRootScale" null null))
    (bind _asbp_enemy (cast `/Game/AI/Enemy/BP_Enemy` _returnvalue))
    (set `/Game/AI/Enemy/BP_Enemy.EnemyType` _enemytype _asbp_enemy)
    (bind _asaic_enemy (cast `/Game/AI/Enemy/AIC_Enemy` (`AIBlueprintHelperLibrary.GetAIController` _asbp_enemy)))
    (`/Game/AI/Enemy/AIC_Enemy.Set Up AIC` _asaic_enemy)
    (`KismetArrayLibrary.Array_AddUnique` (`self.EnemiesSpawned`) _asbp_enemy))
  (set `self.FinishedSpawning` true))

(fn `UserConstructionScript`)