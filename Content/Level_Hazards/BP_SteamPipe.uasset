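; BP_SteamPipe is a level hazard that periodically vents damaging steam.
; On BeginPlay a looping five-second timer starts after a random initial delay, so separate pipes fire out of sync.
; Each burst plays a vent sound and Niagara effect, deals one instant hit to actors in SteamZone implementing I_Combat, then stops the effect after a short delay.
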(event `self.ReceiveBeginPlay`
  (`KismetSystemLibrary.K2_SetTimerDelegate` (delegate `Steampowered`) 5.0 true (`KismetMathLibrary.RandomFloatInRange` 0.5 3.14)))

(event `Steampowered`
  (bind _overlappingactors (`PrimitiveComponent.GetOverlappingActors` (`self.SteamZone`) "/Script/Engine.Actor"))
  (`AudioComponent.Play` (`self.VentNoise`) 0.0)
  (`ActorComponent.Activate` (`self.Niagara`) true)
  (if (`KismetArrayLibrary.Array_IsValidIndex` _overlappingactors)
    (for _array_element _overlappingactors
      (if (`KismetSystemLibrary.DoesImplementInterface` _array_element "/Game/Combat/I_Combat.I_Combat_C")
        (message `/Game/Combat/I_Combat.TakeDamage` _array_element 50.0 null null null "NewEnumerator4" true))))
  (`KismetSystemLibrary.Delay` 0.9)
  (`ActorComponent.Deactivate` (`self.Niagara`)))

(fn `UserConstructionScript`)