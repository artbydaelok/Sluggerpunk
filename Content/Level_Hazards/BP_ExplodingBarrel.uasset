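; BP_ExplodingBarrel is a level hazard that explodes when damaged.
; Any incoming damage applies a large fixed health loss through CHealthAndShield, bypassing shield, and triggers OnDeath once health is depleted.
; OnDeath uses DoOnce to have CExplosion spawn a single blast at the barrel's location, then destroys the actor after a short delay.
; EnemyAttack is a stub returning zero.
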(event `/Game/Combat/I_Combat.TakeDamage`
  (params (Damage :type "Float (single-precision)") (Player :type "/Game/Player/PlayerBaseCharacter Object Reference") (Enemy :type "/Game/AI/Enemy/BP_Enemy Object Reference") (Boss :type "/Game/AI/Boss/BP_Boss Object Reference") (Element :type "/Game/Combat/E_Element Enum" :default "NewEnumerator4"))
  (bind _c_healthandshield (`self.C_HealthAndShield`))
  (`/Game/Combat/C_HealthAndShield.Heal/Take Damage` _c_healthandshield -1000.0 true)
  (if (<= (`/Game/Combat/C_HealthAndShield.Current Health` _c_healthandshield) 0.0)
    (`/Game/Combat/I_Combat.On Death`)))

(event `/Game/Combat/I_Combat.On Death`
  (`/Engine/EditorBlueprintResources/StandardMacros.DoOnce` false
    (:`Completed`
      (`/Game/AI/ExplosionMechanic/C_Explosion.Spawn Explosion` (`self.C_Explosion`) (`SceneComponent.K2_GetComponentLocation` (`self.DefaultSceneRoot`)))
      (`KismetSystemLibrary.Delay` 2.0)
      (`self.K2_DestroyActor`))))

(fn `EnemyAttack`
  (returns (AttackDuration :type "Float (double-precision)"))
  (return 0.0))

(fn `UserConstructionScript`)