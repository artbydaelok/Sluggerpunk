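; BP_Gate is a level hazard gate whose bars rise when its linked Target is hit.
; On BeginPlay it binds LiftBars to the Target's OnTargetHit event and stores the bars' starting world location.
; LiftBars plays a timeline from the start, lerping the bars upward along world Z from that stored location to a fixed height above it.
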(event `self.ReceiveBeginPlay`
  (add `/Game/Level_Hazards/BP_TargetTraining.OnTargetHit` (`self.Target`) (delegate `LiftBars`))
  (set `self.InitialBarsLocation` (`SceneComponent.K2_GetComponentLocation` (`self.Bars`))))

(event `LiftBars`
  (bind _initialbarslocation (`self.InitialBarsLocation`))
  (bind (_direction _alpha) (`Timeline|LiftBarsAnimation` :!via `PlayFromStart`)
    (:`Update`
      (`SceneComponent.K2_SetWorldLocation` (`self.Bars`) (`KismetMathLibrary.VLerp` _initialbarslocation (+ _initialbarslocation (* (`KismetMathLibrary.Vector_Up`) 250.0)) _alpha) false false))))

(fn `UserConstructionScript`)