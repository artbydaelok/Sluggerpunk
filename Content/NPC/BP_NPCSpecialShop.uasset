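; NPC special shop Blueprint that the player talks to in order to open the special shop UI.
; A radius overlap toggles the NPC prompt text and gates the Interact input, which calls the CDialogue component.
; When dialogue returns true, it shows the pre-built shop widget with UI-only input and cursor, and hides the player character.
; Older text-row dialogue logic remains unconnected.
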(event `self.ReceiveBeginPlay`
  (bind _returnvalue (`|CreateWidget` "/Game/Player/PlayerWidgets/W_Interact.W_Interact_C"))
  (set `self.Interact Widget` _returnvalue)
  (bind _returnvalue_2 (`|CreateWidget` "/Game/Player/PlayerWidgets/W_SpecialShop.W_SpecialShop_C"))
  (set `self.W_SpecialShop` _returnvalue_2)
  (bind _returnvalue_3 (`|CreateWidget` "/Game/Player/PlayerWidgets/W_NPCInteract.W_NPCInteract_C"))
  (set `self.W NPCInteract` _returnvalue_3)
  (`/Game/Player/PlayerWidgets/W_SpecialShop.SetSpecials` (`self.W_SpecialShop`))
  (bind _asplayer_base_character (cast `/Game/Player/PlayerBaseCharacter` (`GameplayStatics.GetPlayerCharacter` 0)))
  (set `self.As Player Base Character` _asplayer_base_character)
  (`self.EnableInput` (`GameplayStatics.GetPlayerController` 0)))

(event `self.SpecialShopInteractRadius.OnComponentBeginOverlap`
  (params (OverlappedComponent :type "PrimitiveComponent Object Reference") (OtherActor :type "Actor Object Reference") (OtherComp :type "PrimitiveComponent Object Reference") (OtherBodyIndex :type Integer) (bFromSweep :type Boolean) (SweepResult :type "HitResult Structure (by ref)"))
  (if (== OtherActor (`self.As Player Base Character`))
    (`SceneComponent.SetVisibility` (`self.NPCText`) true false)
    (set `self.PlayerInRadius?` true)))

(event `self.SpecialShopInteractRadius.OnComponentEndOverlap`
  (params (OverlappedComponent :type "PrimitiveComponent Object Reference") (OtherActor :type "Actor Object Reference") (OtherComp :type "PrimitiveComponent Object Reference") (OtherBodyIndex :type Integer))
  (if (== OtherActor (`self.As Player Base Character`))
    (`SceneComponent.SetVisibility` (`self.NPCText`) false false)
    (set `self.PlayerInRadius?` false)))

(event `InputAction|Interact` :consume false
  (params (Key :type "Key Structure"))
  (:`Pressed`
    (if (`self.PlayerInRadius?`)
      (`self.DialogueEventSpecial`))))

(event `DialogueEventSpecial`
  (bind _returnvalue (`GameplayStatics.GetPlayerController` 0))
  (bind _lastdialogue_ (`/Game/DialogueSystem/C_Dialogue.Dialogue` (`self.C_Dialogue`) (`self.SpeechSFX`)))
  (if _lastdialogue_
    (`GameplayStatics.PlaySound2D` "/Game/Audio/OpenShop.OpenShop" 1.0 1.0 0.0 null null)
    (`UserWidget.AddToViewport` (`self.W_SpecialShop`) 0)
    (`WidgetBlueprintLibrary.SetInputMode_UIOnlyEx` _returnvalue null)
    (set `PlayerController.bShowMouseCursor` true _returnvalue)
    (`self.SetActorHiddenInGame` (`self.As Player Base Character`) true)
    (`Widget.SetVisibility` (`/Game/Player/PlayerBaseCharacter.W_HUD` (`self.As Player Base Character`)) "Visible")
    (`Widget.SetVisibility` (`/Game/Player/PlayerWidgets/W_NPCInteract.DialogueBG` (`self.W NPCInteract`)) "Hidden")
    (`Widget.SetVisibility` (`/Game/Player/PlayerWidgets/W_NPCInteract.Dialogue` (`self.W NPCInteract`)) "Hidden")))

(event `ResetDialogueSpecial`)

(fn `UserConstructionScript`)