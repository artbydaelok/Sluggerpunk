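; BP_NPCTrader is a trader NPC that sells randomly chosen upgrades to the player.
; On BeginPlay it creates the shop widget and gathers up to three unique upgrades from its CUpgradeDrop component.
; An overlap radius toggles the prompt text and CDialogue's interact widget.
; Pressing Interact in range runs the dialogue, and when that returns true it opens the shop with those upgrades in UI-only input mode.
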(event `self.ReceiveBeginPlay`
  (bind _returnvalue (`|CreateWidget` "/Game/Player/PlayerWidgets/W_Interact.W_Interact_C"))
  (set `self.Interact Widget` _returnvalue)
  (bind _returnvalue_2 (`|CreateWidget` "/Game/Player/PlayerWidgets/W_TraderShop.W_TraderShop_C"))
  (set `self.TraderShop` _returnvalue_2)
  (bind _asplayer_base_character (cast `/Game/Player/PlayerBaseCharacter` (`GameplayStatics.GetPlayerCharacter` 0)))
  (set `self.As Player Base Character` _asplayer_base_character)
  (`self.EnableInput` (`GameplayStatics.GetPlayerController` 0))
  ;[1 1 1] Chooses 3  upgrades
  (for _ (range 3)
    (bind _out_row (`/Game/Upgrades/C_UpgradeDrop.ChooseRandomUpgrade` (`self.C_UpgradeDrop`)))
    (`KismetArrayLibrary.Array_AddUnique` (`self.Upgrades_`) _out_row)))

(event `self.UpgradeShopInteractRadius.OnComponentBeginOverlap`
  (params (OverlappedComponent :type "PrimitiveComponent Object Reference") (OtherActor :type "Actor Object Reference") (OtherComp :type "PrimitiveComponent Object Reference") (OtherBodyIndex :type Integer) (bFromSweep :type Boolean) (SweepResult :type "HitResult Structure (by ref)"))
  (if (== OtherActor (`self.As Player Base Character`))
    (`SceneComponent.SetVisibility` (`self.TextRender`) true false)
    (set `self.PlayerInRadius?` true)
    (`UserWidget.AddToViewport` (`/Game/DialogueSystem/C_Dialogue.NPC Interact WIdget` (`self.C_Dialogue`)) 0)))

(event `self.UpgradeShopInteractRadius.OnComponentEndOverlap`
  (params (OverlappedComponent :type "PrimitiveComponent Object Reference") (OtherActor :type "Actor Object Reference") (OtherComp :type "PrimitiveComponent Object Reference") (OtherBodyIndex :type Integer))
  (bind _npc_interact_widget (`/Game/DialogueSystem/C_Dialogue.NPC Interact WIdget` (`self.C_Dialogue`)))
  (if (== OtherActor (`self.As Player Base Character`))
    (`SceneComponent.SetVisibility` (`self.TextRender`) false false)
    (set `self.PlayerInRadius?` false)
    (`/Engine/EditorBlueprintResources/StandardMacros.IsValid` _npc_interact_widget
      (:`Is Valid`
        (`Widget.RemoveFromParent` _npc_interact_widget)))))

(event `InputAction|Interact` :consume false
  (params (Key :type "Key Structure"))
  (:`Pressed`
    (if (`self.PlayerInRadius?`)
      (`self.DialogueEvent`))))

(event `DialogueEvent`
  (bind _returnvalue (`GameplayStatics.GetPlayerController` 0))
  (bind _tradershop (`self.TraderShop`))
  (bind _lastdialogue_ (`/Game/DialogueSystem/C_Dialogue.Dialogue` (`self.C_Dialogue`) (`self.DialogueSFX`)))
  (if _lastdialogue_
    (`GameplayStatics.PlaySound2D` "/Game/Audio/OpenShop.OpenShop" 1.0 1.0 0.0 null null)
    (`UserWidget.AddToViewport` _tradershop 0)
    (`/Game/Player/PlayerWidgets/W_TraderShop.RandomUpgrades` _tradershop (`self.Upgrades_`))
    (set `PlayerController.bShowMouseCursor` true _returnvalue)
    (`WidgetBlueprintLibrary.SetInputMode_UIOnlyEx` _returnvalue null)
    (`Widget.SetVisibility` (`/Game/Player/PlayerWidgets/W_NPCInteract.DialogueBG` (`/Game/DialogueSystem/C_Dialogue.NPC Interact WIdget` (`self.C_Dialogue`))) "Hidden")
    (`Widget.SetVisibility` (`/Game/Player/PlayerWidgets/W_NPCInteract.Dialogue` (`/Game/DialogueSystem/C_Dialogue.NPC Interact WIdget` (`self.C_Dialogue`))) "Hidden")))

(fn `UserConstructionScript`)