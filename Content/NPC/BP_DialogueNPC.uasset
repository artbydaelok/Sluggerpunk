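; An NPC actor that the player can talk to, with an optional floating exclamation marker animated by a timeline.
; Entering its interaction field hides the marker, shows a prompt and enables input; leaving hides the prompt.
; While in range, interact, click or trigger calls the dialogue component, whose boolean result toggles between the NPC view with player mesh, prompt and input off, and the restored player view.
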(event `self.ReceiveBeginPlay`
  (bind _exclamation (`self.Exclamation`))
  (if (`self.ExclamationVisible?`)
    (`SceneComponent.SetVisibility` _exclamation true false)
    (else
      (`SceneComponent.SetVisibility` _exclamation false false)))
  (bind _returnvalue (`GameplayStatics.GetActorOfClass` "/Game/Player/PlayerBaseCharacter.PlayerBaseCharacter_C"))
  (set `self.Player` _returnvalue)
  (bind (_direction _newtrack_0) (`Timeline|Float`)
    (:`Update`
      (`SceneComponent.K2_SetRelativeLocation` (`self.Exclamation`) (`KismetMathLibrary.VLerp` (0.0 0.0 200.0) (0.0 0.0 210.0) _newtrack_0) false false))))

(event `self.InteractionField.OnComponentBeginOverlap`
  (params (OverlappedComponent :type "PrimitiveComponent Object Reference") (OtherActor :type "Actor Object Reference") (OtherComp :type "PrimitiveComponent Object Reference") (OtherBodyIndex :type Integer) (bFromSweep :type Boolean) (SweepResult :type "HitResult Structure (by ref)"))
  (if (== OtherActor (`self.Player`))
    (`/Engine/EditorBlueprintResources/StandardMacros.IsValid` (`self.Exclamation`)
      (:`Is Valid`
        (`SceneComponent.SetVisibility` (`self.Exclamation`) false false))
      (:`Is Not Valid`
        _))
    (set `self.PlayerInRadius` true)
    (`SceneComponent.SetVisibility` (`self.InteractText`) true false)
    (`self.EnableInput` (`GameplayStatics.GetPlayerController` 0))))

(event `self.InteractionField.OnComponentEndOverlap`
  (params (OverlappedComponent :type "PrimitiveComponent Object Reference") (OtherActor :type "Actor Object Reference") (OtherComp :type "PrimitiveComponent Object Reference") (OtherBodyIndex :type Integer))
  (if (== OtherActor (`self.Player`))
    (set `self.PlayerInRadius` false)
    (`SceneComponent.SetVisibility` (`self.InteractText`) false false)))

(event `InputAction|Interact` :consume false
  (params (Key :type "Key Structure"))
  (bind _returnvalue (`GameplayStatics.GetPlayerController` 0))
  (:`Pressed`
    (if (`self.PlayerInRadius`) :!label _label
      (bind _lastdialogue_ (`/Game/DialogueSystem/C_Dialogue.Dialogue` (`self.C_Dialogue`) (`self.SpeechSFX`)))
      (`PlayerController.SetViewTargetWithBlend` (`GameplayStatics.GetPlayerController` 0) (select `bool` _lastdialogue_ :`false` self :`true` (`self.Player`) :!type "Actor Object Reference") 0.5 "VTBlend_Linear" 0.0 false)
      (`SceneComponent.SetVisibility` (`/Game/Player/PlayerBaseCharacter.CharacterMesh` (`self.Player`)) _lastdialogue_ true)
      (`SceneComponent.SetVisibility` (`self.InteractText`) _lastdialogue_ true)
      (if _lastdialogue_
        (`self.EnableInput` _returnvalue _returnvalue)
        (`self.EnableInput` (`self.Player`) _returnvalue)
        (`/Game/Player/PlayerBaseCharacter.SetVisibilityActiveWeapon` (`self.Player`))
        (else
          (`self.DisableInput` (`self.Player`) _returnvalue))))))

(event `Key|LeftMouseButton` :consume false
  (params (Key :type "Key Structure"))
  (:`Pressed`
    (goto _label)))

(event `Key|Gamepad_RightTrigger` :consume false
  (params (Key :type "Key Structure"))
  (:`Pressed`
    (goto _label)))

(fn `UserConstructionScript`)