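; BP_WarpBlock is a level warp actor that opens LevelToOpen when the player enters its Box.
; On BeginPlay it finds the PlayerBaseCharacter and builds a "Go to" label from the level's name, cut from its object path.
; Each tick it turns on yaw only to face the player.
; The box overlap opens the level only when the overlapping actor is that player.
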(event `self.ReceiveTick`
  (params (DeltaSeconds :type "Float (single-precision)"))
  (bind (_returnvalue_roll _returnvalue_pitch _returnvalue_yaw) (`KismetMathLibrary.BreakRotator` (`KismetMathLibrary.FindLookAtRotation` (`self.K2_GetActorLocation`) (`self.K2_GetActorLocation` (`self.Player`)))))
  (`self.K2_SetActorRotation` (`KismetMathLibrary.MakeRotator` 0.0 0.0 _returnvalue_yaw)))

(event `self.ReceiveBeginPlay`
  (bind _returnvalue (`KismetSystemLibrary.Conv_SoftObjectReferenceToString` (`self.LevelToOpen`)))
  (bind _returnvalue_2 (`GameplayStatics.GetActorOfClass` "/Game/Player/PlayerBaseCharacter.PlayerBaseCharacter_C"))
  (set `self.Player` _returnvalue_2)
  (`TextRenderComponent.K2_SetText` (`self.TextRender`) (`KismetTextLibrary.Conv_StringToText` (`KismetStringLibrary.Concat_StrStr` "Go to " (`KismetStringLibrary.GetSubstring` _returnvalue (+ (`KismetStringLibrary.FindSubstring` _returnvalue "." false true) 1) 20)))))

(event `self.Box.OnComponentBeginOverlap`
  (params (OverlappedComponent :type "PrimitiveComponent Object Reference") (OtherActor :type "Actor Object Reference") (OtherComp :type "PrimitiveComponent Object Reference") (OtherBodyIndex :type Integer) (bFromSweep :type Boolean) (SweepResult :type "HitResult Structure (by ref)"))
  (if (== OtherActor (`self.Player`))
    (`GameplayStatics.OpenLevelBySoftObjectPtr` (`self.LevelToOpen`))))

(fn `UserConstructionScript`)